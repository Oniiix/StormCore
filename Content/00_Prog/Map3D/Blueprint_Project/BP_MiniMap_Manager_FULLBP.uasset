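; BP_MiniMap_Manager is a minimap actor pairing a MapViewCapture scene capture component with a Niagara system.
; On BeginPlay it sets the capture to perspective HDR final color, rendering only this actor, with automatic capture disabled and rendering state persistent.
; Each Tick manually advances the Niagara simulation by the frame delta, intended to keep it animating while the game is paused.
; No capture call appears in this Blueprint.
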(event EventBeginPlay
  ;[1 1 1] initialize our scene capture component
  (MiniMap|Initialization|InitializeSceneCaptureComponent))

(event EventTick
  (params (DeltaSeconds :type Float%20%28single-precision%29))
  ;[1 1 1] manually tick our Niagara particle system
  (Class|NiagaraComponent|AdvanceSimulation (Variables|Default|GetNiagara) 1 DeltaSeconds))

(fn ConstructionScript)

(fn InitializeSceneCaptureComponent
  (bind _mapviewcapture (Variables|Default|GetMapViewCapture))
  (Utilities|FlowControl|Sequence
    (:then_0
      (Variables|/Script/Engine.SceneCaptureComponent|SetbAlwaysPersistRenderingState _mapviewcapture true)
      (Variables|/Script/Engine.SceneCaptureComponent|SetCaptureSource _mapviewcapture "SCS_FinalColorHDR")
      (Variables|/Script/Engine.SceneCaptureComponent2D|SetCompositeMode _mapviewcapture "SCCM_Overwrite")
      (Variables|/Script/Engine.SceneCaptureComponent2D|SetProjectionType _mapviewcapture "Perspective")
      (Variables|/Script/Engine.SceneCaptureComponent|SetbCaptureEveryFrame _mapviewcapture false)
      (Variables|/Script/Engine.SceneCaptureComponent|SetbCaptureOnMovement _mapviewcapture false))
    (:then_1
      (Variables|/Script/Engine.SceneCaptureComponent|SetShowOnlyActors _mapviewcapture (Utilities|Array|MakeArray self))
      (Variables|/Script/Engine.SceneCaptureComponent|SetPrimitiveRenderMode _mapviewcapture "PRM_UseShowOnlyList"))))