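; Example minimap pawn that wires player input to the MiniMapManager for map navigation and custom marker placement or removal.
; On BeginPlay it sizes the custom marker index list, adds a marker hint widget to the minimap widget and refreshes it when the highlighted marker changes.
; Pause-proof inputs cover look, move, zoom, reset and marker cycling, though their manager calls and the marker helper functions are empty here.
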(event Custom|HighlightedMarkerUpdated
  (params (bHighlight :type Boolean) (HighlightID :type Name) (HighlightMarker :type %20Object%20Reference))
  ;[1 1 1] minimap manager's updated its highlighted marker, we may no longer want to display our 'remove custom marker' widget because we simply may no longer be able to
  (CallFunction|UpdateCustomMarkerWidgetRemoveBox HighlightID HighlightMarker))

(event EventTick
  (params (DeltaSeconds :type Float%20%28single-precision%29))
  ;[1 1 1] add/remove custom marker(s)
  (CallFunction|UpdateCustomMarkerInputTime))

(event EventBeginPlay
  (bind _custommarkerscount (Variables|Default|GetCustomMarkersCount))
  (bind _minimapwidget (Variables|Default|GetMiniMapWidget))
  (Utilities|FlowControl|Sequence
    (:then_0
      ;[1 1 1] initialize our list of available custom markers
      (if (> _custommarkerscount 0)
        (Utilities|Array|SetArrayElem (Variables|Default|GetCustomMarkerIndexes) (- _custommarkerscount 1) false true)))
    (:then_1
      ;[1 1 1] bind manager's highlight marker update event
      (Utilities|IsValid (Variables|Default|GetMiniMapManager)
        (:Is%20Valid
          (EventDispatchers|BindEventtoMiniMapHighlightUpdated (delegate Custom|HighlightedMarkerUpdated))
          ;[1 1 1] get our custom widget and add it to one of our minimap widget's available box and update it
          (bind _widget (CallFunction|GetCustomMarkerWidgetSingleton))
          (Utilities|IsValid _minimapwidget
            (:Is%20Valid
              (Class|VerticalBox|AddChildtoVerticalBox (Variables|/Script/RobotHunter.WDG_MiniMap|GetCursorBottomRightBox _minimapwidget) _widget)
              (CallFunction|UpdateCustomMarkerWidgetAddBox))))))))

(event Input|ActionEvents|InputActionMiniMapMarkerScrollDown
  (params (Key :type Key%20Structure :default "None"))
  ;[1 1 1] loop through *ALL* existing markers
  (:Pressed
    (Utilities|IsValid (Variables|Default|GetMiniMapManager))))

(event Input|ActionEvents|InputActionMiniMapHighlightScrollDown
  (params (Key :type Key%20Structure :default "None"))
  ;[1 1 1] loop through focused markers (if we do focus *multiple* markers)
  (:Pressed
    (Utilities|IsValid (Variables|Default|GetMiniMapManager))))

(event Input|ActionEvents|InputActionMiniMapHighlightScrollUp
  (params (Key :type Key%20Structure :default "None"))
  ;[1 1 1] loop through focused markers (if we do focus *multiple* markers)
  (:Pressed
    (Utilities|IsValid (Variables|Default|GetMiniMapManager))))

(event Input|ActionEvents|InputActionMiniMapMarkerScrollUp
  (params (Key :type Key%20Structure :default "None"))
  ;[1 1 1] loop through *ALL* existing markers
  (:Pressed
    (Utilities|IsValid (Variables|Default|GetMiniMapManager))))

(event Input|ActionEvents|InputActionMiniMapSpeedUp
  (params (Key :type Key%20Structure :default "None"))
  ;[1 1 1] increased movement speed
  (:Pressed
    (Utilities|IsValid (Variables|Default|GetMiniMapManager)))
  (:Released
    (Utilities|IsValid (Variables|Default|GetMiniMapManager))))

(event Input|ActionEvents|InputActionMiniMapReset
  (params (Key :type Key%20Structure :default "None"))
  ;[1 1 1] reset minimap view's location/rotation/zoom on our pawn
  (:Pressed
    (Utilities|IsValid (Variables|Default|GetMiniMapManager))))

(event Input|ActionEvents|InputActionMiniMapMarker
  (params (Key :type Key%20Structure :default "None"))
  ;[1 1 1] add/remove custom marker(s)
  (:Pressed
    (CallFunction|CustomMarkerInputPressed))
  (:Released
    (CallFunction|CustomMarkerInputReleased)))

(event Input|AxisEvents|InputAxisLookUp
  (params (AxisValue :type Float%20%28single-precision%29))
  ;[1 1 1] add minimap view & movement inputs. Note that all events here are configured to tick EVEN IF game is paused (that *is* necessary if you want to pause the game while in the minimap menu and still have it working)
  (if (!= AxisValue 0.0)
    (Utilities|IsValid (Variables|Default|GetMiniMapManager))))

(event Input|AxisEvents|InputAxisLookRight
  (params (AxisValue :type Float%20%28single-precision%29))
  ;[1 1 1] add minimap view & movement inputs. Note that all events here are configured to tick EVEN IF game is paused (that *is* necessary if you want to pause the game while in the minimap menu and still have it working)
  (if (!= AxisValue 0.0)
    (Utilities|IsValid (Variables|Default|GetMiniMapManager))))

(event Input|AxisEvents|InputAxisMoveRight
  (params (AxisValue :type Float%20%28single-precision%29))
  ;[1 1 1] add minimap view & movement inputs. Note that all events here are configured to tick EVEN IF game is paused (that *is* necessary if you want to pause the game while in the minimap menu and still have it working)
  (if (!= AxisValue 0.0)
    (Utilities|IsValid (Variables|Default|GetMiniMapManager))))

(event Input|AxisEvents|InputAxisMoveForward
  (params (AxisValue :type Float%20%28single-precision%29))
  ;[1 1 1] add minimap view & movement inputs. Note that all events here are configured to tick EVEN IF game is paused (that *is* necessary if you want to pause the game while in the minimap menu and still have it working)
  (if (!= AxisValue 0.0)
    (Utilities|IsValid (Variables|Default|GetMiniMapManager))))

(event Input|AxisEvents|InputAxisMiniMapMoveUp
  (params (AxisValue :type Float%20%28single-precision%29))
  ;[1 1 1] add minimap view & movement inputs. Note that all events here are configured to tick EVEN IF game is paused (that *is* necessary if you want to pause the game while in the minimap menu and still have it working)
  (if (!= AxisValue 0.0)
    (Utilities|IsValid (Variables|Default|GetMiniMapManager))))

(event Input|AxisEvents|InputAxisMiniMapZoom
  (params (AxisValue :type Float%20%28single-precision%29))
  ;[1 1 1] add minimap view & movement inputs. Note that all events here are configured to tick EVEN IF game is paused (that *is* necessary if you want to pause the game while in the minimap menu and still have it working)
  (if (!= AxisValue 0.0)
    (Utilities|IsValid (Variables|Default|GetMiniMapManager))))

(event Input|AxisEvents|InputAxisMiniMapZoomGamepad
  (params (AxisValue :type Float%20%28single-precision%29))
  ;[1 1 1] add minimap view & movement inputs. Note that all events here are configured to tick EVEN IF game is paused (that *is* necessary if you want to pause the game while in the minimap menu and still have it working)
  (if (!= AxisValue 0.0)
    (Utilities|IsValid (Variables|Default|GetMiniMapManager))))

(fn ConstructionScript
  (|CallParentFunction))

(fn UpdateCustomMarkerWidgetAddBox)

(fn CustomMarkerInputPressed)

(fn CustomMarkerInputReleased)

(fn UpdateCustomMarkerInputTime)

(fn GetCustomMarkerWidgetSingleton
  (return 0))

(fn UpdateCustomMarkerWidgetRemoveBox
  (params (HighlightMarkerID :type Name) (HighlightMarker :type %20Object%20Reference)))