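; BP_3D_Map_Sector3 is a 3D map actor, apparently for Sector 3, that tracks the main character with an animated marker.
; Each Tick it divides the character capsule's world location by 100 and writes it to the "Player 1 Position" parameter in MPC_Interraction for materials to read.
; The same scaled position sets the Pawn marker's relative location, with a sine-driven vertical bob and a steady time-based yaw spin.
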(event EventBeginPlay)

(event Collision|EventActorBeginOverlap
  (params (OtherActor :type Actor%20Object%20Reference)))

(event EventTick
  (params (DeltaSeconds :type Float%20%28single-precision%29))
  (bind _returnvalue (Actor|GetGameTimeSinceCreation))
  (bind _maincharacter (Variables|Default|GetmainCharacter))
  (bind _capsulecomponent (Variables|/Script/Engine.Character|GetCapsuleComponent _maincharacter))
  (bind _returnvalue_2 (Transformation|GetWorldLocation _capsulecomponent))
  (bind _returnvalue_3 (/ _returnvalue_2 "100.000000,100.000000,100.000000"))
  (bind (_x _y _z) (Math|Vector|BreakVector _returnvalue_3))
  (Rendering|Material|SetVectorParameterValue "/Game/06_Tech/Materials/MPC/MPC_Interraction.MPC_Interraction" "Player 1 Position" (Math|Conversions|ToLinearColor(Vector) _returnvalue_3) :!class /Script/Engine.KismetMaterialLibrary)
  (Transformation|SetRelativeLocationAndRotation (Variables|Default|Getpawn) (Math|Vector|MakeVector _x _y (+ _z (* (* (+ (Math|Trig|Sin(Radians) _returnvalue) 1.0) 0.5) 2.0))) (Math|Rotator|MakeRotator 0.0 0.0 (* _returnvalue 5e+01)) false false))

(fn ConstructionScript)