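; Main player character Blueprint that handles audiovisual feedback for damage, healing, death, bumps, aiming and pausing.
; InitializeMaterials builds dynamic body, arm and leg materials by player and equipped calf, which damage and heal timelines animate with hit direction.
; Smoothed camera velocity, scope and health states feed material parameter collections, while death blends a post-process material.
; Temporary server-to-multicast landed and jump events set a test flag for animation replication.
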(event OnLifeChangebyDamage(lifeComponent)
  (params (_owner :type Actor%20Object%20Reference) (_currentLife :type Integer) (_damage :type Integer) (_damageSource :type Actor%20Object%20Reference))
  (bind _returnvalue (Transformation|GetActorLocation _damageSource))
  (bind _returnvalue_2 (Transformation|GetActorLocation _owner))
  (bind _materialbody (Variables|Default|GetMaterialBody))
  (bind _materialhand (Variables|Default|GetMaterialHand))
  (bind _materiallegs (Variables|Default|GetMaterialLegs))
  (bind _returnvalue_3 (Math|Vector|GetUnitDirection(Vector) _returnvalue _returnvalue_2))
  (bind _returnvalue_4 (Math|Conversions|ToLinearColor(Vector) _returnvalue_3))
  ;[1 1 1] DAMAGED
  (Utilities|FlowControl|Sequence
    (:then_0
      ;;[1 1 1] Camera Feedback (Temp)
      (Rendering|Material|SetScalarParameterValue "/Game/06_Tech/Materials/MPC/MPC_Interraction.MPC_Interraction" "Damage_Statut" (- 1.0 (/ _currentLife (Class|LifeComponent|GetMaxLife (Class|MainCharacter|GetLifeComponent)))) :!class /Script/Engine.KismetMaterialLibrary))
    (:then_1
      (Utilities|IsValid _damageSource
        (:Is%20Valid
          (Audio|PlaySoundatLocation "/Game/05_Audio/SFX/MetaSounds/Player/Getting_Hit/Player1/MSS_GettingHit_Player1.MSS_GettingHit_Player1" (Transformation|GetActorLocation) "0, 0, 0" 1.0 1.0 0.0 0 0 0 0))))
    (:then_2
      ;[1 1 1] Hit direction
      (Utilities|IsValid _damageSource
        (:Is%20Valid
          (Rendering|Material|SetVectorParameterValue (Variables|Default|GetMaterialBody) "Hit_Direction" _returnvalue_4 :!class /Script/Engine.MaterialInstanceDynamic)
          (Rendering|Material|SetVectorParameterValue (Variables|Default|GetMaterialHand) "Hit_Direction" _returnvalue_4 :!class /Script/Engine.MaterialInstanceDynamic)
          (Rendering|Material|SetVectorParameterValue (Variables|Default|GetMaterialLegs) "Hit_Direction" _returnvalue_4 :!class /Script/Engine.MaterialInstanceDynamic))))
    (:then_3
      (bind (_direction _line_position _coloremissive _line_width _visibility_scanner) (Timeline|TL_Damage_Hit PlayFromStart)
        (:Update
          (Utilities|FlowControl|Sequence
            (:then_0
              (Rendering|Material|SetScalarParameterValue _materialbody "Line Position" _line_position :!class /Script/Engine.MaterialInstanceDynamic)
              (Rendering|Material|SetVectorParameterValue _materialbody "Color fresnel" (Math|Conversions|ToLinearColor(Vector) _coloremissive) :!class /Script/Engine.MaterialInstanceDynamic)
              (Rendering|Material|SetScalarParameterValue _materialbody "Line Width" _line_width :!class /Script/Engine.MaterialInstanceDynamic)
              (Rendering|Material|SetScalarParameterValue _materialbody "Visibilty Damage Hit" _visibility_scanner :!class /Script/Engine.MaterialInstanceDynamic))
            (:then_1
              (Rendering|Material|SetScalarParameterValue _materialhand "Line Position" _line_position :!class /Script/Engine.MaterialInstanceDynamic)
              (Rendering|Material|SetVectorParameterValue _materialhand "Color fresnel" (Math|Conversions|ToLinearColor(Vector) _coloremissive) :!class /Script/Engine.MaterialInstanceDynamic)
              (Rendering|Material|SetScalarParameterValue _materialhand "Line Width" _line_width :!class /Script/Engine.MaterialInstanceDynamic)
              (Rendering|Material|SetScalarParameterValue _materialhand "Visibilty Damage Hit" _visibility_scanner :!class /Script/Engine.MaterialInstanceDynamic))
            (:then_2
              (Rendering|Material|SetScalarParameterValue _materiallegs "Line Position" _line_position :!class /Script/Engine.MaterialInstanceDynamic)
              (Rendering|Material|SetVectorParameterValue _materiallegs "Color fresnel" (Math|Conversions|ToLinearColor(Vector) _coloremissive) :!class /Script/Engine.MaterialInstanceDynamic)
              (Rendering|Material|SetScalarParameterValue _materiallegs "Line Width" _line_width :!class /Script/Engine.MaterialInstanceDynamic)
              (Rendering|Material|SetScalarParameterValue _materiallegs "Visibilty Damage Hit" _visibility_scanner :!class /Script/Engine.MaterialInstanceDynamic))))))))

(event OnLifeChangebyHeal(lifeComponent)
  (params (_owner :type Actor%20Object%20Reference) (_currentLife :type Integer) (_heal :type Integer) (_damageSource :type Actor%20Object%20Reference))
  (bind _returnvalue (Math|Conversions|ToLinearColor(Vector) "0.000000,0.000000,1.000000"))
  (bind _materialbody (Variables|Default|GetMaterialBody))
  (bind _materiallegs (Variables|Default|GetMaterialLegs))
  (bind _materialhand (Variables|Default|GetMaterialHand))
  ;[1 1 1] HEALED
  (Utilities|FlowControl|Sequence
    (:then_0
      (Utilities|FlowControl|Delay 0.57)
      ;;[1 1 1] Camera Feedback (Temp)
      (bind _switchcolor (Timeline|TL_Effect PlayFromStart)
        (:Update
          (Rendering|Material|SetScalarParameterValue "/Game/06_Tech/Materials/MPC/MPC_Interraction.MPC_Interraction" "Effect_Lerp" _switchcolor :!class /Script/Engine.KismetMaterialLibrary)
          (Rendering|Material|SetScalarParameterValue "/Game/06_Tech/Materials/MPC/MPC_Interraction.MPC_Interraction" "Damage_Statut" _switchcolor :!class /Script/Engine.KismetMaterialLibrary))
        (:Finished
          (Rendering|Material|SetScalarParameterValue "/Game/06_Tech/Materials/MPC/MPC_Interraction.MPC_Interraction" "Damage_Statut" (- 1.0 (/ _currentLife (Class|LifeComponent|GetMaxLife (Class|MainCharacter|GetLifeComponent)))) :!class /Script/Engine.KismetMaterialLibrary))))
    (:then_1
      ;;[1 1 1] Healed SFX
      (Utilities|FlowControl|Delay 0.57)
      (Audio|PlaySoundatLocation "/Game/05_Audio/SFX/MetaSounds/Player/Healed/MSS_Healed_v1.MSS_Healed_v1" (Transformation|GetActorLocation) "0, 0, 0" 1.0 1.0 0.0 0 0 0 0))
    (:then_2
      (Utilities|FlowControl|Sequence
        (:then_0
          (Rendering|Material|SetVectorParameterValue (Variables|Default|GetMaterialBody) "Hit_Direction" _returnvalue :!class /Script/Engine.MaterialInstanceDynamic)
          (Rendering|Material|SetVectorParameterValue (Variables|Default|GetMaterialHand) "Hit_Direction" _returnvalue :!class /Script/Engine.MaterialInstanceDynamic)
          (Rendering|Material|SetVectorParameterValue (Variables|Default|GetMaterialLegs) "Hit_Direction" _returnvalue :!class /Script/Engine.MaterialInstanceDynamic))
        (:then_1
          (bind (_direction _line_position _coloremissive _line_width _visibility_scanner) (Timeline|TL_Heal PlayFromStart)
            (:Update
              (Utilities|FlowControl|Sequence
                (:then_0
                  (Rendering|Material|SetScalarParameterValue _materialbody "Line Position" _line_position :!class /Script/Engine.MaterialInstanceDynamic)
                  (Rendering|Material|SetVectorParameterValue _materialbody "Color fresnel" (Math|Conversions|ToLinearColor(Vector) _coloremissive) :!class /Script/Engine.MaterialInstanceDynamic)
                  (Rendering|Material|SetScalarParameterValue _materialbody "Line Width" _line_width :!class /Script/Engine.MaterialInstanceDynamic)
                  (Rendering|Material|SetScalarParameterValue _materialbody "Visibilty Damage Hit" _visibility_scanner :!class /Script/Engine.MaterialInstanceDynamic))
                (:then_1
                  (Rendering|Material|SetScalarParameterValue _materialhand "Line Position" _line_position :!class /Script/Engine.MaterialInstanceDynamic)
                  (Rendering|Material|SetVectorParameterValue _materialhand "Color fresnel" (Math|Conversions|ToLinearColor(Vector) _coloremissive) :!class /Script/Engine.MaterialInstanceDynamic)
                  (Rendering|Material|SetScalarParameterValue _materialhand "Line Width" _line_width :!class /Script/Engine.MaterialInstanceDynamic)
                  (Rendering|Material|SetScalarParameterValue _materialhand "Visibilty Damage Hit" _visibility_scanner :!class /Script/Engine.MaterialInstanceDynamic))
                (:then_2
                  (Rendering|Material|SetScalarParameterValue _materiallegs "Line Position" _line_position :!class /Script/Engine.MaterialInstanceDynamic)
                  (Rendering|Material|SetVectorParameterValue _materiallegs "Color fresnel" (Math|Conversions|ToLinearColor(Vector) _coloremissive) :!class /Script/Engine.MaterialInstanceDynamic)
                  (Rendering|Material|SetScalarParameterValue _materiallegs "Line Width" _line_width :!class /Script/Engine.MaterialInstanceDynamic)
                  (Rendering|Material|SetScalarParameterValue _materiallegs "Visibilty Damage Hit" _visibility_scanner :!class /Script/Engine.MaterialInstanceDynamic))))))))))

(event OnUpdateLife(lifeComponent)
  (params (_owner :type Actor%20Object%20Reference) (_currentLife :type Integer) (_change :type Integer) (_damageSource :type Actor%20Object%20Reference)))

(event OnDie(lifeComponent)
  (Utilities|FlowControl|Sequence
    (:then_0
      (bind _deathvaluepp (Timeline|TL_Death Play)
        (:Update
          _)
        (:Finished
          _))
      (Utilities|Struct|SetmembersinPostProcessSettings (Variables|/Script/Engine.CameraComponent|GetPostProcessSettings (Variables|/Script/RobotHunter.CustomCameraComponent|Getcamera (Variables|Default|GetcameraComponent))) (Utilities|Struct|MakeWeightedBlendables (Utilities|Array|MakeArray (Utilities|Struct|MakeWeightedBlendable _deathvaluepp "/Game/04_FX/MaterialPostprocess/MmPP_Death.MmPP_Death") (Utilities|Struct|MakeWeightedBlendable 1.0 "/Game/04_FX/MaterialPostprocess/MMPP_DamageStatut.MMPP_DamageStatut")))))
    (:then_1
      (Audio|PushSoundMixModifier "/Game/05_Audio/SoundClass_Mixes/Day_Message/SCM_Day_Message3.SCM_Day_Message3"))))

(event Custom|RotateCameraSpringArm
  (params (Rotation :type Rotator))
  (Transformation|SetWorldRotation (Variables|/Script/RobotHunter.CustomCameraComponent|GetspringArm (Variables|Default|GetcameraComponent)) Rotation false false))

(event Custom|onJump_Event
  (params (_status :type Boolean))
  ;[1 0.3512 0.4109] ABP Replication Test (A SUPPRIMER DES QUE LES VARIABLES EN C++ SONT RÉPLIQUÉES)
  ;;[1 1 1] On Jumped
  (CallFunction|SonJump _status))

(event Custom|onScopeSound_Event
  (params (_status :type Boolean))
  (Audio|PlaySoundatLocation (select _status "/Game/05_Audio/SFX/MetaSounds/Player/Weapons/Right_Arm/Shotgun/Shotgun_Aim_Start/v4/MSS_Shotgun_Aim_Start_v4.MSS_Shotgun_Aim_Start_v4" "/Game/05_Audio/SFX/MetaSounds/Player/Weapons/Right_Arm/Shotgun/Shotgun_Aim_Start/v4/MSS_Shotgun_Aim_Start_v4.MSS_Shotgun_Aim_Start_v4") (Transformation|GetActorLocation) "0, 0, 0" 1.0 1.0 0.0 0 0 0 0))

(event Custom|S_OnJump
  (params (Status :type Boolean))
  ;[1 0.3512 0.4109] ABP Replication Test (A SUPPRIMER DES QUE LES VARIABLES EN C++ SONT RÉPLIQUÉES)
  ;;[1 1 1] On Jumped
  (CallFunction|MonJump Status))

(event Custom|M_OnJump
  (params (Status :type Boolean))
  ;[1 0.3512 0.4109] ABP Replication Test (A SUPPRIMER DES QUE LES VARIABLES EN C++ SONT RÉPLIQUÉES)
  ;;[1 1 1] On Jumped
  (Variables|Default|SetTEST_IsJumping true))

(event Custom|onScopeSound_Event_0
  (params (_status :type Boolean))
  (if _status
    (Rendering|Material|SetScalarParameterValue "/Game/06_Tech/UI/Material/UI_Material/MPC/MPC_HUD.MPC_HUD" "Scope" 1.0 :!class /Script/Engine.KismetMaterialLibrary)
    (else
      (Rendering|Material|SetScalarParameterValue "/Game/06_Tech/UI/Material/UI_Material/MPC/MPC_HUD.MPC_HUD" "Scope" 0.0 :!class /Script/Engine.KismetMaterialLibrary))))

(event Custom|S_OnLanded
  ;[1 0.3512 0.4109] ABP Replication Test (A SUPPRIMER DES QUE LES VARIABLES EN C++ SONT RÉPLIQUÉES)
  ;;[1 1 1] On Landed
  (CallFunction|MonLanded))

(event Custom|M_OnLanded
  ;[1 0.3512 0.4109] ABP Replication Test (A SUPPRIMER DES QUE LES VARIABLES EN C++ SONT RÉPLIQUÉES)
  ;;[1 1 1] On Landed
  (Variables|Default|SetTEST_IsJumping false))

(event Custom|onShoot_Event
  (params (tiltRatio :type Float%20%28single-precision%29)))

(event Custom|onCalfInit_Event
  (params (_calf :type Calf%20Actor%20Object%20Reference))
  (CallFunction|InitializeMaterials _calf))

(event Custom|OnBump_Event
  (params (_status :type Boolean) (_isBumpByAI :type Boolean))
  (Audio|SpawnSoundatLocation "/Game/05_Audio/SFX/MetaSounds/Player/Getting_Bumped/Mono_Version/MSS_Getting_Bumped_Mono.MSS_Getting_Bumped_Mono" (Transformation|GetActorLocation) "0, 0, 0" (+ (* (not _isBumpByAI) 0.55) 1.0) 1.0 0.0 0 0))

(event EventTick
  (params (DeltaSeconds :type Float%20%28single-precision%29))
  (bind _rot_delta_max (Variables|Default|GetRot_Delta_Max))
  (bind _returnvalue (- 0.0 _rot_delta_max))
  (Utilities|FlowControl|Sequence
    (:then_0
      (Variables|Default|SetSmooth_UI_Cam_Speeds (Class|KismetMathLibrary|Vector2DInterptoConstant (Variables|Default|GetSmooth_UI_Cam_Speeds) (* (Math|Vector2D|MakeVector2D (Math|Float|Clamp(Float) (.Yaw (Math|Rotator|BreakRotator (Math|Rotator|Delta(Rotator) (Variables|Default|GetPrevious_Rotation) (Transformation|GetWorldRotation (Variables|/Script/RobotHunter.CustomCameraComponent|GetspringArm (Variables|Default|GetcameraComponent)))))) _returnvalue _rot_delta_max) (Math|Float|Clamp(Float) (.Pitch (Math|Rotator|BreakRotator (Math|Rotator|Delta(Rotator) (Variables|Default|GetPrevious_Rotation) (Transformation|GetWorldRotation (Variables|/Script/RobotHunter.CustomCameraComponent|GetspringArm (Variables|Default|GetcameraComponent)))))) _returnvalue _rot_delta_max)) DeltaSeconds) DeltaSeconds (Variables|Default|GetUI_Rot_Speed))))
    (:then_1
      (Rendering|Material|SetVectorParameterValue "/Game/06_Tech/UI/Material/UI_Material/MPC/MPC_HUD.MPC_HUD" "Camera_velocity" (Math|Color|MakeColor (.x (Variables|Default|GetSmooth_UI_Cam_Speeds)) (.y (Variables|Default|GetSmooth_UI_Cam_Speeds)) 0.0) :!class /Script/Engine.KismetMaterialLibrary))
    (:then_2
      (Variables|Default|SetPrevious_Rotation (Transformation|GetWorldRotation (Variables|/Script/RobotHunter.CustomCameraComponent|GetspringArm (Variables|Default|GetcameraComponent)))))))

(event EventOnSwitchPauseState
  (params (_state :type Boolean))
  (if _state
    (Audio|PlaySound2D "/Game/05_Audio/SFX/MetaSounds/UI/Pause_Menu/MSS_Activate_Pause_Menu.MSS_Activate_Pause_Menu" 1.0 1.0 0.0 0 0)
    (bind _returnvalue (Game|GetCurrentLevelName true))
    (if (Utilities|Enum|Equal(Enum) _returnvalue "P_Hub")
      (Audio|PushSoundMixModifier "/Game/05_Audio/SoundClass_Mixes/Pause_Menu/SCM_Hub_Pause_Menu1.SCM_Hub_Pause_Menu1")
      (Audio|PushSoundMixModifier "/Game/05_Audio/SoundClass_Mixes/Pause_Menu/SCM_Hub_Pause_Menu2.SCM_Hub_Pause_Menu2")
      (else
        (Audio|PushSoundMixModifier "/Game/05_Audio/SoundClass_Mixes/Pause_Menu/SCM_Game_Pause_Menu1.SCM_Game_Pause_Menu1")
        (Audio|PushSoundMixModifier "/Game/05_Audio/SoundClass_Mixes/Pause_Menu/SCM_Game_Pause_Menu2.SCM_Game_Pause_Menu2")))
    (else
      (Audio|PlaySound2D "/Game/05_Audio/SFX/MetaSounds/UI/Pause_Menu/MSS_Deactivate_Pause_Menu_v1.MSS_Deactivate_Pause_Menu_v1" 1.0 1.0 0.0 0 0)
      (bind _returnvalue_2 (Game|GetCurrentLevelName true))
      (if (Utilities|Enum|Equal(Enum) _returnvalue_2 "P_Hub")
        (Audio|PopSoundMixModifier "/Game/05_Audio/SoundClass_Mixes/Pause_Menu/SCM_Hub_Pause_Menu1.SCM_Hub_Pause_Menu1")
        (Audio|PopSoundMixModifier "/Game/05_Audio/SoundClass_Mixes/Pause_Menu/SCM_Hub_Pause_Menu2.SCM_Hub_Pause_Menu2")
        (else
          (Audio|PopSoundMixModifier "/Game/05_Audio/SoundClass_Mixes/Pause_Menu/SCM_Game_Pause_Menu1.SCM_Game_Pause_Menu1")
          (Audio|PopSoundMixModifier "/Game/05_Audio/SoundClass_Mixes/Pause_Menu/SCM_Game_Pause_Menu2.SCM_Game_Pause_Menu2"))))))

(event EventOnLanded
  (params (Hit :type Hit%20Result%20Structure%20%28by%20ref%29))
  ;[1 0.3512 0.4109] ABP Replication Test (A SUPPRIMER DES QUE LES VARIABLES EN C++ SONT RÉPLIQUÉES)
  ;;[1 1 1] On Landed
  (CallFunction|SonLanded))

(event EventBeginPlay
  (Utilities|FlowControl|Sequence
    (:then_0
      (EventDispatchers|BindEventtoOnScopeSound (delegate Custom|onScopeSound_Event))
      (Components|Timeline|SetPlayRate (Variables|Default|GetTL_Damage_Hit) (/ 1.0 (Variables|Default|GetDuree_Timeline)))
      (Components|Timeline|SetPlayRate (Variables|Default|GetTL_Heal) (/ 1.0 (Variables|Default|GetDuree_Timeline)))
      (EventDispatchers|AssignOnCalfInit (delegate Custom|onCalfInit_Event))
      (EventDispatchers|AssignOnShoot (Variables|Default|GetcameraComponent) (delegate Custom|onShoot_Event))
      (EventDispatchers|AssignOnScopeSound (delegate Custom|onScopeSound_Event_0))
      (EventDispatchers|BindEventtoOnBump (delegate Custom|OnBump_Event)))
    (:then_1
      (CallFunction|InitializeMaterials (Class|MainCharacter|GetUsingCalf)))))

(event Input|KeyboardEvents|B
  (params (Key :type Key%20Structure :default "None")))

(fn ConstructionScript
  (Utilities|FlowControl|Sequence))

(fn DebugLogBool
  (params (Bool :type Boolean)))

(fn HealthColortoVector4
  (params (BaseColorAnim :type Linear%20Color%20Structure) (HealthChangeValue :type Integer))
  (bind (_r _g _b _a) (Math|Color|BreakColor BaseColorAnim))
  (bind _returnvalue (Math|Integer|Absolute(Integer) HealthChangeValue))
  (bind _healthanim_maxcolorscale (Variables|Default|GetHealthAnim_MaxColorScale))
  (bind _returnvalue_2 (Math|Conversions|ToFloat(Integer) _returnvalue))
  (bind _returnvalue_3 (Math|Float|MapRangeClamped _returnvalue_2 0.0 1e+02 1.0 _healthanim_maxcolorscale))
  (return (Math|Vector4|MakeVector4 (* _r _returnvalue_3) (* _g _returnvalue_3) (* _b _returnvalue_3) (* _a _returnvalue_3))))

(fn IsPlayer1
  (if (Networking|IsServer)
    (bind _asplayer_controller (Utilities|Casting|CastToPlayerController (Pawn|GetController)))
    (if (== (Class|GameplayStatics|GetPlayerControllerID _asplayer_controller) 0)
      (return true)
      (else
        (return false)))
    (elif (Utilities|IsValid (Pawn|GetController))
      (return false)
      (else
        (return true)))))

(fn InitializeMaterials
  (params (Calf :type Calf%20Actor%20Object%20Reference))
  (LocalVariables|SetLegsMaterial (.Value (Utilities|Map|Find (Variables|Default|GetAllMaterialsLegs) (Utilities|GetClass Calf))))
  (for _array_element (Class|PrimitiveComponent|GetMaterialSlotNames (Variables|Character|GetMesh))
    (LocalVariables|SetCurrentMaterialIndex (Rendering|Material|GetMaterialIndex (Variables|Character|GetMesh) _array_element))
    (if (== _array_element "Body1")
      (bind _returnvalue (Rendering|Material|CreateDynamicMaterialInstance (select (CallFunction|IsPlayer1) "/Game/03_Graph/Character/Material/MI_Iqron_Body_P1.MI_Iqron_Body_P1" "/Game/03_Graph/Character/Material/MI_Iqron_Body_P2.MI_Iqron_Body_P2") "None" "None" :!class /Script/Engine.KismetMaterialLibrary))
      (bind _output_get (Variables|Default|SetMaterialBody _returnvalue))
      (Rendering|Material|SetMaterial (Variables|Character|GetMesh) (LocalVariables|GetCurrentMaterialIndex) _output_get)
      (elif (== _array_element "Arm1")
        (bind _returnvalue_2 (Rendering|Material|CreateDynamicMaterialInstance "/Game/03_Graph/Character/Material/MI_Iqron_Arm.MI_Iqron_Arm" "None" "None" :!class /Script/Engine.KismetMaterialLibrary))
        (bind _output_get_2 (Variables|Default|SetMaterialHand _returnvalue_2))
        (Rendering|Material|SetMaterial (Variables|Character|GetMesh) (LocalVariables|GetCurrentMaterialIndex) _output_get_2)
        (else
          (bind _returnvalue_3 (Rendering|Material|CreateDynamicMaterialInstance (LocalVariables|GetLegsMaterial) "None" "None" :!class /Script/Engine.KismetMaterialLibrary))
          (bind _output_get_3 (Variables|Default|SetMaterialLegs _returnvalue_3))
          (Rendering|Material|SetMaterial (Variables|Character|GetMesh) (LocalVariables|GetCurrentMaterialIndex) _output_get_3))))))