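; Rail actor that lays instanced rail meshes along a spline and lights them up when path rail detection fires.
; BakeRailsMeshes spaces instances evenly, optionally line-tracing to snap them to surfaces and align to normals.
; Per-instance custom data writes a repeating emissive offset along the rail.
; The construction script creates the dynamic material, whose "On rail" parameter detection events toggle; older construction-time placement and end-warning logic are disconnected.
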(event Custom|On%20path
  (Rendering|Material|SetScalarParameterValue (Variables|00---Generation|GetRail%20Material%20Reference) "On rail" 1.0 :!class /Script/Engine.MaterialInstanceDynamic))

(event Custom|Not%20on%20path
  (Rendering|Material|SetScalarParameterValue (Variables|00---Generation|GetRail%20Material%20Reference) "On rail" 0.0 :!class /Script/Engine.MaterialInstanceDynamic))

(event EventBeginPlay
  (EventDispatchers|BindEventtoOnPathRailDetected (delegate Custom|On%20path))
  (EventDispatchers|AssignRailNotDetectedAnymore (delegate Custom|Not%20on%20path)))

(event Collision|EventActorBeginOverlap
  (params (OtherActor :type Actor%20Object%20Reference)))

(event EventTick
  (params (DeltaSeconds :type Float%20%28single-precision%29)))

(fn ConstructionScript
  (bind _rails (Variables|Default|GetRails))
  (bind _returnvalue (Rendering|Material|CreateDynamicMaterialInstance _rails 0 "/Game/06_Tech/Train/Assets/Material/MI_trainCone.MI_trainCone" "None" :!class /Script/Engine.PrimitiveComponent))
  (bind _output_get (Variables|00---Generation|SetRail%20Material%20Reference _returnvalue))
  (Rendering|Material|SetMaterial _rails 0 _output_get))

(fn BakeRailsMeshes
  (bind _rails (Variables|Default|GetRails))
  (bind _spline (Variables|Default|GetSpline))
  (bind _rail_spacing (Variables|01---GraphParam|GetRail%20Spacing))
  (bind _spline_2 (Variables|Default|GetSpline))
  ;[0 1 0.11] Instanced static mesh component with custom data per instance method
  (Components|InstancedStaticMesh|ClearInstances (Variables|Default|GetRails))
  (for _index (range 0 (.ReturnValue (Math|Float|Division(WholeandRemainder) (Spline|GetSplineLength (Variables|Default|Getspline)) _rail_spacing)))
    (if (Variables|01---GraphParam|GetSnap_Rail)
      (bind (_outhit _returnvalue) (Collision|LineTraceForObjects (+ (Spline|GetLocationatDistanceAlongSpline _spline (* _index _rail_spacing) "World") "0.000000,0.000000,200.000000") (- (Spline|GetLocationatDistanceAlongSpline _spline (* _index _rail_spacing) "World") "0.000000,0.000000,700.000000") (Variables|Default|GetObject%20Types) false 0 "ForDuration"))
      (if _returnvalue
        (Utilities|Array|AddUnique (Variables|00---Generation|GetTransform%20rails) (Math|Transform|MakeTransform (.Location (Collision|BreakHitResult _outhit)) (Math|Rotator|MakeRotfromXZ (Spline|GetTangentatDistanceAlongSpline _spline (* _index _rail_spacing) "Local") (.Normal (Collision|BreakHitResult _outhit)))))
        (else
          (Utilities|Array|AddUnique (Variables|00---Generation|GetTransform%20rails) (Math|Transform|MakeTransform (Spline|GetLocationatDistanceAlongSpline _spline (* _index _rail_spacing) "World") (Math|Rotator|MakeRotfromX (Spline|GetTangentatDistanceAlongSpline _spline (* _index _rail_spacing) "Local"))))))
      (else
        (Utilities|Array|AddUnique (Variables|00---Generation|GetTransform%20rails) (Math|Transform|MakeTransform (Spline|GetLocationatDistanceAlongSpline _spline_2 (* _index _rail_spacing) "World") (Math|Rotator|MakeRotfromX (Spline|GetTangentatDistanceAlongSpline _spline_2 (* _index _rail_spacing) "Local")))))))
  (Variables|00---Generation|SetMeshCount (+ _index 1))
  (Components|StaticMesh|SetStaticMesh _rails (Variables|01---GraphParam|GetRail_Mesh))
  (Components|InstancedStaticMesh|SetCullDistances _rails 0 (Variables|01---GraphParam|GetEnd%20Cull%20Distance))
  (Components|InstancedStaticMesh|AddInstances _rails (Variables|00---Generation|GetTransform%20rails) false true true)
  (Class|InstancedStaticMeshComponent|SetNumCustomDataFloats _rails 1)
  (Variables|00---Generation|SetNewcount 0)
  (Variables|00---Generation|SetCurrentoffset 0.0)
  (for _index_2 (range 0 (Variables|00---Generation|GetMeshCount))
    (if (== (Math|Integer|%(Integer) _index_2 (Variables|Default|GetPeriod%20emissive)) 0)
      (Variables|00---Generation|SetNewcount 0)
      (Variables|00---Generation|SetCurrentoffset 0.0)
      (else
        (bind _result (Math|Integer|IncrementInt (Variables|00---Generation|GetNewcount))
          (:%20%20
            (Variables|00---Generation|SetCurrentoffset (- 1.0 (/ _result (Variables|Default|GetPeriod%20emissive))))))))
    (Components|InstancedStaticMesh|SetCustomDataValue _rails _index_2 0 (Variables|00---Generation|GetCurrentoffset) false)))