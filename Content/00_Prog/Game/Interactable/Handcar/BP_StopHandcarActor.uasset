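; Interactable handcar stop, with a gauntlet-exit variant that the construction script builds with a red emissive, disabled flare color and no platform.
; On interact, a timeline rolls the base by a set amount, the child scanner hand animates and the tutorial quest is validated.
; Handcar overlap plays or reverses an emissive fade through a material parameter collection.
; Handcar stop events spawn Niagara effects at platform sockets, gated by a delay-reset flag.
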(event Custom|onInteract_Event
  (params (_character :type Main%20Character%20Object%20Reference))
  (bind _questmanager (Variables|Default|GetQuestManager))
  ;[1 1 1] Animation
  (Utilities|FlowControl|Sequence
    (:then_0
      ;;[1 1 1] Base Rotation
      (Variables|Default|SetBase_PreviousAngle (.roll (Variables|/Script/Engine.SceneComponent|GetRelativeRotation (Variables|Default|GetBase))))
      (bind _rotate_alpha (Timeline|TL_AnimateBase PlayFromStart)
        (:Update
          _)
        (:Finished
          _))
      (Transformation|SetRelativeRotation (Variables|Default|GetBase) (Math|Rotator|MakeRotator (+ (Variables|Default|GetBase_PreviousAngle) (* (Variables|Default|GetBase_RotationAmount) _rotate_alpha)) 0.0 0.0) false false)
      (Variables|Default|GetQuestManager
        (:then
          (if (Utilities|IsValidSoftObjectReference _questmanager)
            (Class|QuestManager|ValidQuest (Utilities|ResolveSoftReference _questmanager) "/Game/00_Prog/Game/Quest/Tuto/TutoQuest_02.TutoQuest_02")))
        (:else)))
    (:then_1
      ;;[1 1 1] Handle rotation
      (bind _asbp_scanner_mesh (Utilities|Casting|CastToBP_ScannerMesh (Variables|/Script/Engine.ChildActorComponent|GetChildActor (Variables|Default|GetHand))))
      (Default|PlayAnimation _asbp_scanner_mesh))))

(event Custom|onHandcarStop_Event
  (params (isStopped :type Boolean))
  (bind _platform (Variables|Default|GetPlatform))
  (if (and (Variables|Default|GetSpawn_Vap) (Utilities|IsValid _platform))
    (Variables|Default|SetSpawn_Vap false)
    (for _array_element (Transformation|GetAllSocketNames _platform)
      (Niagara|SpawnSystematLocation "/Game/04_FX/NS/Draisine/NS_HandCarOverlap.NS_HandCarOverlap" (Transformation|GetSocketLocation _platform _array_element))
      (Utilities|FlowControl|Delay 2.0)
      (Variables|Default|SetSpawn_Vap true))))

(event Custom|onHandcarOverlap_Event
  (params (isOverlapping :type Boolean))
  (if isOverlapping
    (bind _slide_emissive (Timeline|Timeline Play)
      (:Update
        (Rendering|Material|SetScalarParameterValue "/Game/06_Tech/Materials/MPC/MPC_Interraction.MPC_Interraction" "HandCar_Overlap" _slide_emissive :!class /Script/Engine.KismetMaterialLibrary)))
    (else
      (Timeline|Timeline Reverse))))

(event EventBeginPlay
  (CallFunction|UpdateWidgetPosition)
  (EventDispatchers|AssignOnInteract (delegate Custom|onInteract_Event))
  (EventDispatchers|AssignOnHandcarStop (delegate Custom|onHandcarStop_Event))
  (EventDispatchers|AssignOnHandcarOverlap (delegate Custom|onHandcarOverlap_Event)))

(event Collision|EventActorBeginOverlap
  (params (OtherActor :type Actor%20Object%20Reference)))

(fn ConstructionScript
  (bind _is_gauntlet_exit_ (Variables|State|GetIs_Gauntlet_Exit?))
  (Utilities|FlowControl|Sequence
    (:then_0
      (Rendering|Material|SetMaterial (Variables|Default|GetEmissive) 0 (select _is_gauntlet_exit_ "/Game/03_Graph/Assets/Materials/MI_Emissive_Antenna_red.MI_Emissive_Antenna_red" "/Game/03_Graph/Assets/Materials/MI_Emissive_Antenna_blue.MI_Emissive_Antenna_blue")))
    (:then_1
      (if _is_gauntlet_exit_
        (Components|DestroyComponent (Variables|Default|GetPlatform))
        (Components|DestroyComponent (Variables|Default|Getplatform_emmisive))
        (Niagara|SetNiagaraVariable(LinearColor) (Variables|Default|GetNS_Flare) "Lens_Color" (Variables|Default|GetDiseable_Color))
        (else
          (Niagara|SetNiagaraVariable(LinearColor) (Variables|Default|GetNS_Flare) "Lens_Color" (Variables|Default|GetEnable_Color)))))))

(fn UpdateWidgetPosition
  (bind _buttonmesh (Variables|Default|GetbuttonMesh))
  (bind _widgetoffset (Variables|Default|GetWidgetOffset))
  (bind (_x _y _z) (Math|Vector|BreakVector _widgetoffset))
  (Transformation|SetWorldLocationAndRotation (Variables|Default|GetinteractionFeedback) (+ (Transformation|GetWorldLocation (Variables|Default|GetbuttonMesh)) (* (Math|Vector|GetForwardVector _buttonmesh) _x) (* (Math|Vector|GetRightVector _buttonmesh) _y) (Math|Vector|MakeVector 0.0 0.0 _z)) (Transformation|GetWorldRotation (Variables|Default|GetbuttonMesh)) false true))