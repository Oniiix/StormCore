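; BP_BrakeHandcarActor is the brake actor for the handcar, animating the brake mesh when the brake is released or re-engaged.
; The Released event plays or reverses a timeline that lerps the mesh's relative Z down from InitZOffset by BrakeHeightOffset.
; The nodes that capture InitZOffset and bind Released to OnReleaseBrake are disconnected, so this graph never runs that setup.
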(event Custom|Released
  (params (isReleased :type Boolean))
  (bind _init_z_offset (Variables|Default|GetInit_Z_Offset))
  (if isReleased
    (bind _brake_lerp (Timeline|Timeline Play)
      (:Update
        (Transformation|SetRelativeLocation (Variables|Default|GetBrake_mesh) (Math|Vector|MakeVector 0.0 0.0 (Math|Float|Lerp _init_z_offset (- _init_z_offset (Variables|Default|GetBrake_Height_Offset)) _brake_lerp)) false false)))
    (else
      (Timeline|Timeline Reverse))))

(event EventBeginPlay)

(event Collision|EventActorBeginOverlap
  (params (OtherActor :type Actor%20Object%20Reference)))

(event EventTick
  (params (DeltaSeconds :type Float%20%28single-precision%29)))

(fn ConstructionScript)