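; PlantLootActor_BP is an interactable plant loot actor that reacts visually when a character gathers it.
; On BeginPlay it binds a handler to its interact event.
; On interact, it spawns a Niagara gather burst at a locator component, destroys its point light and flower, and deactivates the ambient plant particle system without resetting it.
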(event Custom|CustomEvent
  (params (_character :type Main%20Character%20Object%20Reference))
  (Niagara|SpawnSystematLocation "/Game/04_FX/NS/NS_Dynamics_Plants/NS_LifePlant_gather.NS_LifePlant_gather" (Transformation|GetWorldLocation (Variables|Default|GetNiagara_Locator)))
  (Components|DestroyComponent (Variables|Default|GetPointLight))
  (Components|DestroyComponent (Variables|Default|Getlife_flower))
  (Components|Activation|SetActive (Variables|Default|GetNS_Life_Plant) false false))

(event EventBeginPlay
  (EventDispatchers|BindEventtoOnInteract (delegate Custom|CustomEvent)))

(event Collision|EventActorBeginOverlap
  (params (OtherActor :type Actor%20Object%20Reference)))

(event EventTick
  (params (DeltaSeconds :type Float%20%28single-precision%29)))

(fn ConstructionScript)