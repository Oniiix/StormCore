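; Hub radio actor that plays the daily broadcast with subtitles when OnLightOnRadio fires with the current weather and day.
; It fades out looping interference, then chains day intro, weather report and day outro, timing each step by MetaSound-to-wave durations.
; Afterward it restores the interference and sends the full transcript to the radio widget.
; The same event completes the listen-to-radio quest, adds HeadOut and makes StartActor detectable.
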(event Custom|onLightOnRadio_Event
  (params (_currentweather :type Weather%20Class%20Reference) (_day :type Integer))
  (bind _questmanager (Variables|Default|GetQuestManager))
  (bind _output (Utilities|ResolveSoftReference _questmanager))
  ;[0.301 0.301 0.301 0.348] Systeme Dynamique
  (Utilities|FlowControl|Sequence
    (:then_0
      ;;[1 1 1] SETUP
      (Audio|Components|Audio|FadeOut (Variables|Default|GetRadio%20Interference%20SFX) 0.1 0.0 "Linear" :!class /Script/Engine.AudioComponent)
      ;;;[1 1 1] Enum Météo
      (Variables|Default|SetMeteo (CallFunction|GetCurrentWeather _currentweather))
      ;;;[1 1 1] Index jour (de 0 à 2)
      (bind _output_get (Variables|Default|SetJour _day))
      (Math|Integer|DecrementInt _output_get))
    (:then_1
      (Utilities|FlowControl|DelayUntilNextTick)
      ;;[1 1 1] Global Intro
      (switch int (Variables|Default|GetJour)
        (:0
          (bind _duree (CallFunction|PlaySound "/Game/05_Audio/VO/Radio_Messages/Mono/MSS_Radio_Message_Global_Intro_Day1_Mono.MSS_Radio_Message_Global_Intro_Day1_Mono" 0.0)) ; Day 1
          (Class|RadioActor|PlaySubtitles "/Game/05_Audio/VO/Radio_Messages/Subtitles/REWORK/Lines/DT_Subs_GlobalIntro_D1.DT_Subs_GlobalIntro_D1")
          (Utilities|FlowControl|Delay _duree))
        (:1
          _)
        (:2
          (bind _duree_2 (CallFunction|PlaySound "/Game/05_Audio/VO/Radio_Messages/Mono/MSS_Radio_Message_Global_Intro_Day3_Mono.MSS_Radio_Message_Global_Intro_Day3_Mono" 0.0)) ; Day 3
          (Class|RadioActor|PlaySubtitles "/Game/05_Audio/VO/Radio_Messages/Subtitles/REWORK/Lines/DT_Subs_GlobalIntro_D3.DT_Subs_GlobalIntro_D3")
          (Utilities|FlowControl|Delay _duree_2)))
      ;;[1 1 1] Meteo Intro
      (bind _duree_3 (CallFunction|PlaySound "/Game/05_Audio/VO/Radio_Messages/Mono/MSS_Radio_Message_Meteo_Part_Intro_Mono.MSS_Radio_Message_Meteo_Part_Intro_Mono" 0.0))
      (Class|RadioActor|PlaySubtitles "/Game/05_Audio/VO/Radio_Messages/Subtitles/REWORK/Lines/DT_Subs_MeteoIntro.DT_Subs_MeteoIntro")
      (Utilities|FlowControl|Delay _duree_3)
      ;;[1 1 1] Meteo
      (bind _duree_4 (CallFunction|PlaySound (Utilities|Select :Index (Variables|Default|GetMeteo) :NewEnumerator0 "/Game/05_Audio/VO/Radio_Messages/Mono/MSS_Radio_Message_Meteo_Frost_Mono.MSS_Radio_Message_Meteo_Frost_Mono" :NewEnumerator1 "/Game/05_Audio/VO/Radio_Messages/Mono/MSS_Radio_Message_Meteo_WetStorm_Mono.MSS_Radio_Message_Meteo_WetStorm_Mono" :NewEnumerator2 "/Game/05_Audio/VO/Radio_Messages/Mono/MSS_Radio_Message_Meteo_DryStorm_Mono.MSS_Radio_Message_Meteo_DryStorm_Mono" :NewEnumerator3 "/Game/05_Audio/VO/Radio_Messages/Mono/MSS_Radio_Message_Meteo_Mist_Mono.MSS_Radio_Message_Meteo_Mist_Mono" :NewEnumerator4 "/Game/05_Audio/VO/Radio_Messages/Mono/MSS_Radio_Message_Meteo_Hurricane_Mono.MSS_Radio_Message_Meteo_Hurricane_Mono" :NewEnumerator5 "/Game/05_Audio/VO/Radio_Messages/Mono/MSS_Radio_Message_Meteo_ClearSky_Mono.MSS_Radio_Message_Meteo_ClearSky_Mono" :NewEnumerator6 "/Game/05_Audio/VO/Radio_Messages/Mono/MSS_Radio_Message_Meteo_RedStorm_Mono.MSS_Radio_Message_Meteo_RedStorm_Mono") (Utilities|Select :Index (Variables|Default|GetMeteo) :NewEnumerator0 0.0 :NewEnumerator1 0.0 :NewEnumerator2 0.0 :NewEnumerator3 0.0 :NewEnumerator4 0.0 :NewEnumerator5 0.0 :NewEnumerator6 0.0)))
      (Class|RadioActor|PlaySubtitles (Utilities|Select :Index (Variables|Default|GetMeteo) :NewEnumerator0 "/Game/05_Audio/VO/Radio_Messages/Subtitles/REWORK/Lines/DT_Subs_Meteo_Frost.DT_Subs_Meteo_Frost" :NewEnumerator1 "/Game/05_Audio/VO/Radio_Messages/Subtitles/REWORK/Lines/DT_Subs_Meteo_WetStorm.DT_Subs_Meteo_WetStorm" :NewEnumerator2 "/Game/05_Audio/VO/Radio_Messages/Subtitles/REWORK/Lines/DT_Subs_Meteo_DryStorm.DT_Subs_Meteo_DryStorm" :NewEnumerator3 "/Game/05_Audio/VO/Radio_Messages/Subtitles/REWORK/Lines/DT_Subs_Meteo_Mist.DT_Subs_Meteo_Mist" :NewEnumerator4 "/Game/05_Audio/VO/Radio_Messages/Subtitles/REWORK/Lines/DT_Subs_Meteo_Hurricane.DT_Subs_Meteo_Hurricane" :NewEnumerator5 "/Game/05_Audio/VO/Radio_Messages/Subtitles/REWORK/Lines/DT_Subs_Meteo_ClearSky.DT_Subs_Meteo_ClearSky" :NewEnumerator6 "/Game/05_Audio/VO/Radio_Messages/Subtitles/REWORK/Lines/DT_Subs_Meteo_RedStorm.DT_Subs_Meteo_RedStorm"))
      (Utilities|FlowControl|Delay _duree_4)
      ;;[1 1 1] Outro
      (bind _duree_5 (CallFunction|PlaySound (Utilities|Select :Index (Variables|Default|GetJour) :Option%200 "/Game/05_Audio/VO/Radio_Messages/Mono/MSS_Radio_Message_Outro_Day1_Mono.MSS_Radio_Message_Outro_Day1_Mono" :Option%201 "/Game/05_Audio/VO/Radio_Messages/Mono/MSS_Radio_Message_Outro_Day2_Mono.MSS_Radio_Message_Outro_Day2_Mono" :Option%202 "/Game/05_Audio/VO/Radio_Messages/Mono/MSS_Radio_Message_Outro_Day3_Mono.MSS_Radio_Message_Outro_Day3_Mono") (Utilities|Select :Index (Variables|Default|GetJour) :Option%200 0.0 :Option%201 0.0 :Option%202 0.0)))
      (Class|RadioActor|PlaySubtitles (Utilities|Select :Index (Variables|Default|GetJour) :Option%200 "/Game/05_Audio/VO/Radio_Messages/Subtitles/REWORK/Lines/DT_Subs_Outro_D1.DT_Subs_Outro_D1" :Option%201 "/Game/05_Audio/VO/Radio_Messages/Subtitles/REWORK/Lines/DT_Subs_Outro_D2.DT_Subs_Outro_D2" :Option%202 "/Game/05_Audio/VO/Radio_Messages/Subtitles/REWORK/Lines/DT_Subs_Outro_D3.DT_Subs_Outro_D3"))
      (Utilities|FlowControl|Delay _duree_5)
      ;;[1 1 1] END
      (Audio|Components|Audio|FadeIn (Variables|Default|GetRadio%20Interference%20SFX) 2.0 0.3825 0.0 "Linear" :!class /Script/Engine.AudioComponent)
      (CallFunction|UpdateTranscript (Text||Transcript|GetFullTranscript) true)
      (bind _subtitles_widget (Variables|Default|GetSubtitles_Widget)
        (:then
          (Widget|RemovefromParent _subtitles_widget))
        (:else)))
    (:then_2
      ;;[1 1 1] QUEST
      (bind _returnvalue (Class|QuestManager|ValidQuest _output "/Game/00_Prog/Game/Quest/Quest_ListenToRadio.Quest_ListenToRadio"))
      (if _returnvalue
        (bind _returnvalue_2 (Class|QuestManager|CheckCompleteQuest _output (Variables|/Script/RobotHunter.QuestAsset|GetId (Variables|Default|GetStockQuestAsset))))
        (if _returnvalue_2
          (Class|QuestManager|AddQuest _output "/Game/00_Prog/Game/Quest/Quest_HeadOut.Quest_HeadOut")
          (Variables|/Script/RobotHunter.InteractableActor|SetcanBeDetected (Variables|Default|GetStartActor) true))))))

(event Custom|onInteract_Event
  (params (_character :type Main%20Character%20Object%20Reference))
  ;[1 1 1] Test
  (CallFunction|OnLightonRadioEvent (.OutItem (Utilities|Array|Random (Utilities|Array|MakeArray "/Game/00_Prog/Game/GPE/Weather/BP_BlueSkyWeather.BP_BlueSkyWeather_C" "/Game/00_Prog/Game/GPE/Weather/BP_DryStormWeather.BP_DryStormWeather_C" "/Game/00_Prog/Game/GPE/Weather/BP_FrostWeather.BP_FrostWeather_C" "/Game/00_Prog/Game/GPE/Weather/BP_MistWeather.BP_MistWeather_C" "/Game/00_Prog/Game/GPE/Weather/BP_RedStormWeather.BP_RedStormWeather_C" "/Game/00_Prog/Game/GPE/Weather/BP_WetStormWeather.BP_WetStormWeather_C" "/Game/00_Prog/Game/GPE/Weather/BP_WindWeather.BP_WindWeather_C"))) (Math|Random|RandomIntegerinRange 0 2)))

(event EventBeginPlay
  (bind _returnvalue (Audio|SpawnSoundatLocation "/Game/05_Audio/Amb_SFX/Props/Hub/Radio/MSS_Radio_SFX.MSS_Radio_SFX" "1887.096649,17387.716069,94.674235" "0, 0, 0" 1.0 1.0 0.0 0 0 false))
  (Variables|Default|SetRadio%20Interference%20SFX _returnvalue)
  (EventDispatchers|AssignOnLightonRadio (delegate Custom|onLightOnRadio_Event)))

(fn ConstructionScript)

(fn GetCurrentWeather
  (params (WeatherClass :type Weather%20Class%20Reference))
  (if (== WeatherClass "/Game/00_Prog/Game/GPE/Weather/BP_FrostWeather.BP_FrostWeather_C")
    (return "NewEnumerator0")
    (elif (== WeatherClass "/Game/00_Prog/Game/GPE/Weather/BP_WetStormWeather.BP_WetStormWeather_C")
      (return "NewEnumerator1")
      (elif (== WeatherClass "/Game/00_Prog/Game/GPE/Weather/BP_DryStormWeather.BP_DryStormWeather_C")
        (return "NewEnumerator2")
        (elif (== WeatherClass "/Game/00_Prog/Game/GPE/Weather/BP_MistWeather.BP_MistWeather_C")
          (return "NewEnumerator3")
          (elif (== WeatherClass "/Game/00_Prog/Game/GPE/Weather/BP_WindWeather.BP_WindWeather_C")
            (return "NewEnumerator4")
            (elif (== WeatherClass "/Game/00_Prog/Game/GPE/Weather/BP_BlueSkyWeather.BP_BlueSkyWeather_C")
              (return "NewEnumerator5")
              (else
                (return "NewEnumerator6")))))))))

(fn PlaySound
  (params (SFX :type Sound%20Base%20Object%20Reference) (DelaiOffset :type Float%20%28double-precision%29))
  (Utilities|FlowControl|Sequence
    (:then_0
      (Audio|PlaySound2D SFX 1.0 1.0 0.0 0 0))
    (:then_1
      (return (+ (Variables|/Script/Engine.SoundBase|GetDuration (.Value (Utilities|Map|Find (LocalVariables|GetMetasoundToWave) SFX))) DelaiOffset)))))

(fn GetFullTranscript
  (return (Utilities|Text|FormatText "{Global_Intro} 
 
{Meteo_Intro} 
 
{Meteo} 
 
{Outro}" (Text||Transcript|GetGlobalIntroTranscript) (Text||Transcript|GetMeteoIntroTranscript) (Text||Transcript|GetMeteoTranscript) (Text||Transcript|GetOutroTranscript))))

(fn GetGlobalIntroTranscript
  (if (or (== (Variables|Default|GetJour) 0) (== (Variables|Default|GetJour) 2))
    (return (Text|ConcatenateLines (Text||Lines|GetGlobalIntroLines)))
    (else
      (return ""))))

(fn GetMeteoIntroTranscript
  (return (Text|ConcatenateLines (Text||Lines|GetMeteoIntroLines))))

(fn GetMeteoTranscript
  (return (Text|ConcatenateLines (Text||Lines|GetMeteoLines))))

(fn GetOutroTranscript
  (return (Text|ConcatenateLines (Text||Lines|GetOutroLines))))

(fn UpdateTranscript
  (params (Updated_Text :type Text) (FinalTransmission? :type Boolean))
  (bind _asbp_radio_floating (Utilities|Casting|CastToBp_RadioFloating (Variables|Default|GetRadioWidget)))
  (Default|EndTransmission _asbp_radio_floating Updated_Text FinalTransmission?))

(fn ConcatenateLines
  (params (InLines :type Array%20of%20Texts))
  (for _array_element InLines
    (LocalVariables|SetFinalLine (Utilities|Text|FormatText "{full line} 
{new line}" (LocalVariables|GetFinalLine) _array_element)))
  (return (LocalVariables|GetFinalLine)))

(fn GetAllLines
  (Utilities|FlowControl|Sequence
    (:then_0
      (LocalVariables|SetAllLines (Text||Lines|GetGlobalIntroLines)))
    (:then_1
      (Utilities|Array|Add (LocalVariables|GetAllLines) (Text||Transcript|GetMeteoIntroTranscript)))
    (:then_2
      (Utilities|Array|AppendArray (LocalVariables|GetAllLines) (Text||Lines|GetMeteoLines)))
    (:then_3
      (Utilities|Array|AppendArray (LocalVariables|GetAllLines) (Text||Lines|GetOutroLines)))
    (:then_4
      (return (LocalVariables|GetAllLines)))))

(fn GetGlobalIntroLines
  (switch int (Variables|Default|GetJour)
    (:Default
      _)
    (:0
      (return (Utilities|Array|MakeArray "Global_Intro_Day1_00" "Global_Intro_Day1_01" "Global_Intro_Day1_02" "Global_Intro_Day1_03" "Global_Intro_Day1_04" "Global_Intro_Day1_05" "Global_Intro_Day1_06")))
    (:1
      _)
    (:2
      (return (Utilities|Array|MakeArray "Global_Intro_Day3_00" "Global_Intro_Day3_01" "Global_Intro_Day3_02" "Global_Intro_Day3_03"))))
  (return 0))

(fn GetMeteoIntroLines
  (return (Utilities|Array|MakeArray "Meteo_Intro_00")))

(fn GetMeteoLines
  (switch Utilities|FlowControl|Switch|SwitchonEnum_weatherType (Variables|Default|GetMeteo)
    (:NewEnumerator0
      (return (Utilities|Array|MakeArray "Meteo_Frost_00" "Meteo_Frost_01" "Meteo_Frost_02")))
    (:NewEnumerator1
      (return (Utilities|Array|MakeArray "Meteo_Storm_00" "Meteo_Storm_01" "Meteo_Storm_02")))
    (:NewEnumerator2
      (return (Utilities|Array|MakeArray "Meteo_DryStorm_00" "Meteo_DryStorm_01" "Meteo_DryStorm_02")))
    (:NewEnumerator3
      (return (Utilities|Array|MakeArray "Meteo_Mist_00" "Meteo_Mist_01" "Meteo_Mist_02")))
    (:NewEnumerator4
      (return (Utilities|Array|MakeArray "Meteo_Hurricane_00" "Meteo_Hurricane_01" "Meteo_Hurricane_02")))
    (:NewEnumerator5
      (return (Utilities|Array|MakeArray "Meteo_ClearSky_00" "Meteo_ClearSky_01" "Meteo_ClearSky_02")))
    (:NewEnumerator6
      (return (Utilities|Array|MakeArray "Meteo_RedStorm_00" "Meteo_RedStorm_01" "Meteo_RedStorm_02")))))

(fn GetOutroLines
  (switch int (Variables|Default|GetJour)
    (:Default
      (return 0))
    (:0
      (return (Utilities|Array|MakeArray "Outro_Day1_00" "Outro_Day1_01")))
    (:1
      (return (Utilities|Array|MakeArray "Outro_Day2_00" "Outro_Day2_01")))
    (:2
      (return (Utilities|Array|MakeArray "Outro_Day3_00" "Outro_Day3_01")))))