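; Hub interactable for the weapon stock that handles its UI sounds and advances the hub's quest flow.
; On interact, it plays a delayed activation sound and binds to the character's menu-quit event, which plays the deactivation sound and unbinds.
; Interacting also validates the equip-self quest through the QuestManager; if that succeeds and the radio quest is complete, it adds the head-out quest and makes the StartActor detectable.
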(event Custom|On%20Interact%20%28Weapon%20Stock%29
  (params (_character :type Main%20Character%20Object%20Reference))
  (bind _questmanager (Variables|Default|GetQuestManager))
  (bind _output (Utilities|ResolveSoftReference _questmanager))
  ;[1 1 1] UI SFX
  (Utilities|FlowControl|Sequence
    (:then_0
      (Utilities|FlowControl|Delay 0.15)
      (Audio|PlaySound2D "/Game/05_Audio/SFX/MetaSounds/UI/Weapon_Stock_Activate/MSS_Weapon_Stock_Activate_v1.MSS_Weapon_Stock_Activate_v1" 1.0 1.0 0.0 0 0))
    (:then_1
      (EventDispatchers|BindEventtoOnQuitMenu _character (delegate Custom|On%20Quit%20%28Weapon%20Stock%29)))
    (:then_2
      (bind _returnvalue (Class|QuestManager|ValidQuest _output "/Game/00_Prog/Game/Quest/Quest_EquipSelf.Quest_EquipSelf"))
      (if _returnvalue
        (bind _returnvalue_2 (Class|QuestManager|CheckCompleteQuest _output (Variables|/Script/RobotHunter.QuestAsset|GetId (Variables|Default|GetRadioQuestAsset))))
        (if _returnvalue_2
          (Class|QuestManager|AddQuest _output "/Game/00_Prog/Game/Quest/Quest_HeadOut.Quest_HeadOut")
          (Variables|/Script/RobotHunter.InteractableActor|SetcanBeDetected (Variables|Default|GetStartActor) true))))))

(event Custom|On%20Quit%20%28Weapon%20Stock%29
  ;[1 1 1] UI SFX
  (Audio|PlaySound2D "/Game/05_Audio/SFX/MetaSounds/UI/Weapon_Stock_Deactivate/MSS_Weapon_Stock_Deactivate_v1.MSS_Weapon_Stock_Deactivate_v1" 1.0 1.0 0.0 0 0)
  (EventDispatchers|UnbindEventfromOnQuitMenu (stale Custom|On%20Interact%20%28Weapon%20Stock%29 _character) (delegate Custom|On%20Quit%20%28Weapon%20Stock%29)))

(event EventBeginPlay
  (EventDispatchers|BindEventtoOnInteract (delegate Custom|On%20Interact%20%28Weapon%20Stock%29)))

(event Collision|EventActorBeginOverlap
  (params (OtherActor :type Actor%20Object%20Reference)))

(event EventTick
  (params (DeltaSeconds :type Float%20%28single-precision%29)))

(fn ConstructionScript)