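; Hub interactable with a crystal that completes the Head Out quest and plays an activation animation when a character interacts with it.
; Shortly after BeginPlay, it disables detection if it is day 1, the tutorial has started and quests are ongoing.
; On interact, delayed grab and activate sounds run alongside a timeline that rotates the crystal, then reverses it to rest after a short pause.
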(event Custom|onInteract_Event
  (params (_character :type Main%20Character%20Object%20Reference))
  (bind _crystal (Variables|Default|GetCrystal))
  (bind _returnvalue (Transformation|GetWorldLocation _crystal))
  (Utilities|FlowControl|Sequence
    (:then_0
      (Class|QuestManager|ValidQuest (Utilities|ResolveSoftReference (Variables|Default|GetQuestManager)) "/Game/00_Prog/Game/Quest/Quest_HeadOut.Quest_HeadOut")
      (Utilities|FlowControl|Delay 1.4)
      (bind (_direction _rotation) (Timeline|Timeline Play)
        (:Update
          (Transformation|SetRelativeRotation (Variables|Default|GetCrystal) (Math|Rotator|Lerp(Rotator) "0, 0, 0" "0.000000,-90.000000,0.000000" _rotation) false false))
        (:Finished
          (Utilities|FlowControl|Delay 0.5)
          (switch Utilities|FlowControl|Switch|SwitchonETimelineDirection _direction
            (:Forward
              (CallFunction|Reset))))))
    (:then_1
      (Utilities|FlowControl|Delay 0.5)
      (Audio|PlaySoundatLocation "/Game/05_Audio/SFX/MetaSounds/GPE/Start_Interactable/MSS_Start_Interactable_Stage1_Grab.MSS_Start_Interactable_Stage1_Grab" _returnvalue "0, 0, 0" 1.0 1.0 0.0 0 0 0 0)
      (Utilities|FlowControl|Delay 1.3)
      (Audio|PlaySoundatLocation "/Game/05_Audio/SFX/MetaSounds/GPE/Start_Interactable/MSS_Start_Interactable_Stage2_Activate.MSS_Start_Interactable_Stage2_Activate" _returnvalue "0, 0, 0" 1.0 1.0 0.0 0 0 0 0))))

(event Custom|Reset
  (bind (_direction _rotation) (Timeline|Timeline Reverse)
    (:Update
      (Transformation|SetRelativeRotation (Variables|Default|GetCrystal) (Math|Rotator|Lerp(Rotator) "0, 0, 0" "0.000000,-90.000000,0.000000" _rotation) false false))
    (:Finished
      (Utilities|FlowControl|Delay 0.5)
      (switch Utilities|FlowControl|Switch|SwitchonETimelineDirection _direction
        (:Forward
          (CallFunction|Reset))))))

(event EventBeginPlay
  (bind _returnvalue (Subsystems|GetSaveManagerSubsystem))
  (bind _returnvalue_2 (Class|SaveManagerSubsystem|GetCurrentSave _returnvalue))
  (EventDispatchers|BindEventtoOnInteract (delegate Custom|onInteract_Event))
  (Utilities|FlowControl|Delay 0.2)
  (Variables|Default|SetcanBeDetected (not (Math|Boolean|ANDBoolean (== (.day (Variables|/Script/RobotHunter.GameplaySave|GetgameSave _returnvalue_2)) 1) (.hasstarttuto (Variables|/Script/RobotHunter.GameplaySave|GettutoSave _returnvalue_2)) (> (Utilities|Array|Length (Class|QuestManager|GetonGoingQuests (Utilities|ResolveSoftReference (Variables|Default|GetQuestManager)))) 0)))))

(fn ConstructionScript)