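; Modular drawbridge that deploys from both ends when its bound action event fires, with drawbridge sounds.
; The construction script spawns mid, plate and barrier meshes into per-side arrays by Subdivision count and offsets the Ending component to match the length.
; Three chained timelines reveal and animate them: mid modules extend lengthwise, plates slide out sideways, then barriers rotate into place and gain collision.
; The deploy event ignores IsActive, so no retraction exists.
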(event Custom|OnDeployement
  (params (_isActive :type Boolean))
  (Utilities|FlowControl|Sequence
    (:then_0
      (bind _linear (Timeline|Timeline Play)
        (:Update
          (Utilities|FlowControl|Sequence
            (:then_0
              ;[1 0.04999 0] Mid_Section
              (for (_array_element _array_index) (Variables|Begin_Meshes_Array|GetBegin_mid_modules)
                (Rendering|SetVisibility _array_element true false)
                (Transformation|SetRelativeLocation _array_element (Math|Vector|MakeVector (* (+ _array_index 1) (Math|Float|Lerp 0.0 4e+02 _linear)) 0.0 0.0) false false)))
            (:then_1
              ;[1 0.04999 0] Mid_Section
              (for (_array_element_2 _array_index_2) (Variables|Ending_Meshes_Array|GetEnding_Mid_Modules)
                (Rendering|SetVisibility _array_element_2 true false)
                (Transformation|SetRelativeLocation _array_element_2 (+ (Variables|Default|GetEnd_Offset) (Math|Vector|MakeVector (* (+ _array_index_2 1) (Math|Float|Lerp 0.0 -4e+02 _linear)) 0.0 0.0)) false false)))))
        (:Finished
          (bind _x_offset (Timeline|Timeline_0 PlayFromStart)
            (:Update
              ;[0 0.761 1] Left_plateform
              (Utilities|FlowControl|Sequence
                (:then_0
                  (for (_array_element_3 _array_index_3) (Variables|BeginMeshesArray|GetBegin_Left_Plates)
                    (Rendering|SetVisibility _array_element_3 true false)
                    (Transformation|SetRelativeLocation _array_element_3 (Math|Vector|MakeVector (* (+ _array_index_3 1) 4e+02) (Math|Float|Lerp 0.0 (Variables|Default|GetEnd_Plateform_offset) _x_offset) 0.0) false false)
                    (Transformation|SetRelativeRotation _array_element_3 "0.000000,-90.000000,0.000000" false false)))
                (:then_1
                  (for (_array_element_4 _array_index_4) (Variables|BeginMeshesArray|Getbegin_Right_Plates)
                    (Rendering|SetVisibility _array_element_4 true false)
                    (Transformation|SetRelativeLocation _array_element_4 (Math|Vector|MakeVector (* (+ _array_index_4 1) 4e+02) (Math|Float|Lerp 0.0 (* (Variables|Default|GetEnd_Plateform_offset) -1.0) _x_offset) 0.0) false false)
                    (Transformation|SetRelativeRotation _array_element_4 "0.000000,90.000000,0.000000" false false)))
                (:then_2
                  ;[0 0.761 1] End_Left_plateform
                  (for (_array_element_5 _array_index_5) (Variables|EndingMeshesArray|GetEnding_Left_Plates)
                    (Rendering|SetVisibility _array_element_5 true false)
                    (Transformation|SetRelativeLocation _array_element_5 (+ (Variables|Default|GetEnd_Offset) (Math|Vector|MakeVector (* (+ _array_index_5 1) -4e+02) (Math|Float|Lerp 0.0 (Variables|Default|GetEnd_Plateform_offset) _x_offset) 0.0)) false false)
                    (Transformation|SetRelativeRotation _array_element_5 "0.000000,-90.000000,0.000000" false false)))
                (:then_3
                  (for (_array_element_6 _array_index_6) (Variables|EndingMeshesArray|GetEnding_Right_Plates)
                    (Rendering|SetVisibility _array_element_6 true false)
                    (Transformation|SetRelativeLocation _array_element_6 (+ (Variables|Default|GetEnd_Offset) (Math|Vector|MakeVector (* (+ _array_index_6 1) -4e+02) (Math|Float|Lerp 0.0 (* (Variables|Default|GetEnd_Plateform_offset) -1.0) _x_offset) 0.0)) false false)
                    (Transformation|SetRelativeRotation _array_element_6 "0.000000,90.000000,0.000000" false false)))))
            (:Finished
              ;[1 0.1755 0] Barrier
              (bind _newtrack_0 (Timeline|Timeline_1 PlayFromStart)
                (:Update
                  (Utilities|FlowControl|Sequence
                    (:then_0
                      (for (_array_element_7 _array_index_7) (Variables|BeginMeshesArray|GetBegin_Left_Barrier)
                        (Rendering|SetVisibility _array_element_7 true false)
                        (Transformation|SetRelativeLocation _array_element_7 (Math|Vector|MakeVector (* (+ _array_index_7 1) 4e+02) (Variables|Default|GetBarrier%20Offset%20Latteral) (Variables|Default|GetBarrier_offset_height)) false false)
                        (Transformation|SetRelativeRotation _array_element_7 (Math|Rotator|Lerp(Rotator) "45.000000,-90.000000,0.000000" (Variables|Default|Getbarrier_End_Pos_left) _newtrack_0) false false)
                        (Collision|SetCollisionEnabled _array_element_7 "QueryAndPhysics")))
                    (:then_1
                      (for (_array_element_8 _array_index_8) (Variables|BeginMeshesArray|GetBegin_Right_Barrier)
                        (Rendering|SetVisibility _array_element_8 true false)
                        (Transformation|SetRelativeLocation _array_element_8 (Math|Vector|MakeVector (* (+ _array_index_8 1) 4e+02) (* (Variables|Default|GetBarrier%20Offset%20Latteral) -1.0) (Variables|Default|GetBarrier_offset_height)) false false)
                        (Transformation|SetRelativeRotation _array_element_8 (Math|Rotator|Lerp(Rotator) "45.000000,90.000000,0.000000" (Variables|Default|GetBarrier%20End%20Pos%20Right) _newtrack_0) false false)
                        (Collision|SetCollisionEnabled _array_element_8 "QueryAndPhysics")))
                    (:then_2
                      ;[0.03292 1 0] End_Barrier
                      (for (_array_element_9 _array_index_9) (Variables|EndingMeshesArray|GetEnding_Left_Barrier)
                        (Rendering|SetVisibility _array_element_9 true false)
                        (Transformation|SetRelativeLocation _array_element_9 (+ (Variables|Default|GetEnd_Offset) (Math|Vector|MakeVector (* (+ _array_index_9 1) -4e+02) (Variables|Default|GetBarrier%20Offset%20Latteral) (Variables|Default|GetBarrier_offset_height))) false false)
                        (Transformation|SetRelativeRotation _array_element_9 (Math|Rotator|Lerp(Rotator) "45.000000,-90.000000,0.000000" (Variables|Default|Getbarrier_End_Pos_left) _newtrack_0) false false)
                        (Collision|SetCollisionEnabled _array_element_9 "QueryAndPhysics")))
                    (:then_3
                      (for (_array_element_10 _array_index_10) (Variables|EndingMeshesArray|GetEnding_Right_Barrier)
                        (Rendering|SetVisibility _array_element_10 true false)
                        (Transformation|SetRelativeLocation _array_element_10 (+ (Variables|Default|GetEnd_Offset) (Math|Vector|MakeVector (* (+ _array_index_10 1) -4e+02) (* (Variables|Default|GetBarrier%20Offset%20Latteral) -1.0) (Variables|Default|GetBarrier_offset_height))) false false)
                        (Transformation|SetRelativeRotation _array_element_10 (Math|Rotator|Lerp(Rotator) "45.000000,90.000000,0.000000" (Variables|Default|GetBarrier%20End%20Pos%20Right) _newtrack_0) false false)
                        (Collision|SetCollisionEnabled _array_element_10 "QueryAndPhysics")))))))))))
    (:then_1
      (Audio|PlaySoundatLocation "/Game/05_Audio/SFX/MetaSounds/GPE/DrawBridge/DrawBridge_v2/MSS_DrawBridge_v2_Dry_Mono.MSS_DrawBridge_v2_Dry_Mono" (Transformation|GetSocketLocation (Variables|Default|GetArrow) "None") "0, 0, 0" 0.85 1.0 0.0 0 0 0 0)
      (Audio|PlaySound2D "/Game/05_Audio/SFX/MetaSounds/GPE/DrawBridge/DrawBridge_v2/MSS_DrawBridge_v2_Stereo_Reverb.MSS_DrawBridge_v2_Stereo_Reverb" 0.85 1.0 0.0 0 0))))

(event EventBeginPlay
  (EventDispatchers|BindEventtoOnAction (delegate Custom|OnDeployement)))

(fn ConstructionScript
  (bind _ending (Variables|Default|GetEnding))
  ;[0 0.8653 1] Lenght Count
  (for _index (range 0 (- (Variables|BridgeLength|GetSubdivision) 1))
    (Utilities|FlowControl|Sequence
      (:then_0
        ;[1 0.1008 0] Mid_begin
        (CallFunction|SpawnStaticMeshes (Utilities|Array|Get(acopy) (Variables|Default|GetStatic_meshes) 1) (Math|Transform|MakeTransform "0, 0, 0" "0.000000,90.000000,0.000000") false (Variables|Begin_Meshes_Array|GetBegin_mid_modules) (Variables|Default|GetInitial%20%20floor%20Collision))
        ;[1 0.9513 0] Plateform_begin
        (CallFunction|SpawnStaticMeshes (Utilities|Array|Get(acopy) (Variables|Default|GetStatic_meshes) 2) (Math|Transform|MakeTransform "0, 0, 0") false (Variables|BeginMeshesArray|GetBegin_Left_Plates) (Variables|Default|GetInitial%20%20floor%20Collision))
        (CallFunction|SpawnStaticMeshes (Utilities|Array|Get(acopy) (Variables|Default|GetStatic_meshes) 2) (Math|Transform|MakeTransform "0, 0, 0") false (Variables|BeginMeshesArray|Getbegin_Right_Plates) (Variables|Default|GetInitial%20%20floor%20Collision))
        ;[0 1 0.1477] Barrier_begin
        (CallFunction|SpawnStaticMeshes (Utilities|Array|Get(acopy) (Variables|Default|GetStatic_meshes) 3) (Math|Transform|MakeTransform "0, 0, 0") false (Variables|BeginMeshesArray|GetBegin_Left_Barrier) (Variables|Default|GetInitial%20barrier%20Collision))
        (CallFunction|SpawnStaticMeshes (Utilities|Array|Get(acopy) (Variables|Default|GetStatic_meshes) 3) (Math|Transform|MakeTransform "0, 0, 0") false (Variables|BeginMeshesArray|GetBegin_Right_Barrier) (Variables|Default|GetInitial%20barrier%20Collision)))
      (:then_1
        ;[1 0.1008 0] Mid
        (CallFunction|SpawnStaticMeshes (Utilities|Array|Get(acopy) (Variables|Default|GetStatic_meshes) 1) (Math|Transform|MakeTransform (Variables|Default|GetEnd_Offset) "0.000000,90.000000,0.000000") false (Variables|Ending_Meshes_Array|GetEnding_Mid_Modules) (Variables|Default|GetInitial%20%20floor%20Collision))
        ;[1 0.9513 0] Plateform
        (CallFunction|SpawnStaticMeshes (Utilities|Array|Get(acopy) (Variables|Default|GetStatic_meshes) 2) (Math|Transform|MakeTransform (Variables|Default|GetEnd_Offset) (Variables|Default|GetEnd_Rotation)) false (Variables|EndingMeshesArray|GetEnding_Left_Plates) (Variables|Default|GetInitial%20%20floor%20Collision))
        (CallFunction|SpawnStaticMeshes (Utilities|Array|Get(acopy) (Variables|Default|GetStatic_meshes) 2) (Math|Transform|MakeTransform (Variables|Default|GetEnd_Offset) (Variables|Default|GetEnd_Rotation)) false (Variables|EndingMeshesArray|GetEnding_Right_Plates) (Variables|Default|GetInitial%20%20floor%20Collision))
        ;[0 1 0.1477] Barrier
        (CallFunction|SpawnStaticMeshes (Utilities|Array|Get(acopy) (Variables|Default|GetStatic_meshes) 3) (Math|Transform|MakeTransform (Variables|Default|GetEnd_Offset) (Variables|Default|GetEnd_Rotation)) false (Variables|EndingMeshesArray|GetEnding_Left_Barrier) (Variables|Default|GetInitial%20barrier%20Collision))
        (CallFunction|SpawnStaticMeshes (Utilities|Array|Get(acopy) (Variables|Default|GetStatic_meshes) 3) (Math|Transform|MakeTransform (Variables|Default|GetEnd_Offset) (Variables|Default|GetEnd_Rotation)) false (Variables|EndingMeshesArray|GetEnding_Right_Barrier) (Variables|Default|GetInitial%20barrier%20Collision)))))
  ;[0.6538 0 1] End Part
  (Transformation|SetRelativeLocation _ending (+ (Math|Vector|MakeVector (* _index 8e+02) 0.0 0.0) "400.000000,0.000000,0.000000") false false)
  (Variables|Default|SetEnd_Rotation (Variables|/Script/Engine.SceneComponent|GetRelativeRotation _ending))
  (Variables|Default|SetEnd_Offset (+ (Math|Vector|MakeVector (* _index 8e+02) 0.0 0.0) "400.000000,0.000000,0.000000")))

(fn SpawnStaticMeshes
  (params (Static%20Mesh%20to%20spawn :type Static%20Mesh%20Object%20Reference) (Transform :type Transform) (initial%20Visibility :type Boolean) (Static%20Meshes%20to%20Array :type Array%20of%20Static%20Mesh%20Component%20Object%20References) (initial_collision :type ECollisionEnabled%20Enum :default "NoCollision"))
  (bind _returnvalue (AddComponent|AddStaticMeshComponent false Transform))
  (Components|StaticMesh|SetStaticMesh _returnvalue Static%20Mesh%20to%20spawn)
  (Rendering|SetVisibility _returnvalue initial%20Visibility false)
  (Collision|SetCollisionEnabled _returnvalue initial_collision)
  (Utilities|Array|AddUnique Static%20Meshes%20to%20Array _returnvalue))