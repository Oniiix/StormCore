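; Arena alien door that animates tendrils opening and closing in response to bound open and close events.
; Both events share one path that swaps the static filler mesh for a tendril cache, played in reverse to open and forward to close.
; After playback, the matching open or closed mesh returns and sound mixes muting enemies and lightning are popped.
; A delayed door sound plays alongside the animation.
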(event Custom|Alien_open
  (bind _alien_filler_mesh (Variables|Default|GetAlien_filler_mesh))
  (bind _alien_tendril_door_cache (Variables|Default|GetAlien_tendril_door_Cache))
  (bind _alien_filler_mesh_2 (Variables|Default|GetAlien_filler_mesh))
  (Variables|Default|SetIS_Openning true)
  ;[0.02277 1 0] Open
  (Rendering|SetVisibility (Variables|Default|GetAlien_tendril_door_Cache) true false)
  (Rendering|SetVisibility _alien_filler_mesh false false)
  (Utilities|FlowControl|Sequence
    (:then_0
      (if (Variables|Default|GetIS_Openning)
        (Class|GeometryCacheComponent|PlayReversedfromEnd _alien_tendril_door_cache)
        (else
          (Components|Timeline|PlayfromStart _alien_tendril_door_cache)))
      (Utilities|FlowControl|Delay (Variables|/Script/GeometryCache.GeometryCacheComponent|GetDuration _alien_tendril_door_cache))
      (Components|StaticMesh|SetStaticMesh _alien_filler_mesh_2 (select (Variables|Default|GetIS_Openning) "/Game/06_Tech/Alien_door/Alien_door_open.Alien_door_open" "/Game/06_Tech/Alien_door/Alien_door_close.Alien_door_close"))
      (Rendering|SetVisibility _alien_tendril_door_cache false false)
      (Rendering|SetVisibility _alien_filler_mesh_2 true false)
      ;;[1 1 1] Enemies + Hazard SFX ON
      (Audio|PopSoundMixModifier "/Game/05_Audio/SoundClass_Mixes/Enemies_Muted/SCM_Enemies_Muted.SCM_Enemies_Muted")
      (Audio|PopSoundMixModifier "/Game/05_Audio/SoundClass_Mixes/Enemies_Muted/SCM_Agressive_Lightnings_Muted.SCM_Agressive_Lightnings_Muted"))
    (:then_1
      ;[1 1 1] Opening/ClosingSFX
      (Utilities|FlowControl|Delay 0.7)
      (Audio|PlaySoundatLocation "/Game/05_Audio/SFX/MetaSounds/GPE/Alien_Door/MSS_Alien_Door.MSS_Alien_Door" (Transformation|GetSocketLocation _alien_filler_mesh "None") "0, 0, 0" 1.0 1.0 0.0 0 0 0 0))))

(event Custom|Alien_Close
  (bind _alien_filler_mesh (Variables|Default|GetAlien_filler_mesh))
  (bind _alien_tendril_door_cache (Variables|Default|GetAlien_tendril_door_Cache))
  (bind _alien_filler_mesh_2 (Variables|Default|GetAlien_filler_mesh))
  (Variables|Default|SetIS_Openning false)
  ;[0.02277 1 0] Open
  (Rendering|SetVisibility (Variables|Default|GetAlien_tendril_door_Cache) true false)
  (Rendering|SetVisibility _alien_filler_mesh false false)
  (Utilities|FlowControl|Sequence
    (:then_0
      (if (Variables|Default|GetIS_Openning)
        (Class|GeometryCacheComponent|PlayReversedfromEnd _alien_tendril_door_cache)
        (else
          (Components|Timeline|PlayfromStart _alien_tendril_door_cache)))
      (Utilities|FlowControl|Delay (Variables|/Script/GeometryCache.GeometryCacheComponent|GetDuration _alien_tendril_door_cache))
      (Components|StaticMesh|SetStaticMesh _alien_filler_mesh_2 (select (Variables|Default|GetIS_Openning) "/Game/06_Tech/Alien_door/Alien_door_open.Alien_door_open" "/Game/06_Tech/Alien_door/Alien_door_close.Alien_door_close"))
      (Rendering|SetVisibility _alien_tendril_door_cache false false)
      (Rendering|SetVisibility _alien_filler_mesh_2 true false)
      ;;[1 1 1] Enemies + Hazard SFX ON
      (Audio|PopSoundMixModifier "/Game/05_Audio/SoundClass_Mixes/Enemies_Muted/SCM_Enemies_Muted.SCM_Enemies_Muted")
      (Audio|PopSoundMixModifier "/Game/05_Audio/SoundClass_Mixes/Enemies_Muted/SCM_Agressive_Lightnings_Muted.SCM_Agressive_Lightnings_Muted"))
    (:then_1
      ;[1 1 1] Opening/ClosingSFX
      (Utilities|FlowControl|Delay 0.7)
      (Audio|PlaySoundatLocation "/Game/05_Audio/SFX/MetaSounds/GPE/Alien_Door/MSS_Alien_Door.MSS_Alien_Door" (Transformation|GetSocketLocation _alien_filler_mesh "None") "0, 0, 0" 1.0 1.0 0.0 0 0 0 0))))

(event Custom|Debug_Anim_Open)

(event Custom|Debug_Anim_Close)

(event EventBeginPlay
  (bind _alien_filler_mesh (Variables|Default|GetAlien_filler_mesh))
  (Rendering|SetVisibility (Variables|Default|GetAlien_tendril_door_Cache) false false)
  (Components|StaticMesh|SetStaticMesh _alien_filler_mesh "/Game/06_Tech/Alien_door/Alien_door_open.Alien_door_open")
  (Rendering|SetVisibility _alien_filler_mesh true false)
  (EventDispatchers|BindEventtoOnOpen (delegate Custom|Alien_open))
  (EventDispatchers|BindEventtoOnClose (delegate Custom|Alien_Close)))

(event Collision|EventActorBeginOverlap
  (params (OtherActor :type Actor%20Object%20Reference)))

(event EventTick
  (params (DeltaSeconds :type Float%20%28single-precision%29)))

(fn ConstructionScript)