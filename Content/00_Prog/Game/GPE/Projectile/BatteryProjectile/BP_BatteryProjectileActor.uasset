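; Battery projectile actor that presents a thrown Zeus lance and its electric area of effect, handling visuals and sound.
; On launch it attaches a Niagara trail to the spear mesh and starts tracking its position.
; Each tick it rotates the spear along its frame-to-frame movement, playing the throw sound on first movement.
; The AOE event spawns a Niagara effect sized by RadiusRange and a one-time electrocute sound.
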(event Custom|onSpawnAOE_Event
  (Utilities|FlowControl|Sequence
    (:then_0
      (bind _returnvalue (Niagara|SpawnSystematLocation "/Game/04_FX/NS/Player/Zeus_Battery_Bolt/NS_Zeus_AOE.NS_Zeus_AOE" (Transformation|GetActorLocation)))
      (Niagara|SetNiagaraVariable(Float) _returnvalue "Radius" (Variables|Default|GetradiusRange)))
    (:then_1
      (Utilities|FlowControl|DoOnce false
        (:Completed
          (Audio|SpawnSoundAttached "/Game/05_Audio/SFX/MetaSounds/Player/Weapons/Left_Arm/ZBB/MSS_ZBB_Electrocute.MSS_ZBB_Electrocute" (Variables|Default|GetspearMesh) "None" "0, 0, 0" "0, 0, 0" "KeepRelativeOffset" false 1.0 1.0 0.0 0 0))))))

(event Custom|onLaunch_Event
  (Variables|Default|SetPos (Transformation|GetActorLocation))
  (Niagara|SpawnSystemAttached "/Game/04_FX/NS/Player/Zeus_Battery_Bolt/NS_Zeus_Lance.NS_Zeus_Lance" (Variables|Default|GetspearMesh) "Trail_Pos" "0, 0, 0" "0, 0, 0" "KeepRelativeOffset" false)
  (Variables|Default|SetisLaunch true))

(event EventBeginPlay
  (EventDispatchers|AssignOnLaunch (delegate Custom|onLaunch_Event))
  (EventDispatchers|AssignOnSpawnAOE (delegate Custom|onSpawnAOE_Event)))

(event EventTick
  (params (DeltaSeconds :type Float%20%28single-precision%29))
  (bind _returnvalue (Transformation|GetActorLocation))
  (if (Variables|Default|GetisLaunch)
    (Variables|Default|SetPos_Delay (Variables|Default|GetPos))
    (Variables|Default|SetPos _returnvalue)
    (if (not (Utilities|Operators|EqualEqual :A (Math|Vector|Normalize (- (Variables|Default|GetPos) (Variables|Default|GetPos_Delay)))))
      (Transformation|SetWorldRotation (Variables|Default|GetspearMesh) (Math|Conversions|RotationFromXVector (Math|Vector|Normalize (- (Variables|Default|GetPos) (Variables|Default|GetPos_Delay)))) false false)
      (Utilities|FlowControl|DoOnce false
        (:Completed
          (Audio|PlaySoundatLocation "/Game/05_Audio/SFX/MetaSounds/Player/Weapons/Left_Arm/ZBB/ZBB_Throw.ZBB_Throw" _returnvalue "0, 0, 0" 1.0 1.0 0.0 0 0 0 0))))))

(fn ConstructionScript)