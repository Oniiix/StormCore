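; End-of-game trigger actor that plays the ending cinematic when the main character overlaps it, then shows the credits.
; On overlap it hides the character and HUD, disables input, notifies the game instance, stops the tower SFX timer and plays the level sequence.
; Alongside, it overrides the audio listener, fades out tower SFX layers and briefly fades in end-cinematic ambience.
; Achievements update through the player controller's leaderboard call at start and finish.
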(event Custom|OnComponentBeginOverlap_Event
  (params (OverlappedComponent :type Primitive%20Component%20Object%20Reference) (OtherActor :type Actor%20Object%20Reference) (OtherComp :type Primitive%20Component%20Object%20Reference) (OtherBodyIndex :type Integer) (bFromSweep :type Boolean) (SweepResult :type Hit%20Result%20Structure%20%28by%20ref%29))
  (bind _isvalid (CallFunction|HideandDisableInput OtherActor))
  (if _isvalid
    (Default|CallOnEndingTriggered (Variables|Default|GetAs%20Custom%20Game%20Instance%20BP))
    (bind _outactor (Sequencer|Player|CreateLevelSequencePlayer (Variables|Custom|GetLevel%20Sequence)))
    (Utilities|FlowControl|Sequence
      (:then_0
        (EventDispatchers|BindEventtoOnFinished (Variables|/Script/LevelSequence.LevelSequenceActor|GetSequencePlayer _outactor) (delegate Custom|CustomEvent))
        (bind _outactors (Actor|GetAllActorsOfClass "/Game/05_Audio/BP/BP_TowerField_SFX.BP_TowerField_SFX_C"))
        (Utilities|Time|ClearandInvalidateTimerbyHandle (Variables|/Game/05_Audio/BP/BP_TowerField_SFX.BP_TowerField_SFX_C|GetTimer%20Check (Utilities|Array|Get(acopy) _outactors)))
        (Sequencer|Player|Play (Variables|/Script/LevelSequence.LevelSequenceActor|GetSequencePlayer _outactor) :!class /Script/MovieScene.MovieSceneSequencePlayer)
        (CallFunction|UpdateAchievement (Utilities|Array|MakeArray "The_Eye_of_the_Storm")))
      (:then_1
        ;[1 1 1] Tower SFX Fade Out
        (Class|PlayerController|SetAudioListenerOverride (Game|GetPlayerController 0) 0 (Transformation|GetWorldLocation (Variables|Default|GetDefaultSceneRoot)) "0, 0, 0")
        (bind _outactors_2 (Actor|GetAllActorsOfClass "/Game/05_Audio/BP/BP_TowerField_SFX.BP_TowerField_SFX_C"))
        (Utilities|IsValid (Variables|/Game/05_Audio/BP/BP_TowerField_SFX.BP_TowerField_SFX_C|GetLayer%201%20SFX (Utilities|Array|Get(acopy) _outactors_2))
          (:Is%20Valid
            (Audio|Components|Audio|AdjustVolume (Variables|/Game/05_Audio/BP/BP_TowerField_SFX.BP_TowerField_SFX_C|GetLayer%201%20SFX (Utilities|Array|Get(acopy) _outactors_2)) 0.2 1.0 "Linear" :!class /Script/Engine.AudioComponent))
          (:Is%20Not%20Valid
            _))
        (Utilities|IsValid (Variables|/Game/05_Audio/BP/BP_TowerField_SFX.BP_TowerField_SFX_C|GetLayer%202%20SFX (Utilities|Array|Get(acopy) _outactors_2))
          (:Is%20Valid
            (Audio|Components|Audio|AdjustVolume (Variables|/Game/05_Audio/BP/BP_TowerField_SFX.BP_TowerField_SFX_C|GetLayer%202%20SFX (Utilities|Array|Get(acopy) _outactors_2)) 0.2 1.0 "Linear" :!class /Script/Engine.AudioComponent))
          (:Is%20Not%20Valid
            _))
        (Utilities|IsValid (Variables|/Game/05_Audio/BP/BP_TowerField_SFX.BP_TowerField_SFX_C|GetLayer%203%20SFX (Utilities|Array|Get(acopy) _outactors_2))
          (:Is%20Valid
            (Audio|Components|Audio|AdjustVolume (Variables|/Game/05_Audio/BP/BP_TowerField_SFX.BP_TowerField_SFX_C|GetLayer%203%20SFX (Utilities|Array|Get(acopy) _outactors_2)) 0.2 1.0 "SCurve" :!class /Script/Engine.AudioComponent))
          (:Is%20Not%20Valid
            _))
        (Utilities|FlowControl|Sequence
          (:then_0
            (Utilities|FlowControl|Delay 4.75)
            (bind _outactors_3 (Actor|GetAllActorsOfClass "/Game/05_Audio/BP/BP_TowerField_SFX.BP_TowerField_SFX_C"))
            (Utilities|IsValid (Variables|/Game/05_Audio/BP/BP_TowerField_SFX.BP_TowerField_SFX_C|GetLayer%201%20SFX (Utilities|Array|Get(acopy) _outactors_3))
              (:Is%20Valid
                (Audio|Components|Audio|FadeOut (Variables|/Game/05_Audio/BP/BP_TowerField_SFX.BP_TowerField_SFX_C|GetLayer%201%20SFX (Utilities|Array|Get(acopy) _outactors_3)) 8.7 0.0 "SCurve" :!class /Script/Engine.AudioComponent))
              (:Is%20Not%20Valid
                _))
            (Utilities|IsValid (Variables|/Game/05_Audio/BP/BP_TowerField_SFX.BP_TowerField_SFX_C|GetLayer%202%20SFX (Utilities|Array|Get(acopy) _outactors_3))
              (:Is%20Valid
                (Audio|Components|Audio|FadeOut (Variables|/Game/05_Audio/BP/BP_TowerField_SFX.BP_TowerField_SFX_C|GetLayer%202%20SFX (Utilities|Array|Get(acopy) _outactors_3)) 8.7 0.0 "Logarithmic" :!class /Script/Engine.AudioComponent))
              (:Is%20Not%20Valid
                _))
            (Utilities|IsValid (Variables|/Game/05_Audio/BP/BP_TowerField_SFX.BP_TowerField_SFX_C|GetLayer%203%20SFX (Utilities|Array|Get(acopy) _outactors_3))
              (:Is%20Valid
                (Audio|Components|Audio|FadeOut (Variables|/Game/05_Audio/BP/BP_TowerField_SFX.BP_TowerField_SFX_C|GetLayer%203%20SFX (Utilities|Array|Get(acopy) _outactors_3)) 4.0 0.0 "SCurve" :!class /Script/Engine.AudioComponent))))
          (:then_1
            ;[1 1 1] Weather Condition SFX Reappearing in the end, just for a few sec
            (Utilities|FlowControl|Delay 10.7)
            (bind _returnvalue (Audio|SpawnSound2D "/Game/05_Audio/SFX/MetaSounds/Cinematic/End_Cinematic/MSS_Amb_SFX_End_Cinematic.MSS_Amb_SFX_End_Cinematic" 1.0 1.0 0.0 0))
            (bind _output_get (Variables|Default|SetAmb_SFX_End_Cinematic _returnvalue))
            (Audio|Components|Audio|FadeIn _output_get 4.2 1.0 0.0 "Linear" :!class /Script/Engine.AudioComponent)
            (Utilities|FlowControl|Delay 1.3)
            (Audio|Components|Audio|FadeOut (Variables|Default|GetAmb_SFX_End_Cinematic) 2.3 0.0 "Linear" :!class /Script/Engine.AudioComponent)))))))

(event Custom|CustomEvent
  ;[1 1 1] Fin séquencer
  (bind _asbp_game_hud (Utilities|Casting|CastToBp_GameHUD (HUD|GetHUD (Game|GetPlayerController 0))))
  (Utilities|IsValid _asbp_game_hud
    (:Is%20Valid
      (Class|MainHUD|SetState _asbp_game_hud "MainCredit")
      (Default|CallOnEndingCredit (Variables|Default|GetAs%20Custom%20Game%20Instance%20BP))
      (CallFunction|UpdateAchievement (Utilities|Array|MakeArray "D-3"))
      (Class|PlayerController|ClearAudioListenerOverride (Game|GetPlayerController 0)))))

(event EventBeginPlay
  (bind _ascustom_game_instance_bp (Utilities|Casting|CastToCustomGameInstance_BP (Game|GetGameInstance)))
  (Variables|Default|SetAs%20Custom%20Game%20Instance%20BP _ascustom_game_instance_bp)
  (Collision|AssignOnComponentBeginOverlap (Variables|Default|GetTrigger) (delegate Custom|OnComponentBeginOverlap_Event)))

(fn ConstructionScript)

(fn HideandDisableInput
  (params (Object :type Object%20Object%20Reference))
  (bind _asmain_character_bp (Utilities|Casting|CastToMainCharacter_BP Object))
  (Utilities|IsValid _asmain_character_bp
    (:Is%20Valid
      (Class|MainCharacter|SetDisableInput _asmain_character_bp true)
      (bind _asbp_game_hud (Utilities|Casting|CastToBp_GameHUD (HUD|GetHUD (Game|GetPlayerController 0))))
      (Class|MainHUD|HideUI _asbp_game_hud)
      (Rendering|SetActorHiddenInGame _asmain_character_bp true)
      (return true))
    (:Is%20Not%20Valid
      (return false))))

(fn UpdateAchievement
  (params (Achievement%20Name :type Array%20of%20Names))
  (bind _asbp_custom_player_controller (Utilities|Casting|CastToBP_CustomPlayerController (Game|GetPlayerController 0)))
  (for _array_element Achievement%20Name
    (Class|CustomPlayerController|UpdateLeaderboard _asbp_custom_player_controller _array_element 1)))