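; DroneFireflies_BP is a drone fireflies actor that displays its target-marking state through a lock-on widget.
; On BeginPlay it caches the BP_Fireflies_Lock_ATH widget and binds marking event dispatchers.
; View enter and exit toggle the widget's in/out material parameter, while init, progress and confirmation drive its zoom parameter.
; The mark-disable handler is bound but empty.
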(event Custom|onProgress_Event
  (params (_markProgress :type Float%20%28single-precision%29))
  ;[1 1 1] Progtress
  (Default|SetTargetScalarParameter (Variables|Default|GetWidget_Target) (Variables|Default|GetZoom_Parameter) _markProgress))

(event Custom|onInit_Event
  ;[1 1 1] Progtress
  (Default|SetTargetScalarParameter (Variables|Default|GetWidget_Target) (Variables|Default|GetZoom_Parameter) 0.0))

(event Custom|onInView_Event
  (params (_target :type Actor%20Object%20Reference))
  ;[1 1 1] View
  (Default|SetTargetScalarParameter (Variables|Default|GetWidget_Target) (Variables|Default|GetInOut_Parameter) 0.0))

(event Custom|onOutView_Event
  (params (_target :type Actor%20Object%20Reference))
  ;[1 1 1] View
  (Default|SetTargetScalarParameter (Variables|Default|GetWidget_Target) (Variables|Default|GetInOut_Parameter) 1.0))

(event Custom|onMarkConfirmed_Event
  (params (_target :type Actor%20Object%20Reference) (_drone :type Drone%20Fireflies%20Object%20Reference))
  ;[1 1 1] Confirlatuion
  (Default|SetTargetScalarParameter (Variables|Default|GetWidget_Target) (Variables|Default|GetZoom_Parameter) 1.0))

(event Custom|onDisableMark_Event
  (params (_target :type Actor%20Object%20Reference) (_drone :type Drone%20Fireflies%20Object%20Reference))
  ;[1 1 1] Confirlatuion
)

(event EventBeginPlay
  (bind _asbp_fireflies_lock_ath (Utilities|Casting|CastToBP_Fireflies_Lock_ATH (UserInterface|GetWidget (Variables|Default|GetWidget))))
  (Variables|Default|SetWidget_Target _asbp_fireflies_lock_ath)
  (EventDispatchers|AssignOnInit (delegate Custom|onInit_Event))
  (EventDispatchers|AssignOnProgress (delegate Custom|onProgress_Event))
  (EventDispatchers|AssignOninView (delegate Custom|onInView_Event))
  (EventDispatchers|AssignOnOutView (delegate Custom|onOutView_Event))
  (EventDispatchers|AssignOnMarkConfirmed (delegate Custom|onMarkConfirmed_Event))
  (EventDispatchers|AssignOnDisableMark (delegate Custom|onDisableMark_Event)))

(event Collision|EventActorBeginOverlap
  (params (OtherActor :type Actor%20Object%20Reference)))

(fn ConstructionScript)