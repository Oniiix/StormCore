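; Handcar (hovercraft draisine) actor that handles presentation of stopping and moving, whether player-driven or remote.
; OnStop drives a gated State event that animates doors, ramps and hull height and toggles turbine VFX and startup, shutdown and travel sounds.
; Tick maps CurrentSpeed to pitch and volume on four layers of both player and remote travel sounds.
; Construction gathers turbine, stock, nitro and brake child actors.
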(event OnComponentEndOverlap(hitBox)
  (params (OverlappedComponent :type Primitive%20Component%20Object%20Reference) (OtherActor :type Actor%20Object%20Reference) (OtherComp :type Primitive%20Component%20Object%20Reference) (OtherBodyIndex :type Integer))
  ;[1 1 1] Hitbox Overlaps
  (if (== (Utilities|GetClass OtherActor) "/Game/00_Prog/CCC/Character/MainCharacter_BP.MainCharacter_BP_C")
    (Variables|Default|SetPlayer_On_Handcar? false)
    (Audio|Components|Audio|Stop (Variables|Default|GetHovercraft_Travel_By_Player_SFX))
    (Variables|Default|SetHovercraft%20Travel%20By%20Player%20SFX%20Already%20Played false)))

(event OnComponentBeginOverlap(hitBox)
  (params (OverlappedComponent :type Primitive%20Component%20Object%20Reference) (OtherActor :type Actor%20Object%20Reference) (OtherComp :type Primitive%20Component%20Object%20Reference) (OtherBodyIndex :type Integer) (bFromSweep :type Boolean) (SweepResult :type Hit%20Result%20Structure%20%28by%20ref%29))
  ;[1 1 1] Hitbox Overlaps
  (if (== (Utilities|GetClass OtherActor) "/Game/00_Prog/CCC/Character/MainCharacter_BP.MainCharacter_BP_C")
    (Variables|Default|SetPlayer_On_Handcar? true)))

(event Custom|State
  (params (isStopped :type Boolean) (inAutoMode :type Boolean))
  ;[1 0 0.004591] On Stop
  (Utilities|FlowControl|Sequence
    (:then_0
      (Utilities|FlowControl|Gate true :!label _label
        (:Exit
          (Variables|Default|SetRemote_Travel? inAutoMode)
          (Variables|Default|SetFirstTimeActivation? false)
          (if isStopped
            (CallFunction|OpenDraisine)
            (Utilities|FlowControl|Sequence
              (:then_0
                (for _array_element (Variables|Default|GetTurbines)
                  (Variables|/Game/06_Tech/Draisine/BP_Turbine.BP_Turbine_C|SetHandcarStopped? _array_element true)))
              (:then_1
                (CallFunction|VFXTurbinesActivation false)
                (CallFunction|TurbinesShutdownSFX)
                (CallFunction|SFXRemoteTravelState false)
                (CallFunction|SFXPlayerTravelState false)))
            (else
              (CallFunction|CloseDraisine)
              (Utilities|FlowControl|Sequence
                (:then_0
                  (for _array_element_2 (Variables|Default|GetTurbines)
                    (Variables|/Game/06_Tech/Draisine/BP_Turbine.BP_Turbine_C|SetHandcarStopped? _array_element_2 false)))
                (:then_1
                  (CallFunction|VFXTurbinesActivation true)
                  (Variables|Default|SetHovercraft%20Already%20Moved? true)
                  (if (Variables|Default|GetRemote_Travel?)
                    (CallFunction|SFXRemoteTravelState true)
                    (else
                      (CallFunction|SFXPlayerTravelState true)
                      (CallFunction|HovercraftStartupSFX))))))))))
    (:then_1
      (Utilities|FlowControl|Delay 0.1)
      (goto _label Open))))

(event Custom|onUseControls_Event
  (params (isUsing :type Boolean))
  ;[1 0 0.004591] On Stop
  (Utilities|FlowControl|Sequence
    (:then_0
      (if (Variables|Default|GetDriver%20Seat%20Activated)
        (Audio|PlaySoundatLocation "/Game/05_Audio/SFX/MetaSounds/Hovercraft/Hovercraft_Cockpit_Deactivate/MSS_Hovercraft_Cockpit_Deactivate.MSS_Hovercraft_Cockpit_Deactivate" (Transformation|GetSocketLocation (Variables|Character|GetMesh) "None") "0, 0, 0" 1.0 1.0 0.0 0 0 0 0)
        (Variables|Default|SetDriver%20Seat%20Activated false)
        (else
          (Audio|PlaySoundatLocation "/Game/05_Audio/SFX/MetaSounds/Hovercraft/Hovercraft_Cockpit_Activate/MSS_Hovercraft_Cockpit_Activate.MSS_Hovercraft_Cockpit_Activate" (Transformation|GetSocketLocation (Variables|Character|GetMesh) "None") "0, 0, 0" 1.0 1.0 0.0 0 0 0 0)
          (Variables|Default|SetDriver%20Seat%20Activated true))))
    (:then_1
      (if (Variables|Default|GetFirstTimeActivation?)
        (CallFunction|EventFirstTimeActivation)))))

(event Custom|Turbines%20Shutdown%20SFX
  (bind _startup_sfx (Variables|Default|GetStartup%20SFX))
  ;[1 1 1] Hovercraft Shutdown SFX (OS)
  (Utilities|FlowControl|Sequence
    (:then_0
      (if (Variables|Default|GetHovercraft%20Already%20Moved?)
        (Audio|PlaySoundatLocation "/Game/05_Audio/SFX/MetaSounds/Hovercraft/HoverCraft_Shutdown/Layer_1/MSS_Hovercraft_Shutdown_Layer1.MSS_Hovercraft_Shutdown_Layer1" (Transformation|GetSocketLocation (Variables|Default|GetTurbine1) "None") "0, 0, 0" 1.0 1.0 0.0 0 0 0 0)
        (Audio|PlaySoundatLocation "/Game/05_Audio/SFX/MetaSounds/Hovercraft/HoverCraft_Shutdown/Layer_1/MSS_Hovercraft_Shutdown_Layer1.MSS_Hovercraft_Shutdown_Layer1" (Transformation|GetSocketLocation (Variables|Default|GetTurbine2) "None") "0, 0, 0" 1.0 1.0 0.0 0 0 0 0)
        (Audio|PlaySoundatLocation "/Game/05_Audio/SFX/MetaSounds/Hovercraft/HoverCraft_Shutdown/Layer_1/MSS_Hovercraft_Shutdown_Layer1.MSS_Hovercraft_Shutdown_Layer1" (Transformation|GetSocketLocation (Variables|Default|GetTurbine3) "None") "0, 0, 0" 1.0 1.0 0.0 0 0 0 0)
        (Audio|PlaySoundatLocation "/Game/05_Audio/SFX/MetaSounds/Hovercraft/HoverCraft_Shutdown/Layer_1/MSS_Hovercraft_Shutdown_Layer1.MSS_Hovercraft_Shutdown_Layer1" (Transformation|GetSocketLocation (Variables|Default|GetTurbine4) "None") "0, 0, 0" 1.0 1.0 0.0 0 0 0 0)
        (Utilities|IsValid _startup_sfx ; Add is valid beacause of errors
          (:Is%20Valid
            (if (Audio|Components|Audio|IsPlaying _startup_sfx)
              (Audio|Components|Audio|FadeOut _startup_sfx 1.0 0.0 "SCurve" :!class /Script/Engine.AudioComponent))))))
    (:then_1
      (if (Variables|Default|GetPlayer_On_Handcar?)
        (bind _returnvalue (Audio|SpawnSound2D "/Game/05_Audio/SFX/MetaSounds/Hovercraft/HoverCraft_Shutdown/Layer_2/By_Player/MSS_Hovercraft_Shutdown_By_Player_Layer2.MSS_Hovercraft_Shutdown_By_Player_Layer2" 1.0 1.0 0.0 0 false false))
        (Variables|Default|SetHovercraft%20Shutdown%20By%20Player%20SFX _returnvalue)
        (else
          (bind _returnvalue_2 (Audio|SpawnSoundatLocation "/Game/05_Audio/SFX/MetaSounds/Hovercraft/HoverCraft_Shutdown/Layer_2/By_Remote/MSS_Hovercraft_Shutdown_By_Remote_Layer2.MSS_Hovercraft_Shutdown_By_Remote_Layer2" (Transformation|GetSocketLocation (Variables|Default|GetHandcar) "None") "0, 0, 0" 1.0 1.0 0.0 0 0 false))
          (Variables|Default|SetHovercraft%20Shutdown%20By%20Remote%20SFX _returnvalue_2))))))

(event Custom|open%20Draisine
  (bind _mesh_startpos (Variables|Default|GetMesh_StartPos))
  ;[0 1 0.08467] Doors
  (Components|Timeline|SetPlayRate (Variables|Default|GetTimeline_Door) 1.5)
  (bind (_direction _door_anim _ramp_anim _brake _height_anim) (Timeline|Timeline_Door Play)
    (:Update
      (Transformation|SetRelativeLocation (Variables|Default|GetDoor_first_right) (Math|Vector|Lerp(Vector) "0.000000,-150.000000,0.000000" "0, 0, 0" _door_anim) false false)
      ;[1 0.05399 0] Ramp
      (Transformation|SetRelativeLocation (Variables|Default|GetRamp_F_R_) (Math|Vector|Lerp(Vector) "0, 0, 0" "-115.000000,0.000000,0.000000" _ramp_anim) false false)
      (Transformation|SetRelativeLocation (Variables|Default|GetRamp_M_R) (Math|Vector|Lerp(Vector) "0, 0, 0" "-100.000000,0.000000,0.000000" _ramp_anim) false false)
      (Transformation|SetRelativeRotation (Variables|Default|GetRamp_F_L) (Math|Rotator|Lerp(Rotator) "0, 0, 0" "12.500000,0.000000,0.000000" _ramp_anim) false false)
      (Transformation|SetRelativeLocation (Variables|Character|GetMesh) (Math|Vector|MakeVector (.x _mesh_startpos) (.y _mesh_startpos) (Math|Float|Lerp (.z _mesh_startpos) (+ (.z _mesh_startpos) (Variables|Default|GetMoving_Height_Offset)) _height_anim)) false false))))

(event Custom|Close_Draisine
  (bind _mesh_startpos (Variables|Default|GetMesh_StartPos))
  ;[0 1 0.08467] Doors
  (bind (_direction _door_anim _ramp_anim _brake _height_anim) (Timeline|Timeline_Door Reverse)
    (:Update
      (Transformation|SetRelativeLocation (Variables|Default|GetDoor_first_right) (Math|Vector|Lerp(Vector) "0.000000,-150.000000,0.000000" "0, 0, 0" _door_anim) false false)
      ;[1 0.05399 0] Ramp
      (Transformation|SetRelativeLocation (Variables|Default|GetRamp_F_R_) (Math|Vector|Lerp(Vector) "0, 0, 0" "-115.000000,0.000000,0.000000" _ramp_anim) false false)
      (Transformation|SetRelativeLocation (Variables|Default|GetRamp_M_R) (Math|Vector|Lerp(Vector) "0, 0, 0" "-100.000000,0.000000,0.000000" _ramp_anim) false false)
      (Transformation|SetRelativeRotation (Variables|Default|GetRamp_F_L) (Math|Rotator|Lerp(Rotator) "0, 0, 0" "12.500000,0.000000,0.000000" _ramp_anim) false false)
      (Transformation|SetRelativeLocation (Variables|Character|GetMesh) (Math|Vector|MakeVector (.x _mesh_startpos) (.y _mesh_startpos) (Math|Float|Lerp (.z _mesh_startpos) (+ (.z _mesh_startpos) (Variables|Default|GetMoving_Height_Offset)) _height_anim)) false false))))

(event Custom|VFX_Turbines_Activation
  (params (Active? :type Boolean))
  ;[1 0 0.004591] On Stop
  (for _array_element (Variables|Default|GetTurbines)
    (Default|SetActivation _array_element Active?)))

(event Custom|SFX_Remote_Travel_State
  (params (Play? :type Boolean))
  ;[1 1 1] SFX States
  (if Play?
    ;[1 1 1] Travel SFX ON/OFF System
    (Audio|Components|Audio|Play (Variables|Default|GetMSS_HoverCraft_Travel_By_Remote) 0.0)
    (bind (_direction _fade_in_out_curve) (Timeline|Hovercraft%20Travel%20By%20Remote%20SFX%20Fade%20IN/OUT PlayFromStart)
      (:Update
        (Audio|Parameter|SetFloatParameter (Variables|Default|GetMSS_HoverCraft_Travel_By_Remote) "Master Volume" (* _fade_in_out_curve 0.85) :!class /Script/AudioExtensions.AudioParameterControllerInterface))
      (:Finished
        (switch Utilities|FlowControl|Switch|SwitchonETimelineDirection _direction)))
    (else
      (Timeline|Hovercraft%20Travel%20By%20Remote%20SFX%20Fade%20IN/OUT Reverse))))

(event Custom|SFX_Player_Travel_State
  (params (Play? :type Boolean))
  ;[1 1 1] SFX States
  (CallFunction|SFXRemoteTravelState false)
  (if Play?
    ;[1 1 1] Travel SFX ON/OFF System
    (Audio|Components|Audio|FadeIn (Variables|Default|GetHovercraft_Travel_By_Player_SFX) 0.35 1.0 0.0 "SCurve" :!class /Script/Engine.AudioComponent)
    (bind (_direction _fade_in_out_curve) (Timeline|Hovercraft%20Travel%20By%20Player%20SFX%20Fade%20IN/OUT Play)
      (:Update
        (Audio|Parameter|SetFloatParameter (Variables|Default|GetHovercraft_Travel_By_Player_SFX) "Master Volume" (* _fade_in_out_curve 0.85) :!class /Script/AudioExtensions.AudioParameterControllerInterface))
      (:Finished
        (switch Utilities|FlowControl|Switch|SwitchonETimelineDirection _direction)))
    (else
      (Timeline|Hovercraft%20Travel%20By%20Player%20SFX%20Fade%20IN/OUT Reverse))))

(event Custom|Hovercraft%20Startup%20SFX
  (bind _hovercraft_shutdown_by_player_sfx (Variables|Default|GetHovercraft%20Shutdown%20By%20Player%20SFX))
  (bind _hovercraft_shutdown_by_remote_sfx (Variables|Default|GetHovercraft%20Shutdown%20By%20Remote%20SFX))
  ;[1 1 1] Hovercraft Startup SFX (OS)
  (bind _returnvalue (Audio|SpawnSound2D "/Game/05_Audio/SFX/MetaSounds/Hovercraft/Hovercraft_Startup/MSS_Hovercraft_Startup.MSS_Hovercraft_Startup" 1.0 1.0 0.0 0 false false))
  (Variables|Default|SetStartup%20SFX _returnvalue)
  (Utilities|IsValid _hovercraft_shutdown_by_player_sfx :!pinned true ; Was empty add shutdown SFX
    (:Is%20Valid
      (if (Audio|Components|Audio|IsPlaying _hovercraft_shutdown_by_player_sfx)
        (Audio|Components|Audio|FadeOut _hovercraft_shutdown_by_player_sfx 1.0 0.0 "SCurve" :!class /Script/Engine.AudioComponent)
        (Utilities|IsValid _hovercraft_shutdown_by_remote_sfx
          (:Is%20Valid
            (if (Audio|Components|Audio|IsPlaying _hovercraft_shutdown_by_remote_sfx)
              (Audio|Components|Audio|FadeOut _hovercraft_shutdown_by_remote_sfx 1.0 0.0 "SCurve" :!class /Script/Engine.AudioComponent))))))))

(event Custom|Event_FirstTimeActivation
  ;[1 0 0.004591] On Stop
  (Variables|Default|SetRemote_Travel? false)
  (Variables|Default|SetFirstTimeActivation? false)
  (CallFunction|CloseDraisine)
  (Utilities|FlowControl|Sequence
    (:then_0
      (for _array_element (Variables|Default|GetTurbines)
        (Variables|/Game/06_Tech/Draisine/BP_Turbine.BP_Turbine_C|SetHandcarStopped? _array_element false)))
    (:then_1
      (CallFunction|VFXTurbinesActivation true)
      (Variables|Default|SetHovercraft%20Already%20Moved? true)
      (if (Variables|Default|GetRemote_Travel?)
        (CallFunction|SFXRemoteTravelState true)
        (else
          (CallFunction|SFXPlayerTravelState true)
          (CallFunction|HovercraftStartupSFX))))))

(event EventBeginPlay
  ;[1 0 0.004591] On Stop
  (EventDispatchers|BindEventtoOnStop (delegate Custom|State))
  (Variables|Default|SetMesh_StartPos (Variables|/Script/Engine.SceneComponent|GetRelativeLocation (Variables|Character|GetMesh)))
  (Variables|Default|SethandcarMesh (Variables|Default|GetHandcar))
  (Class|CustomHandcarActor|SetBumpBoxArray (Utilities|Array|MakeArray (Variables|Default|GetForwardBumpBox) (Variables|Default|GetBackwardBumpBox) (Variables|Default|GetLeftBumpBox) (Variables|Default|GetRightBumpBox)))
  (bind _asbp_nitro_handcar_actor (Utilities|Casting|CastToBP_NitroHandcarActor (Variables|/Script/Engine.ChildActorComponent|GetChildActor (Variables|Default|GetPilot))))
  (EventDispatchers|AssignOnUseControls _asbp_nitro_handcar_actor (delegate Custom|onUseControls_Event)))

(event Collision|EventActorBeginOverlap
  (params (OtherActor :type Actor%20Object%20Reference)))

(event EventTick
  (params (DeltaSeconds :type Float%20%28single-precision%29))
  ;[1 1 1] Engine (Travel) RPM Sound System
  (CallFunction|SetHovercraftTravelbyPlayerSound(AccordingtoSpeed))
  (CallFunction|SetHovercraftTravelbyRemoteSound(AccordingtoSpeed)))

(fn ConstructionScript
  (Utilities|FlowControl|Sequence
    (:then_0
      (Utilities|Array|Clear (Variables|Default|GetlifeStocks))
      (Utilities|Array|Clear (Variables|Default|GetTurbines))
      (Utilities|Array|Clear (Variables|Default|GeteggsStock)))
    (:then_1
      (for _array_element (Utilities|Array|MakeArray (Variables|Default|GetTurbine1) (Variables|Default|GetTurbine2) (Variables|Default|GetTurbine3) (Variables|Default|GetTurbine4))
        (bind _asbp_turbine (Utilities|Casting|CastToBP_Turbine (Variables|/Script/Engine.ChildActorComponent|GetChildActor _array_element)))
        (Utilities|Array|Add (Variables|Default|GetTurbines) _asbp_turbine))
      (for _array_element_2 (Utilities|Array|MakeArray (Variables|Default|GetLifeStock) (Variables|Default|GetLifeStock1) (Variables|Default|GetLifeStock2) (Variables|Default|GetLifeStock3))
        (bind _asbp_life_stock_handcar_actor (Utilities|Casting|CastToBP_LifeStockHandcarActor (Variables|/Script/Engine.ChildActorComponent|GetChildActor _array_element_2)))
        (Utilities|Array|Add (Variables|Default|GetlifeStocks) _asbp_life_stock_handcar_actor))
      (for _array_element_3 (Utilities|Array|MakeArray (Variables|Default|GetEggStock) (Variables|Default|GetEggStock1))
        (bind _asbp_egg_stock_handcar_actor (Utilities|Casting|CastToBP_EggStockHandcarActor (Variables|/Script/Engine.ChildActorComponent|GetChildActor _array_element_3)))
        (Utilities|Array|Add (Variables|Default|GeteggsStock) _asbp_egg_stock_handcar_actor))
      (bind _asbp_nitro_handcar_actor (Utilities|Casting|CastToBP_NitroHandcarActor (Variables|/Script/Engine.ChildActorComponent|GetChildActor (Variables|Default|GetPilot))))
      (Variables|Default|Setnitro _asbp_nitro_handcar_actor)
      (bind _asbp_brake_handcar_actor (Utilities|Casting|CastToBP_BrakeHandcarActor (Variables|/Script/Engine.ChildActorComponent|GetChildActor (Variables|Default|Getbrake_actor))))
      (Variables|Default|Setbrake _asbp_brake_handcar_actor))))

(fn SetHovercraftTravelbyPlayerSound(AccordingtoSpeed)
  (bind _currentspeed (Variables|Default|GetcurrentSpeed))
  ;[1 1 1] Set Hovercraft Travel By Player Sound (According To Speed)
  (if (>= _currentspeed 0.0)
    ;;[1 0 0.4608] Layer 1 Pitch
    (Audio|Parameter|SetFloatParameter (Variables|Default|GetHovercraft_Travel_By_Player_SFX) "Layer 1 Pitch" (Math|Float|MapRangeClamped _currentspeed 0.0 3.5e+02 -8.3 0.0) :!class /Script/AudioExtensions.AudioParameterControllerInterface)
    ;;[0 0.3916 1] Layer 1 Volume
    (Audio|Parameter|SetFloatParameter (Variables|Default|GetHovercraft_Travel_By_Player_SFX) "Layer 1 Volume" (Math|Float|MapRangeClamped _currentspeed 0.0 3.5e+02 0.45 1.0) :!class /Script/AudioExtensions.AudioParameterControllerInterface)
    ;;[1 0 0.4608] Layer 2 Pitch
    (Audio|Parameter|SetFloatParameter (Variables|Default|GetHovercraft_Travel_By_Player_SFX) "Layer 2 Pitch" (Math|Float|MapRangeClamped _currentspeed 0.0 3.5e+02 -3.0 0.0) :!class /Script/AudioExtensions.AudioParameterControllerInterface)
    ;;[0 0.3916 1] Layer 2 Volume
    (Audio|Parameter|SetFloatParameter (Variables|Default|GetHovercraft_Travel_By_Player_SFX) "Layer 2 Volume" (Math|Float|MapRangeClamped _currentspeed 0.0 3.5e+02 0.45 1.1) :!class /Script/AudioExtensions.AudioParameterControllerInterface)
    ;;[1 0 0.4608] Layer 3 Pitch
    (Audio|Parameter|SetFloatParameter (Variables|Default|GetHovercraft_Travel_By_Player_SFX) "Layer 3 Pitch" (Math|Float|MapRangeClamped _currentspeed 0.0 3.5e+02 -2.1 1.5) :!class /Script/AudioExtensions.AudioParameterControllerInterface)
    ;;[0 0.3916 1] Layer 3 Volume
    (Audio|Parameter|SetFloatParameter (Variables|Default|GetHovercraft_Travel_By_Player_SFX) "Layer 3 Volume" (Math|Float|MapRangeClamped _currentspeed 0.0 3.5e+02 0.45 1.25) :!class /Script/AudioExtensions.AudioParameterControllerInterface)
    ;;[1 0 0.4608] Layer 4 Pitch
    (Audio|Parameter|SetFloatParameter (Variables|Default|GetHovercraft_Travel_By_Player_SFX) "Layer 4 Pitch" (Math|Float|MapRangeClamped _currentspeed 0.0 3.5e+02 -3.0 2.5) :!class /Script/AudioExtensions.AudioParameterControllerInterface)
    ;;[0 0.3916 1] Layer 4 Volume
    (Audio|Parameter|SetFloatParameter (Variables|Default|GetHovercraft_Travel_By_Player_SFX) "Layer 4 Volume" (Math|Float|MapRangeClamped _currentspeed 0.0 3.5e+02 0.25 0.75) :!class /Script/AudioExtensions.AudioParameterControllerInterface)
    (else
      (Audio|Parameter|SetFloatParameter (Variables|Default|GetHovercraft_Travel_By_Player_SFX) "Layer 1 Pitch" (Math|Float|MapRangeClamped _currentspeed 0.0 -3.5e+02 -8.3 0.0) :!class /Script/AudioExtensions.AudioParameterControllerInterface)
      (Audio|Parameter|SetFloatParameter (Variables|Default|GetHovercraft_Travel_By_Player_SFX) "Layer 1 Volume" (Math|Float|MapRangeClamped _currentspeed 0.0 -3.5e+02 0.45 1.0) :!class /Script/AudioExtensions.AudioParameterControllerInterface)
      (Audio|Parameter|SetFloatParameter (Variables|Default|GetHovercraft_Travel_By_Player_SFX) "Layer 2 Pitch" (Math|Float|MapRangeClamped _currentspeed 0.0 -3.5e+02 -3.0 0.0) :!class /Script/AudioExtensions.AudioParameterControllerInterface)
      (Audio|Parameter|SetFloatParameter (Variables|Default|GetHovercraft_Travel_By_Player_SFX) "Layer 2 Volume" (Math|Float|MapRangeClamped _currentspeed 0.0 -3.5e+02 0.45 1.1) :!class /Script/AudioExtensions.AudioParameterControllerInterface)
      (Audio|Parameter|SetFloatParameter (Variables|Default|GetHovercraft_Travel_By_Player_SFX) "Layer 3 Pitch" (Math|Float|MapRangeClamped _currentspeed 0.0 -3.5e+02 -2.1 1.5) :!class /Script/AudioExtensions.AudioParameterControllerInterface)
      (Audio|Parameter|SetFloatParameter (Variables|Default|GetHovercraft_Travel_By_Player_SFX) "Layer 3 Volume" (Math|Float|MapRangeClamped _currentspeed 0.0 -3.5e+02 0.45 1.25) :!class /Script/AudioExtensions.AudioParameterControllerInterface)
      (Audio|Parameter|SetFloatParameter (Variables|Default|GetHovercraft_Travel_By_Player_SFX) "Layer 4 Pitch" (Math|Float|MapRangeClamped _currentspeed 0.0 -3.5e+02 -3.0 2.5) :!class /Script/AudioExtensions.AudioParameterControllerInterface)
      (Audio|Parameter|SetFloatParameter (Variables|Default|GetHovercraft_Travel_By_Player_SFX) "Layer 4 Volume" (Math|Float|MapRangeClamped _currentspeed 0.0 -3.5e+02 0.25 0.75) :!class /Script/AudioExtensions.AudioParameterControllerInterface))))

(fn SetHovercraftTravelbyRemoteSound(AccordingtoSpeed)
  (bind _currentspeed (Variables|Default|GetcurrentSpeed))
  ;[1 1 1] Set Hovercraft Travel By  Remote Sound (According To Speed)
  (if (>= _currentspeed 0.0)
    ;;[1 0 0.4608] Layer 1 Pitch
    (Audio|Parameter|SetFloatParameter (Variables|Default|GetMSS_HoverCraft_Travel_By_Remote) "Layer 1 Pitch" (Math|Float|MapRangeClamped _currentspeed 0.0 3.5e+02 -8.3 0.0) :!class /Script/AudioExtensions.AudioParameterControllerInterface)
    ;;[0 0.3916 1] Layer 1 Volume
    (Audio|Parameter|SetFloatParameter (Variables|Default|GetMSS_HoverCraft_Travel_By_Remote) "Layer 1 Volume" (Math|Float|MapRangeClamped _currentspeed 0.0 3.5e+02 0.45 1.0) :!class /Script/AudioExtensions.AudioParameterControllerInterface)
    ;;[1 0 0.4608] Layer 2 Pitch
    (Audio|Parameter|SetFloatParameter (Variables|Default|GetMSS_HoverCraft_Travel_By_Remote) "Layer 2 Pitch" (Math|Float|MapRangeClamped _currentspeed 0.0 3.5e+02 -3.0 0.0) :!class /Script/AudioExtensions.AudioParameterControllerInterface)
    ;;[0 0.3916 1] Layer 2 Volume
    (Audio|Parameter|SetFloatParameter (Variables|Default|GetMSS_HoverCraft_Travel_By_Remote) "Layer 2 Volume" (Math|Float|MapRangeClamped _currentspeed 0.0 3.5e+02 0.45 1.1) :!class /Script/AudioExtensions.AudioParameterControllerInterface)
    ;;[1 0 0.4608] Layer 3 Pitch
    (Audio|Parameter|SetFloatParameter (Variables|Default|GetMSS_HoverCraft_Travel_By_Remote) "Layer 3 Pitch" (Math|Float|MapRangeClamped _currentspeed 0.0 3.5e+02 -2.1 1.5) :!class /Script/AudioExtensions.AudioParameterControllerInterface)
    ;;[0 0.3916 1] Layer 3 Volume
    (Audio|Parameter|SetFloatParameter (Variables|Default|GetMSS_HoverCraft_Travel_By_Remote) "Layer 3 Volume" (Math|Float|MapRangeClamped _currentspeed 0.0 3.5e+02 0.45 1.25) :!class /Script/AudioExtensions.AudioParameterControllerInterface)
    ;;[1 0 0.4608] Layer 4 Pitch
    (Audio|Parameter|SetFloatParameter (Variables|Default|GetMSS_HoverCraft_Travel_By_Remote) "Layer 4 Pitch" (Math|Float|MapRangeClamped _currentspeed 0.0 3.5e+02 -3.0 2.5) :!class /Script/AudioExtensions.AudioParameterControllerInterface)
    ;;[0 0.3916 1] Layer 4 Volume
    (Audio|Parameter|SetFloatParameter (Variables|Default|GetMSS_HoverCraft_Travel_By_Remote) "Layer 4 Volume" (Math|Float|MapRangeClamped _currentspeed 0.0 3.5e+02 0.25 0.75) :!class /Script/AudioExtensions.AudioParameterControllerInterface)
    (else
      (Audio|Parameter|SetFloatParameter (Variables|Default|GetMSS_HoverCraft_Travel_By_Remote) "Layer 1 Pitch" (Math|Float|MapRangeClamped _currentspeed 0.0 -3.5e+02 -8.3 0.0) :!class /Script/AudioExtensions.AudioParameterControllerInterface)
      (Audio|Parameter|SetFloatParameter (Variables|Default|GetMSS_HoverCraft_Travel_By_Remote) "Layer 1 Volume" (Math|Float|MapRangeClamped _currentspeed 0.0 -3.5e+02 0.45 1.0) :!class /Script/AudioExtensions.AudioParameterControllerInterface)
      (Audio|Parameter|SetFloatParameter (Variables|Default|GetMSS_HoverCraft_Travel_By_Remote) "Layer 2 Pitch" (Math|Float|MapRangeClamped _currentspeed 0.0 -3.5e+02 -3.0 0.0) :!class /Script/AudioExtensions.AudioParameterControllerInterface)
      (Audio|Parameter|SetFloatParameter (Variables|Default|GetMSS_HoverCraft_Travel_By_Remote) "Layer 2 Volume" (Math|Float|MapRangeClamped _currentspeed 0.0 -3.5e+02 0.45 1.1) :!class /Script/AudioExtensions.AudioParameterControllerInterface)
      (Audio|Parameter|SetFloatParameter (Variables|Default|GetMSS_HoverCraft_Travel_By_Remote) "Layer 3 Pitch" (Math|Float|MapRangeClamped _currentspeed 0.0 -3.5e+02 -2.1 1.5) :!class /Script/AudioExtensions.AudioParameterControllerInterface)
      (Audio|Parameter|SetFloatParameter (Variables|Default|GetMSS_HoverCraft_Travel_By_Remote) "Layer 3 Volume" (Math|Float|MapRangeClamped _currentspeed 0.0 -3.5e+02 0.45 1.25) :!class /Script/AudioExtensions.AudioParameterControllerInterface)
      (Audio|Parameter|SetFloatParameter (Variables|Default|GetMSS_HoverCraft_Travel_By_Remote) "Layer 4 Pitch" (Math|Float|MapRangeClamped _currentspeed 0.0 -3.5e+02 -3.0 2.5) :!class /Script/AudioExtensions.AudioParameterControllerInterface)
      (Audio|Parameter|SetFloatParameter (Variables|Default|GetMSS_HoverCraft_Travel_By_Remote) "Layer 4 Volume" (Math|Float|MapRangeClamped _currentspeed 0.0 -3.5e+02 0.25 0.75) :!class /Script/AudioExtensions.AudioParameterControllerInterface))))