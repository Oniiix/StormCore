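; Lightning hazard actor Blueprint that supplies the sound and visuals for a telegraphed lightning strike.
; BeginPlay binds handlers to the call and strike events.
; The call plays a warning sound and a Niagara effect whose radius and duration come from the actor's damage radius and preview time.
; The strike plays its own sound and effect at the actor's location, plus a fading ground decal.
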(event Custom|Thunder_Call
  ;[1 0.6062 0] Thunder_Call
  (Audio|PlaySoundatLocation "/Game/05_Audio/SFX/MetaSounds/Weather_Condition/Agressive_Lightning/Agressive_Lightning_Stage1/MSS_Agressive_Lightning_Stage1.MSS_Agressive_Lightning_Stage1" (Transformation|GetActorLocation) "0, 0, 0" 1.0 1.0 0.0 0 0 0 0)
  (bind _returnvalue (Niagara|SpawnSystematLocation "/Game/04_FX/NS/Weather/NS_Thunder_Call.NS_Thunder_Call" (Transformation|GetWorldLocation (Variables|Transformation|GetRootComponent))))
  (bind _output_get (Variables|Default|SetThunderCall _returnvalue))
  (Niagara|SetNiagaraVariable(Float) _output_get "Radius" (Class|Lightning|GetRadiusDamage))
  (Niagara|SetNiagaraVariable(Float) _output_get "Call_Duration" (Class|Lightning|GetPreviewTime)))

(event Custom|Thunder_Strike
  ;[0 0.7516 1] Thunder
  (Audio|PlaySoundatLocation "/Game/05_Audio/SFX/MetaSounds/Weather_Condition/Agressive_Lightning/Agressive_Lightning_Stage2/MSS_Agressive_Lightning_Stage2.MSS_Agressive_Lightning_Stage2" (Transformation|GetActorLocation) "0, 0, 0" 1.0 1.0 0.0 0 0 0 0)
  (Niagara|SpawnSystematLocation "/Game/04_FX/NS/Weather/NS_ThunderVar3.NS_ThunderVar3" (Transformation|GetActorLocation))
  (bind _returnvalue (Rendering|Decal|SpawnDecalatLocation "/Game/04_FX/Decals/MI_Decals_thunder.MI_Decals_thunder" (Variables|Default|GetDecal%20Size) (Transformation|GetActorLocation) "-90.000000,0.000000,0.000000" 0.0))
  (Rendering|Components|Decal|SetFadeOut _returnvalue 1.0 1.0 true))

(event EventBeginPlay
  (EventDispatchers|BindEventtoOnCall (delegate Custom|Thunder_Call))
  ;[0 0.7516 1] Thunder
  (EventDispatchers|BindEventtoOnLightningStrike (delegate Custom|Thunder_Strike)))

(fn ConstructionScript)