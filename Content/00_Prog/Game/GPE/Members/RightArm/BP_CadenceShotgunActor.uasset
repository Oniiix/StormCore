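; Cadence shotgun actor for the right-arm member, providing the weapon's visual and audio feedback.
; On BeginPlay it binds to shoot and fail events, playing a muzzle Niagara effect and success sound on a shot, or a jam sound on failure.
; The muzzle effect receives shot count and direction.
; Actor hits spawn impact effects chosen by surface type and oriented to the impact normal.
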(event Custom|onFailed_Event
  (Audio|PlaySoundatLocation "/Game/05_Audio/SFX/MetaSounds/Player/Weapons/Right_Arm/Shotgun/Shotgun_Jam/MSS_Shotgun_Jam.MSS_Shotgun_Jam" (Transformation|GetActorLocation) "0, 0, 0" 1.0 1.0 0.0 0 0 0 0))

(event Custom|Shoot
  (params (_startPosition :type Vector%20%28by%20ref%29) (_direction :type Vector%20%28by%20ref%29))
  (bind _returnvalue (Niagara|SpawnSystematLocation "/Game/04_FX/NS/Player/ShootGun/NS_ShootGun_Shoot.NS_ShootGun_Shoot" _startPosition))
  (Class|NiagaraComponent|SetVariableInt _returnvalue "NB_projectile" (Math|Float|Truncate (Variables|Default|GetnbOfShot)))
  (Niagara|SetNiagaraVariable(Vector3) _returnvalue "Dir" _direction)
  (Audio|PlaySoundatLocation "/Game/05_Audio/SFX/MetaSounds/Player/Weapons/Right_Arm/Shotgun/Shotgun_Success/MSS_Shotgun_Success.MSS_Shotgun_Success" (Transformation|GetActorLocation) "0, 0, 0" 1.0 1.0 0.0 0 0 0 0))

(event Custom|OnActorHit_Event
  (params (SelfActor :type Actor%20Object%20Reference) (OtherActor :type Actor%20Object%20Reference) (NormalImpulse :type Vector) (Hit :type Hit%20Result%20Structure%20%28by%20ref%29))
  (bind (_bblockinghit _binitialoverlap _time _distance _location _impactpoint _normal _impactnormal) (Collision|BreakHitResult Hit))
  (bind _returnvalue (Niagara|SpawnSystematLocation (Utilities|Select :Index (Collision|GetSurfaceType Hit) :SurfaceType_Default "/Game/04_FX/NS/Impacts/NS_Impact_Concrete.NS_Impact_Concrete" :SurfaceType1 "/Game/04_FX/NS/Impacts/NS_Impact_Grass.NS_Impact_Grass" :SurfaceType2 "/Game/04_FX/NS/Impacts/NS_Impact_Concrete.NS_Impact_Concrete" :SurfaceType3 0 :SurfaceType4 "/Game/04_FX/NS/Impacts/NS_Impact_Concrete.NS_Impact_Concrete" :SurfaceType5 "/Game/04_FX/NS/Impacts/NS_Impact_Concrete.NS_Impact_Concrete" :SurfaceType6 "/Game/04_FX/NS/Impacts/NS_Impact_Metal.NS_Impact_Metal" :SurfaceType7 "/Game/04_FX/NS/Impacts/NS_Impact_Grass.NS_Impact_Grass" :SurfaceType8 0 :SurfaceType9 "/Game/04_FX/NS/Impacts/NS_Impact_Grass.NS_Impact_Grass" :SurfaceType10 0 :SurfaceType11 "/Game/04_FX/NS/Enemies/Global/NS_Blood_Hit.NS_Blood_Hit" :SurfaceType12 "/Game/04_FX/NS/Impacts/NS_Impact_Metal.NS_Impact_Metal" :SurfaceType13 0 :SurfaceType14 0 :SurfaceType15 0 :SurfaceType16 0 :SurfaceType17 "/Game/04_FX/NS/Impacts/NS_Impact_Flesh.NS_Impact_Flesh" :SurfaceType18 0) _location))
  (Niagara|SetNiagaraVariable(Vector3) _returnvalue "Impact_Orientation" _impactnormal))

(event Custom|onReductionUpdate_Event
  (params (_reductionRatio :type Float%20%28single-precision%29)))

(event EventBeginPlay
  (EventDispatchers|BindEventtoOnShoot (delegate Custom|Shoot))
  (EventDispatchers|AssignOnFailed (delegate Custom|onFailed_Event))
  (Collision|AssignOnActorHit (delegate Custom|OnActorHit_Event)))

(event Collision|EventActorBeginOverlap
  (params (OtherActor :type Actor%20Object%20Reference)))

(event EventTick
  (params (DeltaSeconds :type Float%20%28single-precision%29)))

(fn ConstructionScript)