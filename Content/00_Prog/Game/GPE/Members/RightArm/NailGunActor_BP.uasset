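; Nail gun weapon actor for the right arm member, handling the visual and audio feedback of shots and hits.
; BeginPlay binds to inherited shoot, projectile and hit events to spawn muzzle and projectile Niagara effects and play fire sounds.
; Hits choose an impact effect by physical surface and orient it to the impact normal.
; Old charge and explosion logic remains disconnected, though hits still clear the charging sound.
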(event Custom|HIT
  (params (_results :type Hit%20Result%20Structure%20%28by%20ref%29))
  (bind (_bblockinghit _binitialoverlap _time _distance _location _impactpoint _normal _impactnormal) (Collision|BreakHitResult _results))
  (bind _returnvalue (Niagara|SpawnSystematLocation (Utilities|Select :Index (Collision|GetSurfaceType _results) :SurfaceType_Default "/Game/04_FX/NS/Impacts/NS_Impact_Concrete.NS_Impact_Concrete" :SurfaceType1 "/Game/04_FX/NS/Impacts/NS_Impact_Grass.NS_Impact_Grass" :SurfaceType2 "/Game/04_FX/NS/Impacts/NS_Impact_Concrete.NS_Impact_Concrete" :SurfaceType3 0 :SurfaceType4 "/Game/04_FX/NS/Impacts/NS_Impact_Concrete.NS_Impact_Concrete" :SurfaceType5 "/Game/04_FX/NS/Impacts/NS_Impact_Concrete.NS_Impact_Concrete" :SurfaceType6 "/Game/04_FX/NS/Impacts/NS_Impact_Metal.NS_Impact_Metal" :SurfaceType7 "/Game/04_FX/NS/Impacts/NS_Impact_Grass.NS_Impact_Grass" :SurfaceType8 0 :SurfaceType9 "/Game/04_FX/NS/Impacts/NS_Impact_Grass.NS_Impact_Grass" :SurfaceType10 0 :SurfaceType11 "/Game/04_FX/NS/Enemies/Global/NS_Blood_Hit.NS_Blood_Hit" :SurfaceType12 "/Game/04_FX/NS/Impacts/NS_Impact_Metal.NS_Impact_Metal" :SurfaceType13 "/Game/04_FX/NS/Impacts/NS_Impact_Grass.NS_Impact_Grass" :SurfaceType14 0 :SurfaceType15 "/Game/04_FX/NS/Impacts/NS_Impact_Concrete.NS_Impact_Concrete" :SurfaceType16 0 :SurfaceType17 "/Game/04_FX/NS/Impacts/NS_Impact_Flesh.NS_Impact_Flesh" :SurfaceType18 "/Game/04_FX/NS/Enemies/Global/NS_Blood_Hit.NS_Blood_Hit") _location))
  (bind _output_get (Variables|Default|SetNiagara_ref _returnvalue))
  (Utilities|IsValid _output_get
    (:Is%20Valid
      (Niagara|SetNiagaraVariable(Vector3) _output_get "Impact_Orientation" _impactnormal)
      ;[1 0.1602 0] Rajouté par Thibaud - Prog
      (bind _charging_sound (Variables|Default|GetCharging%20Sound)
        (:then
          (Audio|Components|Audio|Stop _charging_sound)
          (Components|DestroyComponent _charging_sound))
        (:else)))))

(event Custom|Nailgun_SimpleShoot
  (params (_startPosition :type Vector%20%28by%20ref%29) (_direction :type Vector%20%28by%20ref%29))
  (Niagara|SpawnSystematLocation "/Game/04_FX/NS/Player/Nailgun/NS_NailGunShoot.NS_NailGunShoot" _startPosition (Math|Rotator|MakeRotfromX _direction))
  (Audio|PlaySoundatLocation "/Game/05_Audio/SFX/MetaSounds/Player/Weapons/Right_Arm/Nailgun/NailGun_Fire_v3/MSS_Nailgun_Fire_v3.MSS_Nailgun_Fire_v3" _startPosition "0, 0, 0" 1.0 1.0 0.0 0 0 0 0)
  (Audio|PlaySound2D "/Game/05_Audio/SFX/MetaSounds/Player/Weapons/Right_Arm/Nailgun/NailGun_Fire_v3/MSS_Nailgun_Fire_v3_Tail.MSS_Nailgun_Fire_v3_Tail" 1.0 1.0 0.0 0 0 false))

(event Custom|onProjectileGo_Event
  (params (_startPosition :type Vector%20%28by%20ref%29) (_direction :type Vector%20%28by%20ref%29))
  (Niagara|SpawnSystematLocation "/Game/04_FX/NS/Player/Nailgun/NS_NailGun_Projectile.NS_NailGun_Projectile" _startPosition (Math|Rotator|MakeRotfromX _direction)))

(event EventBeginPlay
  (EventDispatchers|BindEventtoOnShoot (delegate Custom|Nailgun_SimpleShoot))
  (EventDispatchers|BindEventtoOnHit (delegate Custom|HIT))
  (EventDispatchers|AssignOnProjectileGo (delegate Custom|onProjectileGo_Event)))

(event Collision|EventActorBeginOverlap
  (params (OtherActor :type Actor%20Object%20Reference)))

(event EventTick
  (params (DeltaSeconds :type Float%20%28single-precision%29)))

(fn ConstructionScript)