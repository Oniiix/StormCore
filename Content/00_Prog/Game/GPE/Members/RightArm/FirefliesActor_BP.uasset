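; Fireflies right-arm weapon actor that supplies the shooting VFX and audio feedback for the player.
; On BeginPlay it binds to its shoot events, spawning a directional Niagara burst on each shot.
; Auto fire starts one sound attached to the character mesh, guarded by a DoOnce; release fades it out, plays a tail and resets the guard.
; Single shots play a shot sound at the player's location plus a 2D tail.
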(event Custom|onShoot_Event
  (params (_startPosition :type Vector%20%28by%20ref%29) (_direction :type Vector%20%28by%20ref%29))
  (bind _returnvalue (Niagara|SpawnSystematLocation "/Game/04_FX/NS/Player/FireFlies/NS_FireFlies_Shoot.NS_FireFlies_Shoot" _startPosition))
  (Niagara|SetNiagaraVariable(Vector3) _returnvalue "Dir" _direction))

(event Custom|onSingleShoot_Event
  ;[1 1 1] Single Shot Sound
  (Audio|PlaySoundatLocation "/Game/05_Audio/SFX/MetaSounds/Player/Weapons/Right_Arm/Fireflies/Fireflies_Fire_Single/MSS_Fireflies_Fire_Single.MSS_Fireflies_Fire_Single" (Transformation|GetActorLocation (Game|GetPlayerCharacter 0)) "0, 0, 0" 1.0 1.0 0.0 0 0 0 0)
  (Audio|PlaySound2D "/Game/05_Audio/SFX/MetaSounds/Player/Weapons/Right_Arm/Fireflies/Fireflies_Fire_Single/MSS_Fireflies_Fire_Single_Tail_Stereo.MSS_Fireflies_Fire_Single_Tail_Stereo" 1.0 1.0 0.0 0 0))

(event Custom|onAutoShoot_Event
  ;[1 1 1] Auto Shoot Sound
  (Utilities|FlowControl|DoOnce false
    (:Completed
      (bind _asmain_character_bp (Utilities|Casting|CastToMainCharacter_BP (Game|GetPlayerCharacter 0)))
      (bind _output_get (Variables|Default|SetAs%20Main%20Character%20BP _asmain_character_bp))
      (bind _returnvalue (Audio|SpawnSoundAttached "/Game/05_Audio/SFX/MetaSounds/Player/Weapons/Right_Arm/Fireflies/Fireflies_Fire_Auto_v2/MSS_Fireflies_Fire_Auto_v2.MSS_Fireflies_Fire_Auto_v2" (Variables|/Script/Engine.Character|GetMesh _output_get) "arm_modules_Socket_r" "0, 0, 0" "0, 0, 0" "KeepRelativeOffset" false 1.0 1.0 0.0 0 0))
      (Variables|Default|SetFireFlies%20Fire%20Auto%20Shot%20Sound _returnvalue))))

(event Custom|onAutoRelease_Event
  ;[1 1 1] Auto Shoot Sound Ending
  (Utilities|IsValid (Variables|Default|GetFireFlies%20Fire%20Auto%20Shot%20Sound)
    (:Is%20Valid
      (Audio|Components|Audio|FadeOut (Variables|Default|GetFireFlies%20Fire%20Auto%20Shot%20Sound) 0.2 0.0 "SCurve" :!class /Script/Engine.AudioComponent)
      (Variables|Default|SetFireFlies%20Fire%20Auto%20Shot%20Sound 0)
      (Audio|PlaySound2D "/Game/05_Audio/SFX/MetaSounds/Player/Weapons/Right_Arm/Fireflies/Fireflies_Fire_Single/MSS_Fireflies_Fire_Single_Tail_Stereo.MSS_Fireflies_Fire_Single_Tail_Stereo" 1.0 1.0 0.0 0 0)
      ;[1 1 1] Auto Shoot Sound
      (Utilities|FlowControl|DoOnce false) ; enters at Reset
    )))

(event EventBeginPlay
  (EventDispatchers|AssignOnShoot (delegate Custom|onShoot_Event))
  ;[1 1 1] Auto Shoot Sound
  (EventDispatchers|BindEventtoOnAutoShoot (delegate Custom|onAutoShoot_Event))
  ;[1 1 1] Auto Shoot Sound Ending
  (EventDispatchers|BindEventtoOnAutoRelease (delegate Custom|onAutoRelease_Event))
  ;[1 1 1] Single Shot Sound
  (EventDispatchers|BindEventtoOnSingleShoot (delegate Custom|onSingleShoot_Event)))

(event Collision|EventActorBeginOverlap
  (params (OtherActor :type Actor%20Object%20Reference)))

(event EventTick
  (params (DeltaSeconds :type Float%20%28single-precision%29)))

(fn ConstructionScript)