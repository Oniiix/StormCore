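; Snap flash actor for the left-arm member, providing the visual and audio feedback of its explosion.
; On the explosion event it spawns a Niagara burst and moves a light there: point light on a hit, spot light otherwise.
; A sped-up timeline drives that light's intensity, then hides it, while a sound plays at the point light's location.
; The shoot feedback is bound but empty.
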(event Custom|Feedback_Explosion
  (params (_hit :type Boolean) (_position :type Vector%20%28by%20ref%29) (_direction :type Vector%20%28by%20ref%29) (_impactResult :type Hit%20Result%20Structure))
  (Niagara|SpawnSystematLocation "/Game/04_FX/NS/Player/SnapFlash/NS_SnapFlash_Burst.NS_SnapFlash_Burst" _position)
  (if _hit
    (Variables|Default|Setlight%20Type (Variables|Default|GetPointLight))
    (else
      (Variables|Default|Setlight%20Type (Variables|Default|GetSpotLight))))
  (Transformation|SetWorldLocation (Variables|Default|Getlight%20Type) _position false false)
  (Transformation|SetWorldRotation (Variables|Default|Getlight%20Type) (Math|Rotator|MakeRotfromX _direction) false false)
  (Rendering|SetVisibility (Variables|Default|Getlight%20Type) true false)
  (Components|Timeline|SetPlayRate (Variables|Default|GetTL_Flash) 8.0)
  (Utilities|FlowControl|Sequence
    (:then_0
      (bind _flash (Timeline|TL_Flash PlayFromStart)
        (:Update
          (Rendering|Components|Light|SetIntensity (Variables|Default|Getlight%20Type) (* _flash (Variables|Default|GetIntensity))))
        (:Finished
          (Rendering|SetVisibility (Variables|Default|Getlight%20Type) false false))))
    (:then_1
      (Audio|PlaySoundatLocation "/Game/05_Audio/SFX/MetaSounds/Player/Weapons/Left_Arm/Snap_Flash/MSS_Snap_Flash.MSS_Snap_Flash" (Transformation|GetWorldLocation (Variables|Default|GetPointLight)) "0, 0, 0" 1.0 1.0 0.0 0 0 0 0))))

(event Custom|Feedback_Shoot_Direction
  (params (_startPosition :type Vector%20%28by%20ref%29) (_direction :type Vector%20%28by%20ref%29)))

(event EventBeginPlay
  (EventDispatchers|BindEventtoOnExplosion (delegate Custom|Feedback_Explosion))
  (EventDispatchers|BindEventtoOnShoot (delegate Custom|Feedback_Shoot_Direction)))

(event Collision|EventActorBeginOverlap
  (params (OtherActor :type Actor%20Object%20Reference)))

(event EventTick
  (params (DeltaSeconds :type Float%20%28single-precision%29)))

(fn ConstructionScript)