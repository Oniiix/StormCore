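; Test actor for attaching overlapping actors to an object with a spinning cube.
; Tick adds a fixed relative rotation to the Cube each frame, without delta-time scaling.
; Entering the Box attaches any actor to this one, keeping its world transform, and clears CanMOve on a PlayerMover_BP.
; Leaving the Box detaches the actor and sets CanMOve back to true.
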(event OnComponentBeginOverlap(Box)
  (params (OverlappedComponent :type Primitive%20Component%20Object%20Reference) (OtherActor :type Actor%20Object%20Reference) (OtherComp :type Primitive%20Component%20Object%20Reference) (OtherBodyIndex :type Integer) (bFromSweep :type Boolean) (SweepResult :type Hit%20Result%20Structure%20%28by%20ref%29))
  (Transformation|AttachActorToActor OtherActor self "None" "KeepWorld" "KeepWorld" "KeepWorld" false)
  (bind _asplayer_mover_bp (Utilities|Casting|CastToPlayerMover_BP OtherActor))
  (Variables|/Game/00_Prog/Game/TEST/PlayerMover_BP.PlayerMover_BP_C|SetcanMOve _asplayer_mover_bp false))

(event OnComponentEndOverlap(Box)
  (params (OverlappedComponent :type Primitive%20Component%20Object%20Reference) (OtherActor :type Actor%20Object%20Reference) (OtherComp :type Primitive%20Component%20Object%20Reference) (OtherBodyIndex :type Integer))
  (Transformation|DetachFromActor OtherActor "KeepWorld" "KeepWorld" "KeepWorld")
  (bind _asplayer_mover_bp (Utilities|Casting|CastToPlayerMover_BP OtherActor))
  (Variables|/Game/00_Prog/Game/TEST/PlayerMover_BP.PlayerMover_BP_C|SetcanMOve _asplayer_mover_bp true))

(event EventBeginPlay)

(event Collision|EventActorBeginOverlap
  (params (OtherActor :type Actor%20Object%20Reference)))

(event EventTick
  (params (DeltaSeconds :type Float%20%28single-precision%29))
  (Transformation|AddRelativeRotation (Variables|Default|GetCube) "0.000000,1.000000,0.000000" false false))

(fn ConstructionScript)