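; Hitvalue_BP is a test actor that shows a floating hit damage number through a HitTextUI_BP widget and expires after a few seconds.
; InitValue sets the damage text, while AddValue accumulates further damage into the same number.
; Tick moves it along X with a sine-derived Z offset scaled by Speed, and prints a debug value.
; Distance-based widget draw-size scaling is present but disconnected.
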(event EventBeginPlay
  (Actor|SetLifeSpan 3.0)
  (Transformation|SetActorLocation (+ (Transformation|GetActorLocation) "1.000000,0.000000,0.000000") false false))

(event Collision|EventActorBeginOverlap
  (params (OtherActor :type Actor%20Object%20Reference)))

(event EventTick
  (params (DeltaSeconds :type Float%20%28single-precision%29))
  (if (> (Variables|Default|GetRes) 2.0)
    (bind _output_get (Variables|Default|SetRes (+ (Math|Trig|Sin(Radians) DeltaSeconds) (Variables|Default|GetRes))))
    (else
      (Variables|Default|SetRes (- (Math|Trig|Sin(Radians) 0.0) (Variables|Default|GetRes)))))
  (Development|PrintString (Utilities|String|ToString(Float) (+ (Math|Trig|Sin(Radians) DeltaSeconds) (Variables|Default|GetRes))))
  (Transformation|SetActorLocation (+ (Transformation|GetActorLocation) (* (Math|Vector|MakeVector 1.0 0.0 _output_get) (Variables|Default|GetSpeed))) false false))

(fn ConstructionScript)

(fn InitValue
  (params (_value :type Integer))
  (Variables|Default|Setdamage _value)
  (bind _ashit_text_ui_bp (Utilities|Casting|CastToHitTextUI_BP (UserInterface|GetWidget (Variables|Default|GetWidget))))
  (Default|SetHitValue _ashit_text_ui_bp _value))

(fn AddValue
  (params (Value :type Integer))
  (bind _ashit_text_ui_bp (Utilities|Casting|CastToHitTextUI_BP (UserInterface|GetWidget (Variables|Default|GetWidget))))
  (bind _output_get (Variables|Default|Setdamage (+ Value (Variables|Default|Getdamage))))
  (Default|SetHitValue _ashit_text_ui_bp _output_get))