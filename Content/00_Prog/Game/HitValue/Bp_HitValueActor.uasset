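; Floating hit-value actor that drifts a widget beside the impact, sized by a curve of absolute damage.
; BeginPlay offsets it along the player camera's right vector and randomizes vertical drift and speed.
; Tick moves it with a sine bob and an initial speed boost that decays to normal.
; Horizontal distance to the player scales movement through a clamped range whose upper output is its own previous result.
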(event EventTick
  (params (DeltaSeconds :type Float%20%28single-precision%29))
  (bind _amplitude_widget (Variables|Custom|GetAmplitude%20Widget))
  (Variables|Custom|Debug|SetNew%20Height (* _amplitude_widget (- (Math|Trig|Sin(Radians) (* _amplitude_widget (+ DeltaSeconds (Variables|Custom|Debug|GetResult%20Time)))) (Math|Trig|Sin(Radians) (* (Variables|Custom|GetAmplitude%20Widget) (Variables|Custom|Debug|GetResult%20Time))))))
  (Variables|Custom|Debug|SetResult%20Time (+ DeltaSeconds (Variables|Custom|Debug|GetResult%20Time)))
  (CallFunction|UpdateDistanceSpeed)
  (Transformation|AddActorWorldOffset (* (+ (Math|Vector|GetRightVector (Variables|Default|GetCamera_Ref)) (Math|Vector|MakeVector 0.0 0.0 (+ (Variables|Custom|Debug|GetNew%20Height) (Variables|Default|GetRandom_Orient)))) (* (Variables|Custom|GetSpeed%20Moving) (Variables|Default|GetRandom_Speed) (Variables|Default|GetInitial_Speed_Mod) (Variables|Default|GetDistance_Speed_Mod) DeltaSeconds)) false true)
  (if (> (Variables|Default|GetInitial_Speed_Mod) 1.0)
    (Variables|Default|SetInitial_Speed_Mod (Math|Float|Max(Float) (- (Variables|Default|GetInitial_Speed_Mod) (* (Variables|Default|GetInitial_Speed_Mod_LerpTime) DeltaSeconds)) 1.0))))

(event EventBeginPlay
  (bind _damage (Variables|Default|Getdamage))
  (bind _drawsize_curve (Variables|Default|GetDrawsize_Curve))
  (bind _returnvalue (Math|Float|Absolute(Float) _damage))
  (bind _returnvalue_2 (Math|Curves|GetFloatValue _drawsize_curve _returnvalue))
  (bind _asmain_character_bp (Utilities|Casting|CastToMainCharacter_BP (Game|GetPlayerCharacter 0)))
  (Variables|Default|SetCamera_Ref (Variables|/Script/RobotHunter.CustomCameraComponent|Getcamera (Variables|/Script/RobotHunter.MainCharacter|GetcameraComponent _asmain_character_bp)))
  (Variables|Default|SetRandom_Orient (Math|Random|RandomFloatinRange (Variables|Default|GetRandom_Orient_Min) (Variables|Default|GetRandom_Orient_Max)))
  (Variables|Default|SetRandom_Speed (Math|Random|RandomFloatinRange (Variables|Default|GetRandom_Speed_Mod_Min) (Variables|Default|GetRandom_Speed_Mod_Max)))
  (CallFunction|UpdateDistanceSpeed)
  (Transformation|AddActorWorldOffset (* (+ (Math|Vector|GetRightVector (Variables|Default|GetCamera_Ref)) (Math|Vector|MakeVector 0.0 0.0 (+ (Variables|Custom|Debug|GetNew%20Height) (Variables|Default|GetRandom_Orient)))) (* (Variables|Default|GetDistance_Speed_Mod) (Variables|Default|GetInitial_Offset))) false true)
  (Variables|Default|SetInitial_Speed_Mod_Deceleration (/ (Variables|Default|GetInitial_Speed_Mod) (Variables|Default|GetInitial_Speed_Mod_LerpTime)))
  (Utilities|FlowControl|DelayUntilNextTick)
  (Class|WidgetComponent|SetDrawSize (Variables|Default|GetwidgetComponent) (Math|Vector2D|MakeVector2D _returnvalue_2 _returnvalue_2)))

(fn ConstructionScript)

(fn UpdateDistanceSpeed
  (bind _returnvalue (Transformation|GetActorLocation))
  (bind _returnvalue_2 (Game|GetPlayerCharacter 0))
  (bind _returnvalue_3 (Transformation|GetActorLocation _returnvalue_2))
  (Variables|Default|SetDistance_Speed_Mod (Math|Float|MapRangeClamped (Math|Vector|Distance(Vector) (Math|Vector|MakeVector (.x _returnvalue) (.y _returnvalue) 0.0) (Math|Vector|MakeVector (.x _returnvalue_3) (.y _returnvalue_3) 0.0)) (Variables|Default|GetDistance_Min) (Variables|Default|GetDistance_Max) 1.0 (Variables|Default|GetDistance_Speed_Mod))))