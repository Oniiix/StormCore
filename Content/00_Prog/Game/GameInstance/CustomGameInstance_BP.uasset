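; Game instance that runs level transitions between main menu, tutorial, hub and game, plus death, quit and end credits.
; Init binds transition events that play the current HUD's fade, usually triggering the level load when it finishes, and a level-loaded handler fades back in.
; Each transition also crossfades music and ambience through persistent 2D sounds and sound mixes, with looping timers delaying hub audio until prior music stops or P_Hub loads.
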(event Custom|EnterMainMenu
  (bind _hub_music (Variables|Default|GetHub%20Music))
  ;[0 1 0.0615] Enter Main Menu
  (Development|PrintString "ENTER MAIN MENU" true true "(R=1.000000,G=0.274432,B=0.000000,A=1.000000)" 5.0)
  (Input|EnableInput (Game|GetPlayerController 0) 0)
  (Class|GameplayStatics|ClearSoundMixModifiers)
  ;[1 0.695 0] Main Menu Music (1st Play)
  (bind _returnvalue (Audio|SpawnSound2D "/Game/05_Audio/Music/MetaSounds/Main_Menu_Music/MSS_Main_Menu_Music.MSS_Main_Menu_Music" 1.0 1.0 0.0 0 true false))
  (Variables|Default|SetBGM_Menu _returnvalue)
  (Variables|Default|SetHub%20Already%20Visited false)
  ;[1 1 1] Hub Music Fade Out (If Currently Playing)
  (Utilities|IsValid _hub_music
    (:Is%20Valid
      (if (Audio|Components|Audio|IsPlaying _hub_music)
        (Audio|Components|Audio|FadeOut _hub_music 0.5 0.0 "SCurve" :!class /Script/Engine.AudioComponent)))))

(event Custom|Check%20Level%20Change%201
  ;[1 1 1] Hub Global Amb SFX Fade In
  (bind _returnvalue (Game|GetCurrentLevelName true))
  (if (Utilities|Enum|Equal(Enum) _returnvalue "P_Hub")
    (Utilities|Time|ClearandInvalidateTimerbyHandle (stale Custom|onLevelChangeGameToHub_Event _returnvalue))
    (Development|PrintString "RE-INIT SFX AFTER DEATH" true true "(R=0.000000,G=1.000000,B=0.462685,A=1.000000)" 5.0)
    (Class|GameplayStatics|ClearSoundMixModifiers)
    (Audio|Components|Audio|FadeIn (Variables|Default|GetHub%20Global%20Amb%20SFX) 3.0 1.0 0.0 "SCurve" :!class /Script/Engine.AudioComponent)
    ;[1 1 1] Hub Music Fade In
    (Audio|Components|Audio|FadeIn (Variables|Default|GetHub%20Music) 4.0 1.0 0.0 "SCurve" :!class /Script/Engine.AudioComponent)))

(event Custom|onDeathToHub_Event
  ;[1 1 1] Death (To Hub)
  (Development|PrintString "EVENT DEATH TO HUB" true true "(R=1.000000,G=0.274432,B=0.000000,A=1.000000)" 5.0)
  (Audio|PopSoundMixModifier "/Game/05_Audio/SoundClass_Mixes/Radio_OFF_When_Leaving/SCM_Radio_OFF_When_Leaving.SCM_Radio_OFF_When_Leaving")
  (bind (_asbase_frame_bp _fade) (CallFunction|GetBaseFrameandFadeAnimationfromGameHUD))
  (Components|Animation|PlayAnimation _asbase_frame_bp _fade 0.0 1 "Forward" 0.75
    (:then
      (bind _returnvalue (Utilities|Time|SetTimerbyEvent (delegate Custom|Check%20Level%20Change%202) 0.1 true)))))

(event Custom|Check%20Level%20Change%202
  ;[1 1 1] Death (To Hub)
  (bind _returnvalue (Game|GetCurrentLevelName true))
  (if (Utilities|Enum|Equal(Enum) _returnvalue "P_Hub")
    (Utilities|Time|ClearandInvalidateTimerbyHandle (stale Custom|onDeathToHub_Event _returnvalue))
    ;[1 1 1] Hub Global Amb SFX Fade In
    (Audio|Components|Audio|FadeIn (Variables|Default|GetHub%20Global%20Amb%20SFX) 3.0 1.0 0.0 "Linear" :!class /Script/Engine.AudioComponent)
    ;[1 1 1] Hub Music Fade In
    (Audio|Components|Audio|FadeIn (Variables|Default|GetHub%20Music) 4.0 1.0 0.0 "Linear" :!class /Script/Engine.AudioComponent)))

(event Custom|MainToTuto
  (bind _bgm_menu (Variables|Default|GetBGM_Menu))
  ;[1 1 1] Main To Tuto
  (Development|PrintString "MainToTuto" true true "(R=1.000000,G=0.274432,B=0.000000,A=1.000000)" 5.0)
  (Utilities|FlowControl|Sequence
    (:then_0
      (bind (_asbase_frame_bp _fade) (CallFunction|GetBaseFrameandFadeAnimationfromMainHUD))
      (Components|Animation|PlayAnimation _asbase_frame_bp _fade 0.0 1 "Forward" 0.75
        (:Finished
          (Default|CallOnLevelLoad)
          ;;[1 1 1] (Reinit SFX After Death)
          (Audio|PopSoundMixModifier "/Game/05_Audio/SoundClass_Mixes/Day_Message/SCM_Day_Message1.SCM_Day_Message1")
          (Audio|PopSoundMixModifier "/Game/05_Audio/SoundClass_Mixes/Day_Message/SCM_Day_Message2.SCM_Day_Message2"))))
    (:then_1
      (Audio|PlaySound2D "/Game/05_Audio/SFX/MetaSounds/UI/Main_Menu/Positive/v2/MSS_UI_Main_Menu_Positive_v2.MSS_UI_Main_Menu_Positive_v2" 1.0 1.0 0.0 0 0)
      ;[1 1 1] Game Amb SFX Fade Out
      (bind _returnvalue (Actor|GetActorOfClass "/Game/06_Tech/Weather/BP/BP_Atmosphere.BP_Atmosphere_C"))
      (Utilities|IsValid (Variables|/Game/06_Tech/Weather/BP/BP_Atmosphere.BP_Atmosphere_C|GetSFX_MainMenu_Layer1 _returnvalue)
        (:Is%20Valid
          (Audio|Components|Audio|FadeOut (Variables|/Game/06_Tech/Weather/BP/BP_Atmosphere.BP_Atmosphere_C|GetSFX_MainMenu_Layer1 _returnvalue) 1.5 0.0 "Linear" :!class /Script/Engine.AudioComponent))
        (:Is%20Not%20Valid
          _))
      (Utilities|IsValid (Variables|/Game/06_Tech/Weather/BP/BP_Atmosphere.BP_Atmosphere_C|GetSFX_MainMenu_Layer2 _returnvalue)
        (:Is%20Valid
          (Audio|Components|Audio|FadeOut (Variables|/Game/06_Tech/Weather/BP/BP_Atmosphere.BP_Atmosphere_C|GetSFX_MainMenu_Layer2 _returnvalue) 1.5 0.0 "Linear" :!class /Script/Engine.AudioComponent)
          (Audio|PushSoundMixModifier "/Game/05_Audio/SoundClass_Mixes/Main_Menu_Lightnings_Fade_Out/SCM_Main_Menu_Lightnings_Fade_Out.SCM_Main_Menu_Lightnings_Fade_Out")
          ;[1 0.695 0] Start Game Music SFX
          (bind _returnvalue_2 (Audio|SpawnSound2D "/Game/05_Audio/Music/MetaSounds/Main_Menu_Music/MSS_Start_Music_FX_JGoldsmith_Chord_v2.MSS_Start_Music_FX_JGoldsmith_Chord_v2" 1.0 1.0 0.0 0 true false))
          (Variables|Default|SetStart%20Game%20Music%20FX _returnvalue_2)
          ;[1 1 1] Main Menu Music Fade Out
          (Utilities|IsValid _bgm_menu
            (:Is%20Valid
              (Audio|Components|Audio|FadeOut _bgm_menu 1.6 0.0 "SCurve" :!class /Script/Engine.AudioComponent))))))))

(event Custom|onLevelChangeTutoToHub_Event_0
  (bind _returnvalue (Subsystems|GetSaveManagerSubsystem))
  (bind _returnvalue_2 (Class|SaveManagerSubsystem|GetCurrentSave _returnvalue))
  ;[1 1 1] Tuto to Hub
  (Development|PrintString "TutoToHub" true true "(R=1.000000,G=0.274432,B=0.000000,A=1.000000)" 5.0)
  (Utilities|FlowControl|Sequence
    (:then_0
      (bind (_asbase_frame_bp _fade) (CallFunction|GetBaseFrameandFadeAnimationfromGameHUD))
      (Components|Animation|PlayAnimation _asbase_frame_bp _fade 0.0 1 "Forward" 0.75
        (:then
          (Audio|PushSoundMixModifier "/Game/05_Audio/SoundClass_Mixes/Quit_Tuto/SCM_Quit_Tuto.SCM_Quit_Tuto"))
        (:Finished
          (Default|CallOnLevelLoad)
          (Audio|PopSoundMixModifier "/Game/05_Audio/SoundClass_Mixes/Quit_Tuto/SCM_Quit_Tuto.SCM_Quit_Tuto"))))
    (:then_1
      (Class|CustomGameInstance|SetinTutorial false)
      (Class|GameplaySave|SetIsTutorial _returnvalue_2 false)
      (Class|GameplaySave|SaveGameplay _returnvalue_2 0 1))
    (:then_2
      ;[1 1 1] Game Amb SFX Fade Out
      (bind _returnvalue_3 (Actor|GetActorOfClass "/Game/06_Tech/Weather/BP/BP_Atmosphere.BP_Atmosphere_C"))
      (Utilities|IsValid (Variables|/Game/06_Tech/Weather/BP/BP_Atmosphere.BP_Atmosphere_C|GetAmbiant_Sound_First_Layer _returnvalue_3)
        (:Is%20Valid
          (Audio|Components|Audio|FadeOut (Variables|/Game/06_Tech/Weather/BP/BP_Atmosphere.BP_Atmosphere_C|GetAmbiant_Sound_First_Layer _returnvalue_3) 2.5 0.0 "Logarithmic" :!class /Script/Engine.AudioComponent))
        (:Is%20Not%20Valid
          _))
      (Utilities|IsValid (Variables|/Game/06_Tech/Weather/BP/BP_Atmosphere.BP_Atmosphere_C|GetAmbiant_Sound_Second_Layer _returnvalue_3)
        (:Is%20Valid
          (Audio|Components|Audio|FadeOut (Variables|/Game/06_Tech/Weather/BP/BP_Atmosphere.BP_Atmosphere_C|GetAmbiant_Sound_Second_Layer _returnvalue_3) 2.5 0.0 "Logarithmic" :!class /Script/Engine.AudioComponent))
        (:Is%20Not%20Valid
          _))
      ;[1 0 0.01775] Choix Tuto ou Hub
      (if (not (Variables|Default|GetHub%20Already%20Visited))
        (Variables|Default|SetHub%20Already%20Visited true)
        ;[1 0.695 0] Hub Global Amb SFX Fade In
        (bind _returnvalue_4 (Audio|SpawnSound2D "/Game/05_Audio/Amb_SFX/Global_Ambiences/Hub/Hub_Global_Ambience_v2/MSS_Hub_Global_Amb_SFXcomp.MSS_Hub_Global_Amb_SFXcomp" 1.0 1.0 0.0 0 true false))
        (bind _output_get (Variables|Default|SetHub%20Global%20Amb%20SFX _returnvalue_4))
        (Audio|Components|Audio|FadeIn _output_get 3.0 1.0 0.0 "Linear" :!class /Script/Engine.AudioComponent)
        ;[1 1 1] Hub Music Starts When Start Music SFX is OFF
        (if (not (Variables|Default|GetHub%20Music%20Has%20Played))
          (bind _returnvalue_5 (Utilities|Time|SetTimerbyEvent (delegate Custom|Check%20If%20Main%20Menu%20Music%20Is%20OFF) 0.1 true))
          (bind _output_get_2 (Variables|Default|SetTimer%20Check%20For%20Main%20Menu%20Music _returnvalue_5)))))))

(event Custom|onLevelChangeTutoToMain_Event
  ;[1 1 1] Tuto to Main
  (Variables|Default|Setstatus "MAINMENU")
  (Development|PrintString "TutoToMain" true true "(R=1.000000,G=0.274432,B=0.000000,A=1.000000)" 5.0)
  (Utilities|FlowControl|Sequence
    (:then_0
      (bind (_asbase_frame_bp _fade) (CallFunction|GetBaseFrameandFadeAnimationfromGameHUD))
      (Components|Animation|PlayAnimation _asbase_frame_bp _fade 0.0 1 "Forward" 0.75
        (:then
          ;[1 1 1] Game Amb SFX Fade Out
          (bind _returnvalue (Actor|GetActorOfClass "/Game/06_Tech/Weather/BP/BP_Atmosphere.BP_Atmosphere_C"))
          (Audio|Components|Audio|FadeOut (Variables|/Game/06_Tech/Weather/BP/BP_Atmosphere.BP_Atmosphere_C|GetAmbiant_Sound_First_Layer _returnvalue) 1.5 0.0 "Linear" :!class /Script/Engine.AudioComponent)
          (Utilities|IsValid (Variables|/Game/06_Tech/Weather/BP/BP_Atmosphere.BP_Atmosphere_C|GetAmbiant_Sound_Second_Layer _returnvalue)
            (:Is%20Valid
              (Audio|Components|Audio|FadeOut (Variables|/Game/06_Tech/Weather/BP/BP_Atmosphere.BP_Atmosphere_C|GetAmbiant_Sound_Second_Layer _returnvalue) 1.5 0.0 "Linear" :!class /Script/Engine.AudioComponent))))
        (:Finished
          (Default|CallOnLevelLoad))))))

(event Custom|onEndingTriggered_Event
  ;[1 1 1] Ending triggered
  (Development|PrintString "Ending Triggered"))

(event Custom|onEndingCredit_Event
  ;[1 1 1] Ending credit (show)
  (Development|PrintString "Ending Credit")
  (bind _returnvalue (Audio|SpawnSound2D "/Game/05_Audio/Music/MetaSounds/End_Credits_Music/MSS_End_Credits_Music.MSS_End_Credits_Music" 1.0 1.0 0.0 0 true false))
  (Variables|Default|SetEnd%20Credit%20Music _returnvalue))

(event Custom|onEndingCreditClose_Event
  (bind _end_credit_music (Variables|Default|GetEnd%20Credit%20Music))
  ;[1 1 1] Ending credit close with input
  (Development|PrintString "Ending Credit close")
  (Input|DisableInput (Game|GetPlayerController 0) 0)
  (Utilities|IsValid _end_credit_music
    (:Is%20Valid
      (Audio|Components|Audio|FadeOut _end_credit_music 5.0 0.0 "SCurve" :!class /Script/Engine.AudioComponent))))

(event Custom|onLevelChangeHubToGame_Event
  (bind _hub_global_amb_sfx (Variables|Default|GetHub%20Global%20Amb%20SFX))
  (bind _hub_music (Variables|Default|GetHub%20Music))
  ;[1 1 1] Hub To Game
  (Development|PrintString "HUB TO GAME" true true "(R=1.000000,G=0.274432,B=0.000000,A=1.000000)" 5.0)
  (Utilities|FlowControl|Sequence
    (:then_0
      (bind (_asbase_frame_bp _fade) (CallFunction|GetBaseFrameandFadeAnimationfromGlobalHUD))
      (Components|Animation|PlayAnimation _asbase_frame_bp _fade 0.0 1 "Forward" 0.75
        (:Finished
          (Default|CallOnLevelLoad)
          ;;[1 1 1] (Reinit SFX After Death)
          (Audio|PopSoundMixModifier "/Game/05_Audio/SoundClass_Mixes/Day_Message/SCM_Day_Message1.SCM_Day_Message1")
          (Audio|PopSoundMixModifier "/Game/05_Audio/SoundClass_Mixes/Day_Message/SCM_Day_Message2.SCM_Day_Message2"))))
    (:then_1
      ;[1 1 1] Hub Global Amb SFX Fade Out
      (Utilities|IsValid _hub_global_amb_sfx
        (:Is%20Valid
          (Development|PrintString "Fade Out Amb SFX")
          (Audio|Components|Audio|FadeOut _hub_global_amb_sfx 3.0 0.0 "SCurve" :!class /Script/Engine.AudioComponent))
        (:Is%20Not%20Valid
          _))
      ;[1 1 1] Hub Music Fade Out
      (Utilities|IsValid _hub_music
        (:Is%20Valid
          (Development|PrintString "Fade out Music")
          (Audio|Components|Audio|FadeOut _hub_music 4.0 0.0 "SCurve" :!class /Script/Engine.AudioComponent))
        (:Is%20Not%20Valid
          _))
      (Variables|Default|SetHub%20Music%20Has%20Played false)
      (Audio|PushSoundMixModifier "/Game/05_Audio/SoundClass_Mixes/Radio_OFF_When_Leaving/SCM_Radio_OFF_When_Leaving.SCM_Radio_OFF_When_Leaving") ; Fade Out Radio
    )))

(event Custom|onLevelChangeGameToHub_Event
  ;[1 1 1] Game To Hub
  (Development|PrintString "EVENT GAME TO HUB" true true "(R=1.000000,G=0.274432,B=0.000000,A=1.000000)" 5.0)
  (bind (_asbase_frame_bp _fade) (CallFunction|GetBaseFrameandFadeAnimationfromGameHUD))
  (Components|Animation|PlayAnimation _asbase_frame_bp _fade 0.0 1 "Forward" 0.75
    (:Finished
      (Default|CallOnLevelLoad)
      (Audio|PopSoundMixModifier "/Game/05_Audio/SoundClass_Mixes/Radio_OFF_When_Leaving/SCM_Radio_OFF_When_Leaving.SCM_Radio_OFF_When_Leaving")
      (if (Variables|Default|GetHub%20Already%20Visited)
        ;[1 1 1] Hub Global Amb SFX Fade In
        (bind _returnvalue (Utilities|Time|SetTimerbyEvent (delegate Custom|Check%20Level%20Change%201) 0.1 true))
        (else
          (Variables|Default|SetHub%20Already%20Visited true)
          ;[1 0.695 0] Hub Global Amb SFX Fade In
          (bind _returnvalue_2 (Audio|SpawnSound2D "/Game/05_Audio/Amb_SFX/Global_Ambiences/Hub/Hub_Global_Ambience_v2/MSS_Hub_Global_Amb_SFXcomp.MSS_Hub_Global_Amb_SFXcomp" 1.0 1.0 0.0 0 true false))
          (bind _output_get (Variables|Default|SetHub%20Global%20Amb%20SFX _returnvalue_2))
          (Audio|Components|Audio|FadeIn _output_get 3.0 1.0 0.0 "Linear" :!class /Script/Engine.AudioComponent)
          ;[1 1 1] Hub Music Starts When Start Music SFX is OFF
          (if (not (Variables|Default|GetHub%20Music%20Has%20Played))
            (bind _returnvalue_3 (Utilities|Time|SetTimerbyEvent (delegate Custom|Check%20If%20Main%20Menu%20Music%20Is%20OFF) 0.1 true))
            (bind _output_get_2 (Variables|Default|SetTimer%20Check%20For%20Main%20Menu%20Music _returnvalue_3))))))))

(event Custom|onLevelChangeMainToHub_Event
  (bind _bgm_menu (Variables|Default|GetBGM_Menu))
  ;[1 1 1] Main To Hub
  (Development|PrintString "MAIN TO HUB" true true "(R=1.000000,G=0.274432,B=0.000000,A=1.000000)" 5.0)
  (Utilities|FlowControl|Sequence
    (:then_0
      (bind (_asbase_frame_bp _fade) (CallFunction|GetBaseFrameandFadeAnimationfromMainHUD))
      (Components|Animation|PlayAnimation _asbase_frame_bp _fade 0.0 1 "Forward" 0.75
        (:Finished
          (Default|CallOnLevelLoad)
          (Audio|PopSoundMixModifier "/Game/05_Audio/SoundClass_Mixes/Radio_OFF_When_Leaving/SCM_Radio_OFF_When_Leaving.SCM_Radio_OFF_When_Leaving"))))
    (:then_1
      (Audio|PlaySound2D "/Game/05_Audio/SFX/MetaSounds/UI/Main_Menu/Positive/v2/MSS_UI_Main_Menu_Positive_v2.MSS_UI_Main_Menu_Positive_v2" 1.0 1.0 0.0 0 0)
      ;[1 1 1] Game Amb SFX Fade Out
      (bind _returnvalue (Actor|GetActorOfClass "/Game/06_Tech/Weather/BP/BP_Atmosphere.BP_Atmosphere_C"))
      (Audio|Components|Audio|FadeOut (Variables|/Game/06_Tech/Weather/BP/BP_Atmosphere.BP_Atmosphere_C|GetSFX_MainMenu_Layer1 _returnvalue) 1.5 0.0 "Linear" :!class /Script/Engine.AudioComponent)
      (Utilities|IsValid (Variables|/Game/06_Tech/Weather/BP/BP_Atmosphere.BP_Atmosphere_C|GetSFX_MainMenu_Layer2 _returnvalue)
        (:Is%20Valid
          (Audio|Components|Audio|FadeOut (Variables|/Game/06_Tech/Weather/BP/BP_Atmosphere.BP_Atmosphere_C|GetSFX_MainMenu_Layer2 _returnvalue) 1.5 0.0 "Linear" :!class /Script/Engine.AudioComponent)
          (Audio|PushSoundMixModifier "/Game/05_Audio/SoundClass_Mixes/Main_Menu_Lightnings_Fade_Out/SCM_Main_Menu_Lightnings_Fade_Out.SCM_Main_Menu_Lightnings_Fade_Out")
          ;[1 0.695 0] Start Game Music SFX
          (bind _returnvalue_2 (Audio|SpawnSound2D "/Game/05_Audio/Music/MetaSounds/Main_Menu_Music/MSS_Start_Music_FX_JGoldsmith_Chord_v2.MSS_Start_Music_FX_JGoldsmith_Chord_v2" 1.0 1.0 0.0 0 true false))
          (Variables|Default|SetStart%20Game%20Music%20FX _returnvalue_2)
          ;[1 1 1] Main Menu Music Fade Out
          (Utilities|IsValid _bgm_menu
            (:Is%20Valid
              (Audio|Components|Audio|FadeOut _bgm_menu 1.6 0.0 "SCurve" :!class /Script/Engine.AudioComponent)
              ;[1 0 0.01775] Choix Tuto ou Hub
              (if (not (Variables|Default|GetHub%20Already%20Visited))
                (Variables|Default|SetHub%20Already%20Visited true)
                ;[1 0.695 0] Hub Global Amb SFX Fade In
                (bind _returnvalue_3 (Audio|SpawnSound2D "/Game/05_Audio/Amb_SFX/Global_Ambiences/Hub/Hub_Global_Ambience_v2/MSS_Hub_Global_Amb_SFXcomp.MSS_Hub_Global_Amb_SFXcomp" 1.0 1.0 0.0 0 true false))
                (bind _output_get (Variables|Default|SetHub%20Global%20Amb%20SFX _returnvalue_3))
                (Audio|Components|Audio|FadeIn _output_get 3.0 1.0 0.0 "Linear" :!class /Script/Engine.AudioComponent)
                ;[1 1 1] Hub Music Starts When Start Music SFX is OFF
                (if (not (Variables|Default|GetHub%20Music%20Has%20Played))
                  (bind _returnvalue_4 (Utilities|Time|SetTimerbyEvent (delegate Custom|Check%20If%20Main%20Menu%20Music%20Is%20OFF) 0.1 true))
                  (bind _output_get_2 (Variables|Default|SetTimer%20Check%20For%20Main%20Menu%20Music _returnvalue_4)))))))))))

(event Custom|onLevelChangeGameToMain_Event
  ;[1 0.695 0] Game To Main
  (Variables|Default|Setstatus "MAINMENU")
  (Development|PrintString "EVENT GAME TO MAIN" true true "(R=1.000000,G=0.274432,B=0.000000,A=1.000000)" 5.0)
  ;[1 1 1] Tower SFX Fade Out
  (bind _outactors (Actor|GetAllActorsOfClass "/Game/05_Audio/BP/BP_TowerField_SFX.BP_TowerField_SFX_C"))
  (Utilities|IsValid (Variables|/Game/05_Audio/BP/BP_TowerField_SFX.BP_TowerField_SFX_C|GetLayer%201%20SFX (Utilities|Array|Get(acopy) _outactors))
    (:Is%20Valid
      (Audio|Components|Audio|FadeOut (Variables|/Game/05_Audio/BP/BP_TowerField_SFX.BP_TowerField_SFX_C|GetLayer%201%20SFX (Utilities|Array|Get(acopy) _outactors)) 1.0 0.0 "Linear" :!class /Script/Engine.AudioComponent))
    (:Is%20Not%20Valid
      _))
  (Utilities|IsValid (Variables|/Game/05_Audio/BP/BP_TowerField_SFX.BP_TowerField_SFX_C|GetLayer%202%20SFX (Utilities|Array|Get(acopy) _outactors))
    (:Is%20Valid
      (Audio|Components|Audio|FadeOut (Variables|/Game/05_Audio/BP/BP_TowerField_SFX.BP_TowerField_SFX_C|GetLayer%202%20SFX (Utilities|Array|Get(acopy) _outactors)) 1.0 0.0 "Linear" :!class /Script/Engine.AudioComponent))
    (:Is%20Not%20Valid
      _))
  ;[1 1 1] Game Amb SFX Fade Out
  (bind _returnvalue (Actor|GetActorOfClass "/Game/06_Tech/Weather/BP/BP_Atmosphere.BP_Atmosphere_C"))
  (Audio|Components|Audio|FadeOut (Variables|/Game/06_Tech/Weather/BP/BP_Atmosphere.BP_Atmosphere_C|GetAmbiant_Sound_First_Layer _returnvalue) 1.0 0.0 "Linear" :!class /Script/Engine.AudioComponent)
  (Utilities|IsValid (Variables|/Game/06_Tech/Weather/BP/BP_Atmosphere.BP_Atmosphere_C|GetAmbiant_Sound_Second_Layer _returnvalue)
    (:Is%20Valid
      (Audio|Components|Audio|FadeOut (Variables|/Game/06_Tech/Weather/BP/BP_Atmosphere.BP_Atmosphere_C|GetAmbiant_Sound_Second_Layer _returnvalue) 1.0 0.0 "Linear" :!class /Script/Engine.AudioComponent))
    (:Is%20Not%20Valid
      _))
  (bind _outactors_2 (Actor|GetAllActorsOfClass "/Game/05_Audio/BP/P_Sector1_Tunnel_HitBox.P_Sector1_Tunnel_HitBox_C"))
  (Utilities|IsValid (Variables|/Game/05_Audio/BP/P_Sector1_Tunnel_HitBox.P_Sector1_Tunnel_HitBox_C|GetTunnel%20Global%20Amb%20SFX (Utilities|Array|Get(acopy) _outactors_2))
    (:Is%20Valid
      (Audio|Components|Audio|FadeOut (Variables|/Game/05_Audio/BP/P_Sector1_Tunnel_HitBox.P_Sector1_Tunnel_HitBox_C|GetTunnel%20Global%20Amb%20SFX (Utilities|Array|Get(acopy) _outactors_2)) 1.0 0.0 "Linear" :!class /Script/Engine.AudioComponent))
    (:Is%20Not%20Valid
      _))
  (Audio|PushSoundMixModifier "/Game/05_Audio/SoundClass_Mixes/Quit_Game_To_Main/SCM_Quit_Game_To_Main.SCM_Quit_Game_To_Main")
  (bind (_asbase_frame_bp _fade) (CallFunction|GetBaseFrameandFadeAnimationfromGameHUD))
  (Components|Animation|PlayAnimation _asbase_frame_bp _fade 0.0 1 "Forward" 0.75
    (:Finished
      (Default|CallOnLevelLoad))))

(event Custom|onLevelChangeMainToQuit_Event
  ;[1 1 1] Main To Quit
  (Development|PrintString "MAIN TO QUIT" true true "(R=1.000000,G=0.274432,B=0.000000,A=1.000000)" 5.0)
  (Utilities|FlowControl|Sequence
    (:then_0
      (bind (_asbase_frame_bp _fade) (CallFunction|GetBaseFrameandFadeAnimationfromMainHUD))
      (Components|Animation|PlayAnimation _asbase_frame_bp _fade 0.0 1 "Forward" 0.75
        (:Finished
          (Default|CallOnLevelLoad))))
    (:then_1
      ;[1 1 1] BGM Menu Fade Out To Quit Game
      (Audio|Components|Audio|FadeOut (Variables|Default|GetBGM_Menu) 1.45 0.0 "SCurve" :!class /Script/Engine.AudioComponent)
      ;[1 1 1] Main Menu Amb SFX Fade Out
      (bind _returnvalue (Actor|GetActorOfClass "/Game/06_Tech/Weather/BP/BP_Atmosphere.BP_Atmosphere_C"))
      (Utilities|IsValid (Variables|/Game/06_Tech/Weather/BP/BP_Atmosphere.BP_Atmosphere_C|GetSFX_MainMenu_Layer1 _returnvalue)
        (:Is%20Valid
          (Audio|Components|Audio|FadeOut (Variables|/Game/06_Tech/Weather/BP/BP_Atmosphere.BP_Atmosphere_C|GetSFX_MainMenu_Layer1 _returnvalue) 1.3 0.0 "Linear" :!class /Script/Engine.AudioComponent))
        (:Is%20Not%20Valid
          _))
      (Utilities|IsValid (Variables|/Game/06_Tech/Weather/BP/BP_Atmosphere.BP_Atmosphere_C|GetSFX_MainMenu_Layer2 _returnvalue)
        (:Is%20Valid
          (Audio|Components|Audio|FadeOut (Variables|/Game/06_Tech/Weather/BP/BP_Atmosphere.BP_Atmosphere_C|GetSFX_MainMenu_Layer2 _returnvalue) 1.3 0.0 "Linear" :!class /Script/Engine.AudioComponent)
          (Audio|PushSoundMixModifier "/Game/05_Audio/SoundClass_Mixes/Main_Menu_Lightnings_Fade_Out/SCM_Main_Menu_Lightnings_Fade_Out.SCM_Main_Menu_Lightnings_Fade_Out"))))))

(event Custom|onLevelChangeHubToMain_Event
  (bind _hub_music (Variables|Default|GetHub%20Music))
  (bind _hub_global_amb_sfx (Variables|Default|GetHub%20Global%20Amb%20SFX))
  ;[1 1 1] Hub To Main
  (Variables|Default|Setstatus "MAINMENU")
  (Development|PrintString "HUB TO MAIN" true true "(R=1.000000,G=0.274432,B=0.000000,A=1.000000)" 5.0)
  (Utilities|FlowControl|Sequence
    (:then_0
      (bind (_asbase_frame_bp _fade) (CallFunction|GetBaseFrameandFadeAnimationfromGlobalHUD))
      (Components|Animation|PlayAnimation _asbase_frame_bp _fade 0.0 1 "Forward" 0.75
        (:Finished
          (Default|CallOnLevelLoad))))
    (:then_1
      ;[1 1 1] Hub Global Amb SFX Fade Out
      (Utilities|IsValid _hub_global_amb_sfx
        (:Is%20Valid
          (Audio|Components|Audio|FadeOut _hub_global_amb_sfx 1.5 0.0 "Logarithmic" :!class /Script/Engine.AudioComponent)
          ;[1 1 1] Hub Music fade Out
          (Utilities|IsValid _hub_music
            (:Is%20Valid
              (if (Audio|Components|Audio|IsPlaying _hub_music)
                (Audio|Components|Audio|FadeOut _hub_music 1.5 0.0 "SCurve" :!class /Script/Engine.AudioComponent)
                (Variables|Default|SetHub%20Music%20Has%20Played false)
                (Audio|PushSoundMixModifier "/Game/05_Audio/SoundClass_Mixes/Radio_OFF_When_Leaving/SCM_Radio_OFF_When_Leaving.SCM_Radio_OFF_When_Leaving")))))))))

(event Custom|Check%20If%20Main%20Menu%20Music%20Is%20OFF
  ;[1 1 1] Hub Music Starts When Start Music SFX is OFF
  (if (not (Audio|Components|Audio|IsPlaying (Variables|Default|GetStart%20Game%20Music%20FX)))
    (Utilities|Time|ClearandInvalidateTimerbyHandle (stale Custom|onLevelChangeTutoToHub_Event_0 _output_get_2))
    (if (not (Audio|Components|Audio|IsPlaying (Variables|Default|GetBGM_Menu)))
      (bind _returnvalue (Audio|SpawnSound2D "/Game/05_Audio/Music/MetaSounds/Hub_Music/MSS_Hub_Music.MSS_Hub_Music" 1.0 1.0 0.0 0 true false))
      (bind _output_get (Variables|Default|SetHub%20Music _returnvalue))
      (Audio|Components|Audio|FadeIn _output_get 3.75 1.0 0.0 "Linear" :!class /Script/Engine.AudioComponent)
      (Variables|Default|SetHub%20Music%20Has%20Played true))))

(event EventInit
  (Utilities|FlowControl|Sequence
    (:then_0
      (|CreateDiscordRichpresence))
    (:then_1
      (Components|Animation|PlayAnimation))
    (:then_2
      ;[1 1 1] Main To Hub
      (EventDispatchers|AssignOnLevelChangeMaintoHub (delegate Custom|onLevelChangeMainToHub_Event)))
    (:then_3
      ;[1 1 1] Hub To Game
      (EventDispatchers|AssignOnLevelChangeHubtoGame (delegate Custom|onLevelChangeHubToGame_Event)))
    (:then_4
      ;[1 1 1] Game To Hub
      (EventDispatchers|AssignOnLevelChangeGametoHub (delegate Custom|onLevelChangeGameToHub_Event)))
    (:then_5
      ;[1 0.695 0] Game To Main
      (EventDispatchers|AssignOnLevelChangeGametoMain (delegate Custom|onLevelChangeGameToMain_Event)))
    (:then_6
      ;[1 1 1] Main To Quit
      (EventDispatchers|AssignOnLevelChangeMaintoQuit (delegate Custom|onLevelChangeMainToQuit_Event)))
    (:then_7
      ;[1 1 1] Hub To Main
      (EventDispatchers|AssignOnLevelChangeHubtoMain (delegate Custom|onLevelChangeHubToMain_Event)))
    (:then_8
      ;[1 1 1] Death (To Hub)
      (EventDispatchers|AssignOnDeathtoHub (delegate Custom|onDeathToHub_Event)))
    (:then_9
      ;[1 1 1] Main To Tuto
      (EventDispatchers|BindEventtoOnLevelChangeMaintoIntro (delegate Custom|MainToTuto)))
    (:then_10
      ;[1 1 1] Tuto to Main
      (EventDispatchers|AssignOnLevelChangeIntrotoMain (delegate Custom|onLevelChangeTutoToMain_Event)))
    (:then_11
      ;[1 1 1] Tuto to Hub
      (EventDispatchers|AssignOnLevelChangeIntrotoHub (delegate Custom|onLevelChangeTutoToHub_Event_0)))
    (:then_12
      ;[1 1 1] Ending triggered
      (EventDispatchers|AssignOnEndingTriggered (delegate Custom|onEndingTriggered_Event)))
    (:then_13
      ;[1 1 1] Ending credit (show)
      (EventDispatchers|AssignOnEndingCredit (delegate Custom|onEndingCredit_Event)))
    (:then_14
      ;[1 1 1] Ending credit close with input
      (EventDispatchers|AssignOnEndingCreditClose (delegate Custom|onEndingCreditClose_Event)))))

(fn MakeFadeMainHUD
  (bind _asbp_main_hud (Utilities|Casting|CastToBp_MainHUD (HUD|GetHUD (Game|GetPlayerController 0))))
  (bind _asbase_frame_bp (Utilities|Casting|CastToBaseFrameBP (Class|MainHUD|GetCurrentFrame _asbp_main_hud)))
  (Variables|/Script/UMG.Widget|SetbIsEnabled (Variables|/Game/00_Prog/UI/Menu/BaseFrameBP.BaseFrameBP_C|GetBorderFade _asbase_frame_bp) true)
  (Variables|/Script/UMG.Widget|SetVisibility (Variables|/Game/00_Prog/UI/Menu/BaseFrameBP.BaseFrameBP_C|GetBorderFade _asbase_frame_bp) "Visible")
  (Default|CallOnLevelLoad))

(fn MakeFadeGameHUd
  (bind _asbp_game_hud (Utilities|Casting|CastToBp_GameHUD (HUD|GetHUD (Game|GetPlayerController 0))))
  (bind _asbase_frame_bp (Utilities|Casting|CastToBaseFrameBP (Class|MainHUD|GetCurrentFrame _asbp_game_hud)))
  (Variables|/Script/UMG.Widget|SetbIsEnabled (Variables|/Game/00_Prog/UI/Menu/BaseFrameBP.BaseFrameBP_C|GetBorderFade _asbase_frame_bp) true)
  (Variables|/Script/UMG.Widget|SetVisibility (Variables|/Game/00_Prog/UI/Menu/BaseFrameBP.BaseFrameBP_C|GetBorderFade _asbase_frame_bp) "Visible")
  (Default|CallOnLevelLoad))

(fn GetBaseFrameandFadeAnimationfromMainHUD
  (bind _asbp_main_hud (Utilities|Casting|CastToBp_MainHUD (HUD|GetHUD (Game|GetPlayerController 0)))
    (:then
      (bind _asbase_frame_bp (Utilities|Casting|CastToBaseFrameBP (Class|MainHUD|GetCurrentFrame _asbp_main_hud)))
      (Variables|/Script/UMG.Widget|SetbIsEnabled (Variables|/Game/00_Prog/UI/Menu/BaseFrameBP.BaseFrameBP_C|GetBorderFade _asbase_frame_bp) true)
      (Variables|/Script/UMG.Widget|SetVisibility (Variables|/Game/00_Prog/UI/Menu/BaseFrameBP.BaseFrameBP_C|GetBorderFade _asbase_frame_bp) "Visible")
      (return _asbase_frame_bp (Variables|/Game/00_Prog/UI/Menu/BaseFrameBP.BaseFrameBP_C|GetFade _asbase_frame_bp)))
    (:CastFailed
      (Development|PrintString "Error cast failed MainHUD"))))

(fn GetBaseFrameandFadeAnimationfromGlobalHUD
  (bind _asbp_global_hud (Utilities|Casting|CastToBp_GlobalHUD (HUD|GetHUD (Game|GetPlayerController 0)))
    (:then
      (bind _asbase_frame_bp (Utilities|Casting|CastToBaseFrameBP (Class|MainHUD|GetCurrentFrame _asbp_global_hud)))
      (Variables|/Script/UMG.Widget|SetbIsEnabled (Variables|/Game/00_Prog/UI/Menu/BaseFrameBP.BaseFrameBP_C|GetBorderFade _asbase_frame_bp) true)
      (Variables|/Script/UMG.Widget|SetVisibility (Variables|/Game/00_Prog/UI/Menu/BaseFrameBP.BaseFrameBP_C|GetBorderFade _asbase_frame_bp) "Visible")
      (return _asbase_frame_bp (Variables|/Game/00_Prog/UI/Menu/BaseFrameBP.BaseFrameBP_C|GetFade _asbase_frame_bp)))
    (:CastFailed
      (Development|PrintString "Error cast failed GlobalHUD"))))

(fn GetBaseFrameandFadeAnimationfromGameHUD
  (bind _asbp_game_hud (Utilities|Casting|CastToBp_GameHUD (HUD|GetHUD (Game|GetPlayerController 0)))
    (:then
      (bind _asbase_frame_bp (Utilities|Casting|CastToBaseFrameBP (Class|MainHUD|GetCurrentFrame _asbp_game_hud)))
      (Variables|/Script/UMG.Widget|SetbIsEnabled (Variables|/Game/00_Prog/UI/Menu/BaseFrameBP.BaseFrameBP_C|GetBorderFade _asbase_frame_bp) true)
      (Variables|/Script/UMG.Widget|SetVisibility (Variables|/Game/00_Prog/UI/Menu/BaseFrameBP.BaseFrameBP_C|GetBorderFade _asbase_frame_bp) "Visible")
      (return _asbase_frame_bp (Variables|/Game/00_Prog/UI/Menu/BaseFrameBP.BaseFrameBP_C|GetFade _asbase_frame_bp)))
    (:CastFailed
      (Development|PrintString "Error cast failed Game HUD"))))

(fn UpdateRichPresence
  (params (Title :type String) (Details :type String)))

(event Custom|onLevelLoaded_Event
  (bind _returnvalue (Game|GetPlayerController 0))
  (bind _returnvalue_2 (HUD|GetHUD _returnvalue))
  ;[1 1 1] Play Animation Fade In
  (bind _asbp_main_hud (Utilities|Casting|CastToBp_MainHUD _returnvalue_2)
    (:then
      (bind _asbase_frame_bp (Utilities|Casting|CastToBaseFrameBP (Class|MainHUD|GetCurrentFrame _asbp_main_hud)))
      (Variables|/Script/UMG.Widget|SetbIsEnabled (Variables|/Game/00_Prog/UI/Menu/BaseFrameBP.BaseFrameBP_C|GetBorderFade _asbase_frame_bp) true)
      (Variables|/Script/UMG.Widget|SetVisibility (Variables|/Game/00_Prog/UI/Menu/BaseFrameBP.BaseFrameBP_C|GetBorderFade _asbase_frame_bp) "Visible")
      (Components|Animation|PlayAnimation _asbase_frame_bp (Variables|/Game/00_Prog/UI/Menu/BaseFrameBP.BaseFrameBP_C|GetFadeOut _asbase_frame_bp) 0.0 1 "Forward" 0.75
        (:Finished
          (Variables|/Script/UMG.Widget|SetbIsEnabled (Variables|/Game/00_Prog/UI/Menu/BaseFrameBP.BaseFrameBP_C|GetBorderFade _asbase_frame_bp) false)
          (Variables|/Script/UMG.Widget|SetVisibility (Variables|/Game/00_Prog/UI/Menu/BaseFrameBP.BaseFrameBP_C|GetBorderFade _asbase_frame_bp) "HitTestInvisible"))))
    (:CastFailed
      (bind _asbp_global_hud (Utilities|Casting|CastToBp_GlobalHUD _returnvalue_2)
        (:then
          (bind _asbase_frame_bp_2 (Utilities|Casting|CastToBaseFrameBP (Class|MainHUD|GetCurrentFrame _asbp_global_hud)))
          (Variables|/Script/UMG.Widget|SetbIsEnabled (Variables|/Game/00_Prog/UI/Menu/BaseFrameBP.BaseFrameBP_C|GetBorderFade _asbase_frame_bp_2) true)
          (Variables|/Script/UMG.Widget|SetVisibility (Variables|/Game/00_Prog/UI/Menu/BaseFrameBP.BaseFrameBP_C|GetBorderFade _asbase_frame_bp_2) "Visible")
          (Components|Animation|PlayAnimation _asbase_frame_bp_2 (Variables|/Game/00_Prog/UI/Menu/BaseFrameBP.BaseFrameBP_C|GetFadeOut _asbase_frame_bp_2) 0.0 1 "Forward" 0.75
            (:Finished
              (Variables|/Script/UMG.Widget|SetbIsEnabled (Variables|/Game/00_Prog/UI/Menu/BaseFrameBP.BaseFrameBP_C|GetBorderFade _asbase_frame_bp_2) false)
              (Variables|/Script/UMG.Widget|SetVisibility (Variables|/Game/00_Prog/UI/Menu/BaseFrameBP.BaseFrameBP_C|GetBorderFade _asbase_frame_bp_2) "HitTestInvisible"))))
        (:CastFailed
          (bind _asbp_game_hud (Utilities|Casting|CastToBp_GameHUD _returnvalue_2))
          (bind _asbase_frame_bp_3 (Utilities|Casting|CastToBaseFrameBP (Class|MainHUD|GetCurrentFrame _asbp_game_hud)))
          (Variables|/Script/UMG.Widget|SetbIsEnabled (Variables|/Game/00_Prog/UI/Menu/BaseFrameBP.BaseFrameBP_C|GetBorderFade _asbase_frame_bp_3) true)
          (Variables|/Script/UMG.Widget|SetVisibility (Variables|/Game/00_Prog/UI/Menu/BaseFrameBP.BaseFrameBP_C|GetBorderFade _asbase_frame_bp_3) "Visible")
          (Components|Animation|PlayAnimation _asbase_frame_bp_3 (Variables|/Game/00_Prog/UI/Menu/BaseFrameBP.BaseFrameBP_C|GetFadeOut _asbase_frame_bp_3) 0.0 1 "Forward" 0.75
            (:Finished
              (Variables|/Script/UMG.Widget|SetbIsEnabled (Variables|/Game/00_Prog/UI/Menu/BaseFrameBP.BaseFrameBP_C|GetBorderFade _asbase_frame_bp_3) false)
              (Variables|/Script/UMG.Widget|SetVisibility (Variables|/Game/00_Prog/UI/Menu/BaseFrameBP.BaseFrameBP_C|GetBorderFade _asbase_frame_bp_3) "HitTestInvisible"))))))))