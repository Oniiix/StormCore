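; Paralarva AI enemy Blueprint that handles the creature's visual and audio feedback for damage, death and fading.
; Construction creates a dynamic material on the mesh, whose scalars drive a timed hit flash, a low-HP look at half life and a dithered fade.
; LifeComponent damage events update those effects, play a hurt sound only once, and relay OnDamaged.
; Death spawns an attached blood-jet Niagara effect and death sound.
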(event OnDie(lifeComponent)
  (bind _mesh (Variables|Character|GetMesh))
  (Niagara|SpawnSystemAttached "/Game/04_FX/NS/Enemies/Global/NS_Blood_Jet_Stream_para.NS_Blood_Jet_Stream_para" _mesh "spit_06" (Transformation|GetSocketLocation _mesh "spit_06") "0, 0, 0" "KeepWorldPosition" false)
  ;[1 1 1] Death SFX
  (Audio|SpawnSoundAttached "/Game/05_Audio/SFX/MetaSounds/Enemies/ParaLarve/PLarva_Death/MSS_PLarva_Death.MSS_PLarva_Death" _mesh "None" "0, 0, 0" "0, 0, 0" "KeepRelativeOffset" false 1.0 1.0 0.0 0 0))

(event OnLifeChangebyDamage(lifeComponent)
  (params (_owner :type Actor%20Object%20Reference) (_currentLife :type Integer) (_damage :type Integer) (_damageSource :type Actor%20Object%20Reference))
  (bind _dym_material (Variables|Default|GetDym_material))
  (Utilities|FlowControl|Sequence
    (:then_0
      ;[1 1 1] Simple Damage SFX
      (if (> _currentLife 0)
        (if (not (Variables|Default|GetPLarva_Has_Died))
          (Audio|SpawnSoundAttached "/Game/05_Audio/SFX/MetaSounds/Enemies/ParaLarve/Getting_Damaged/MSS_Getting_Damaged.MSS_Getting_Damaged" (Variables|Character|GetMesh) "None" "0, 0, 0" "0, 0, 0" "KeepRelativeOffset" false 1.0 1.0 0.0 0 0)
          (Variables|Default|SetPLarva_Has_Died true))))
    (:then_1
      (bind _hit_switch (Timeline|TL_damage_Hit PlayFromStart)
        (:Update
          (Rendering|Material|SetScalarParameterValue _dym_material "Hit_Shader" _hit_switch :!class /Script/Engine.MaterialInstanceDynamic))))
    (:then_2
      (Variables|Default|GetlifeComponent
        (:then
          (if (<= (/ (Math|Conversions|ToFloat(Integer) _currentLife) (Math|Conversions|ToFloat(Integer) (Class|LifeComponent|GetMaxLife (Variables|Default|GetlifeComponent)))) 0.5)
            (Rendering|Material|SetScalarParameterValue _dym_material "Low_HP" 1.0 :!class /Script/Engine.MaterialInstanceDynamic)))
        (:else)))
    (:then_3
      (Default|CallOnDamaged _damage))))

(event Custom|onFade_Event
  (bind _dither_value (Timeline|Timeline PlayFromStart)
    (:Update
      (Rendering|Material|SetScalarParameterValue (Variables|Default|GetDym_material) "Dither_Threshold" _dither_value :!class /Script/Engine.MaterialInstanceDynamic))))

(event EventBeginPlay
  (Components|Timeline|SetPlayRate (Variables|Default|GetTL_damage_Hit) (/ 1.0 (Variables|Default|GetHit_duree)))
  (EventDispatchers|AssignOnFade (delegate Custom|onFade_Event)))

(event Collision|EventActorBeginOverlap
  (params (OtherActor :type Actor%20Object%20Reference)))

(event EventTick
  (params (DeltaSeconds :type Float%20%28single-precision%29)))

(fn ConstructionScript
  (bind _returnvalue (Rendering|Material|CreateDynamicMaterialInstance "/Game/03_Graph/Enemies/Materials/MI_Paralarve.MI_Paralarve" "None" "None" :!class /Script/Engine.KismetMaterialLibrary))
  (bind _output_get (Variables|Default|SetDym_material _returnvalue))
  (Rendering|Material|SetMaterial (Variables|Character|GetMesh) 0 _output_get))