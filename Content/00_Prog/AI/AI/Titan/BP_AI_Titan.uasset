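; Titan AI enemy Blueprint that handles the visual and audio feedback for damage, fading and death.
; The construction script creates dynamic material instances for the body and two shell slots.
; Timelines drive their hit flash on damage, with play rate set from HitDuree, and their dither on the OnFade event.
; Death spawns an attached Niagara blood jet, plus a death sound guarded to play only once.
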(event OnLifeChangebyDamage(lifeComponent)
  (params (_owner :type Actor%20Object%20Reference) (_currentLife :type Integer) (_damage :type Integer) (_damageSource :type Actor%20Object%20Reference))
  (bind _hit_switch (Timeline|TL_Damage_Shader PlayFromStart)
    (:Update
      (Rendering|Material|SetScalarParameterValue (Variables|Default|GetTitan_Material_body) "Hit_Shader" _hit_switch :!class /Script/Engine.MaterialInstanceDynamic)
      (Rendering|Material|SetScalarParameterValue (Variables|Default|GetTitan_Material_shell_01) "Hit_Shader" _hit_switch :!class /Script/Engine.MaterialInstanceDynamic)
      (Rendering|Material|SetScalarParameterValue (Variables|Default|GetTitan_Material_shell_02) "Hit_Shader" _hit_switch :!class /Script/Engine.MaterialInstanceDynamic))))

(event OnDie(lifeComponent)
  (bind _mesh (Variables|Character|GetMesh))
  (Niagara|SpawnSystemAttached "/Game/04_FX/NS/Enemies/Global/NS_Blood_Jet_Stream_Titan.NS_Blood_Jet_Stream_Titan" _mesh "spit_06" (Transformation|GetSocketLocation _mesh "spit_06") "0, 0, 0" "KeepWorldPosition" false)
  (if (not (Variables|Default|GetTitan_Has_Died))
    (Audio|SpawnSoundAttached "/Game/05_Audio/SFX/MetaSounds/Enemies/Titan/Death/MSS_Titan_Death.MSS_Titan_Death" _mesh "None" "0, 0, 0" "0, 0, 0" "KeepRelativeOffset" false 1.0 1.0 0.0 0 0)
    (Variables|Default|SetTitan_Has_Died true)))

(event Custom|onFade_Event
  (bind _dither_value (Timeline|Timeline PlayFromStart)
    (:Update
      (Rendering|Material|SetScalarParameterValue (Variables|Default|GetTitan_Material_body) "Dither_Threshold" _dither_value :!class /Script/Engine.MaterialInstanceDynamic)
      (Rendering|Material|SetScalarParameterValue (Variables|Default|GetTitan_Material_shell_01) "Dither_Threshold" _dither_value :!class /Script/Engine.MaterialInstanceDynamic)
      (Rendering|Material|SetScalarParameterValue (Variables|Default|GetTitan_Material_shell_02) "Dither_Threshold" _dither_value :!class /Script/Engine.MaterialInstanceDynamic))))

(event EventBeginPlay
  (Components|Timeline|SetPlayRate (Variables|Default|GetTL_Damage_Shader) (/ 1.0 (Variables|Default|GetHit_duree)))
  (EventDispatchers|AssignOnFade (delegate Custom|onFade_Event)))

(event Collision|EventActorBeginOverlap
  (params (OtherActor :type Actor%20Object%20Reference)))

(event EventTick
  (params (DeltaSeconds :type Float%20%28single-precision%29)))

(fn ConstructionScript
  (Utilities|FlowControl|Sequence
    (:then_0
      (bind _returnvalue (Rendering|Material|CreateDynamicMaterialInstance "/Game/03_Graph/Enemies/Materials/MI_Titan_Body.MI_Titan_Body" "None" "None" :!class /Script/Engine.KismetMaterialLibrary))
      (bind _output_get (Variables|Default|SetTitan_Material_body _returnvalue))
      (Rendering|Material|SetMaterial (Variables|Character|GetMesh) 2 _output_get))
    (:then_1
      (bind _returnvalue_2 (Rendering|Material|CreateDynamicMaterialInstance "/Game/03_Graph/Enemies/Materials/MI_Titan_Shells01.MI_Titan_Shells01" "None" "None" :!class /Script/Engine.KismetMaterialLibrary))
      (bind _output_get_2 (Variables|Default|SetTitan_Material_shell_01 _returnvalue_2))
      (Rendering|Material|SetMaterial (Variables|Character|GetMesh) 0 _output_get_2))
    (:then_2
      (bind _returnvalue_3 (Rendering|Material|CreateDynamicMaterialInstance "/Game/03_Graph/Enemies/Materials/MI_Titan_Shells02.MI_Titan_Shells02" "None" "None" :!class /Script/Engine.KismetMaterialLibrary))
      (bind _output_get_3 (Variables|Default|SetTitan_Material_shell_02 _returnvalue_3))
      (Rendering|Material|SetMaterial (Variables|Character|GetMesh) 1 _output_get_3))))