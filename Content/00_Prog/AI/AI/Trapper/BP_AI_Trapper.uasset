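; Trapper AI enemy Blueprint that handles the creature's visual and audio feedback, with eye effects and a socket-attached weak point.
; Camouflage component events play or reverse a timeline that blends a dynamic opaque material with a translucent overlay, cleared after reversing.
; Life component events drive a hit flash, a low-health look at half life, and a death blood jet with one-time layered randomized sounds.
; A fade event animates dithering.
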(event OnTransform(camouflageComponent)
  ;[0 0.4018 1] Camouflage
  (bind (_direction _opaque_exponent _opaque_visibility _transluscent_exponent _transluscent_reflexion _transluscent_switch) (Timeline|TL_Camouflage Play)
    (:Update
      (CallFunction|UpdateOpaqueMaterial true _opaque_exponent true _opaque_visibility :!label _label)
      (CallFunction|UpdateTransluscentMaterial true _transluscent_exponent true _transluscent_reflexion true _transluscent_switch)
      (Rendering|Material|SetOverlayMaterial (Variables|Character|GetMesh) (Variables|Default|GetTransluscent_Material) :!class /Script/Engine.MeshComponent))
    (:Finished
      (Utilities|FlowControl|Sequence
        (:then_0
          (goto _label))
        (:then_1
          (switch Utilities|FlowControl|Switch|SwitchonETimelineDirection _direction
            (:Backward
              (Rendering|Material|SetOverlayMaterial (Variables|Character|GetMesh) 0 :!class /Script/Engine.MeshComponent))))))))

(event OnDisableTransform(camouflageComponent)
  ;[0 0.4018 1] Camouflage
  (bind (_direction _opaque_exponent _opaque_visibility _transluscent_exponent _transluscent_reflexion _transluscent_switch) (Timeline|TL_Camouflage Reverse)
    (:Update
      (CallFunction|UpdateOpaqueMaterial true _opaque_exponent true _opaque_visibility :!label _label)
      (CallFunction|UpdateTransluscentMaterial true _transluscent_exponent true _transluscent_reflexion true _transluscent_switch)
      (Rendering|Material|SetOverlayMaterial (Variables|Character|GetMesh) (Variables|Default|GetTransluscent_Material) :!class /Script/Engine.MeshComponent))
    (:Finished
      (Utilities|FlowControl|Sequence
        (:then_0
          (goto _label))
        (:then_1
          (switch Utilities|FlowControl|Switch|SwitchonETimelineDirection _direction
            (:Backward
              (Rendering|Material|SetOverlayMaterial (Variables|Character|GetMesh) 0 :!class /Script/Engine.MeshComponent))))))))

(event OnLifeChangebyDamage(lifeComponent)
  (params (_owner :type Actor%20Object%20Reference) (_currentLife :type Integer) (_damage :type Integer) (_damageSource :type Actor%20Object%20Reference))
  (bind _opaque_material (Variables|Default|GetOpaque_Material))
  (Utilities|FlowControl|Sequence
    (:then_0
      (bind _hit_switch (Timeline|TL_DamageHit PlayFromStart)
        (:Update
          (Rendering|Material|SetScalarParameterValue _opaque_material "Hit_Shader" _hit_switch :!class /Script/Engine.MaterialInstanceDynamic))))
    (:then_1
      (if (<= (/ (Math|Conversions|ToFloat(Integer) _currentLife) (Math|Conversions|ToFloat(Integer) (Class|LifeComponent|GetMaxLife (Variables|Default|GetlifeComponent)))) 0.5)
        (Rendering|Material|SetScalarParameterValue _opaque_material "Low_HP" 1.0 :!class /Script/Engine.MaterialInstanceDynamic)))))

(event OnDie(lifeComponent)
  (bind _returnvalue (Math|Random|RandomIntegerinRange 0 4))
  (bind _mesh (Variables|Character|GetMesh))
  (Niagara|SpawnSystemAttached "/Game/04_FX/NS/Enemies/Global/NS_Blood_Jet_Stream_Titan.NS_Blood_Jet_Stream_Titan" _mesh "spit_06" (Transformation|GetSocketLocation _mesh "spit_06") "0, 0, 0" "KeepWorldPosition" false)
  ;[1 1 1] Trapper Death SFX
  (if (not (Variables|Default|GetTrapper_Has_Died))
    (Variables|Default|SetRandomIteration _returnvalue)
    (bind _returnvalue_2 (Audio|SpawnSoundatLocation "/Game/05_Audio/SFX/MetaSounds/Enemies/Trapper/Death/MSS_Trapper_Death_Dry.MSS_Trapper_Death_Dry" (Transformation|GetWorldLocation (Variables|Character|GetMesh)) "0, 0, 0" 1.0 1.0 0.0 0 0))
    (bind _returnvalue_3 (Audio|SpawnSound2D "/Game/05_Audio/SFX/MetaSounds/Enemies/Trapper/Death/MSS_Trapper_Death_Delay.MSS_Trapper_Death_Delay" 1.0 1.0 0.0 0))
    (bind _returnvalue_4 (Audio|SpawnSound2D "/Game/05_Audio/SFX/MetaSounds/Enemies/Trapper/Death/MSS_Trapper_Death_Reverb.MSS_Trapper_Death_Reverb" 1.0 1.0 0.0 0))
    (Effects|Components|ParticleSystem|SetIntParameter _returnvalue_3 "IterationIndex" _returnvalue)
    (Variables|Default|SetTrapper_Has_Died true)))

(event Custom|onFade_Event
  (bind _dither_value (Timeline|Timeline PlayFromStart)
    (:Update
      (Rendering|Material|SetScalarParameterValue (Variables|Default|GetOpaque_Material) "Dither_Threshold" _dither_value :!class /Script/Engine.MaterialInstanceDynamic))))

(event EventBeginPlay
  (bind _mesh (Variables|Character|GetMesh))
  (Components|Timeline|SetPlayRate (Variables|Default|GetTL_Camouflage) (/ 1.0 (Variables|Default|GetCamouflage_Duree)))
  (Components|Timeline|SetPlayRate (Variables|Default|GetTL_DamageHit) (/ 1.0 (Variables|Default|GetHit_duree)))
  (Niagara|SpawnSystemAttached "/Game/04_FX/NS/Enemies/Trappeur/NS_Trappeur_Eyes.NS_Trappeur_Eyes" _mesh "eye_l" "0, 0, 0" "0, 0, 0" "KeepRelativeOffset" false)
  (Niagara|SpawnSystemAttached "/Game/04_FX/NS/Enemies/Trappeur/NS_Trappeur_Eyes.NS_Trappeur_Eyes" _mesh "eye_r" "0, 0, 0" "0, 0, 0" "KeepRelativeOffset" false)
  (EventDispatchers|AssignOnFade (delegate Custom|onFade_Event)))

(event Collision|EventActorBeginOverlap
  (params (OtherActor :type Actor%20Object%20Reference)))

(fn ConstructionScript
  (Utilities|FlowControl|Sequence
    (:then_0
      (bind _returnvalue (Rendering|Material|CreateDynamicMaterialInstance "/Game/03_Graph/Enemies/Materials/MI_trappeur.MI_trappeur" "None" "None" :!class /Script/Engine.KismetMaterialLibrary))
      (bind _output_get (Variables|Default|SetOpaque_Material _returnvalue))
      (Rendering|Material|SetMaterial (Variables|Character|GetMesh) 0 _output_get))
    (:then_1
      (bind _returnvalue_2 (Rendering|Material|CreateDynamicMaterialInstance "/Game/03_Graph/Enemies/Materials/MI_TrappeurTransluscent.MI_TrappeurTransluscent" "None" "None" :!class /Script/Engine.KismetMaterialLibrary))
      (Variables|Default|SetTransluscent_Material _returnvalue_2)
      (Rendering|Material|SetOverlayMaterial (Variables|Character|GetMesh) 0 :!class /Script/Engine.MeshComponent))
    (:then_2
      (Transformation|AttachComponentToComponent (Variables|Default|GetweakPoint) (Variables|Character|GetMesh) "Weak_Socket" "SnapToTarget" "SnapToTarget" "SnapToTarget" true))))

(fn UpdateOpaqueMaterial
  (params (UpdateExponent? :type Boolean) (ExponentValue :type Float%20%28double-precision%29) (UpdateVisibility? :type Boolean) (VisibilityValue :type Float%20%28double-precision%29))
  (bind _opaque_material (Variables|Default|GetOpaque_Material))
  (Utilities|FlowControl|Sequence
    (:then_0
      (if UpdateExponent?
        (Rendering|Material|SetScalarParameterValue _opaque_material "ExponentIn" ExponentValue :!class /Script/Engine.MaterialInstanceDynamic)))
    (:then_1
      (if UpdateVisibility?
        (Rendering|Material|SetScalarParameterValue _opaque_material "Trappeur_Visibility" VisibilityValue :!class /Script/Engine.MaterialInstanceDynamic)))))

(fn UpdateTransluscentMaterial
  (params (UpdateExponent? :type Boolean) (ExponentValue :type Float%20%28double-precision%29) (UpdateReflexion? :type Boolean) (ReflexionValue :type Float%20%28double-precision%29) (UpdateSwitch? :type Boolean) (Switch :type Float%20%28double-precision%29))
  (bind _transluscent_material (Variables|Default|GetTransluscent_Material))
  (Utilities|FlowControl|Sequence
    (:then_0
      (if UpdateExponent?
        (Rendering|Material|SetScalarParameterValue _transluscent_material "ExponentIn" ExponentValue :!class /Script/Engine.MaterialInstanceDynamic)))
    (:then_1
      (if UpdateReflexion?
        (Rendering|Material|SetScalarParameterValue _transluscent_material "reflexion_remove" ReflexionValue :!class /Script/Engine.MaterialInstanceDynamic)))
    (:then_2
      (if UpdateSwitch?
        (Rendering|Material|SetScalarParameterValue _transluscent_material "SwitchOverlay" Switch :!class /Script/Engine.MaterialInstanceDynamic)))))