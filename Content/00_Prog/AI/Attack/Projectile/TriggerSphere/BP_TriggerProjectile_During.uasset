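; BP_TriggerProjectile_During is an AI projectile-attack trigger actor that shows a lingering spit area effect.
; On BeginPlay it spawns the NS_AOE_Crachat Niagara system at its location and sets its lifetime.
; The stored hit normal drives the impact orientation, while the decal orientation comes from a fixed up vector.
; Overlap and Tick are empty, so this graph only handles the visuals.
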(event EventBeginPlay
  (bind _returnvalue (Niagara|SpawnSystematLocation "/Game/04_FX/NS/Enemies/Projectile/NS_AOE_Crachat.NS_AOE_Crachat" (Transformation|GetActorLocation)))
  (Niagara|SetNiagaraVariable(Vector3) _returnvalue "Impact_Orientation" (.Normal (Collision|BreakHitResult (Variables|Default|GethitResult))))
  (Niagara|SetNiagaraVariable(Float) _returnvalue "Lifetime" 7.0)
  (Class|NiagaraComponent|SetVariableQuat _returnvalue "Decal_Orientation" (Math|Conversions|ToQuaternion(Rotator) "0.000000,0.000000,1.000000")))

(event Collision|EventActorBeginOverlap
  (params (OtherActor :type Actor%20Object%20Reference)))

(event EventTick
  (params (DeltaSeconds :type Float%20%28single-precision%29)))

(fn ConstructionScript)