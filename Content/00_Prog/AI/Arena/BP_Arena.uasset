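; BP_Arena is a combat arena that responds to close and clear events, handling the intro cinematic, fight music and quest progression.
; On close, it can play a one-time level sequence with AI, player input and HUD disabled; otherwise combat begins directly.
; The appartion_monster event, or closing after the intro has played, restores them and starts combat.
; Clearing validates and adds optional quests, then ends fight music.
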(event Custom|onCloseArena_Event
  (bind _returnvalue (Game|GetPlayerCharacter 0))
  (bind _returnvalue_2 (Game|Player|GetPlayerPawn 0))
  ;[1 0.3486 0] Disable AI
  (if (Variables|Default|GetuseSequencer)
    (for _array_element (Variables|Default|GetlistAIs)
      (Class|AIBase|EnableAI _array_element false))
    (if (and (Variables|Default|GetuseSequencer) (< (Variables|/Script/RobotHunter.ArenaManager|Getindex (Variables|Default|GetarenaManager)) 1))
      (Utilities|FlowControl|Sequence
        (:then_0
          ;[1 0 0.003386 1 25] Deactivate Chara
          (bind _asmain_character (Utilities|Casting|CastToMainCharacter _returnvalue_2))
          (bind _asplayer_controller (Utilities|Casting|CastToPlayerController (Pawn|GetController _returnvalue_2)))
          (Input|DisableInput _asmain_character _asplayer_controller)
          (Class|MainCharacter|DeactivateMembers _asmain_character (Utilities|Array|MakeArray) true))
        (:then_1
          (bind _outactor (Sequencer|Player|CreateLevelSequencePlayer (Variables|Default|GetlevelSequencer)))
          (Variables|Default|SetarenaCameraTransform (Variables|Default|GetTransform_camera))
          (Variables|Default|SetRef_Sequence%20Player (Variables|/Script/LevelSequence.LevelSequenceActor|GetSequencePlayer _outactor))
          ;[1 1 1] Hide UI
          (bind _asbp_game_hud (Utilities|Casting|CastToBp_GameHUD (HUD|GetHUD (Game|GetPlayerController 0))))
          (Class|MainHUD|HideUI _asbp_game_hud)
          (Sequencer|Player|Play (Variables|/Script/LevelSequence.LevelSequenceActor|GetSequencePlayer _outactor) :!class /Script/MovieScene.MovieSceneSequencePlayer)
          (Variables|/Script/RobotHunter.ArenaManager|Setindex (Variables|Default|GetarenaManager) 1))
        (:then_2
          ;[1 1 1] Agressive Lightnings SFX Muted
          (Development|PrintString "AGRESSIVE LIGHTNINGS SFX MUTED" true true "(R=0.000000,G=1.000000,B=0.602688,A=1.000000)" 5.0)
          (Audio|PushSoundMixModifier "/Game/05_Audio/SoundClass_Mixes/Enemies_Muted/SCM_Agressive_Lightnings_Muted.SCM_Agressive_Lightnings_Muted")))
      (else
        (Utilities|FlowControl|Sequence
          (:then_0
            ;[0 0.3796 1] Enable AI
            (for _array_element_2 (Variables|Default|GetlistAIs)
              (Class|AIBase|EnableAI _array_element_2 true))
            ;[0.107 1 0 1 25] Reactivate Chara
            (bind _asmain_character_2 (Utilities|Casting|CastToMainCharacter _returnvalue))
            (bind _asplayer_controller_2 (Utilities|Casting|CastToPlayerController (Pawn|GetController _returnvalue)))
            (Input|EnableInput _asmain_character_2 _asplayer_controller_2)
            (Class|MainCharacter|ReactivateMembers _asmain_character_2 (Utilities|Array|MakeArray))
            ;[1 0 0.9603] Launch Combat
            (Class|Arena|EndSequencer)
            (Utilities|FlowControl|Sequence
              (:then_0
                (bind _bgm_manager_ref (Variables|Default|GetBGM_Manager_Ref)
                  (:then
                    (Default|FightStarted _bgm_manager_ref) ; Start Fight BGM
                  )
                  (:else)))))
          (:then_1
            (bind _asbp_game_hud_2 (Utilities|Casting|CastToBp_GameHUD (HUD|GetHUD (Game|GetPlayerController 0))))
            (Class|MainHUD|ShowUI _asbp_game_hud_2)
            (Class|FocusSystem|SetFocusto (Class|MainHUD|GetFocusSystem _asbp_game_hud_2) "GAME" 0 true false)))))
    (else
      ;;[1 1 1] Combat immediately started
      (bind _bgm_manager_ref_2 (Variables|Default|GetBGM_Manager_Ref)
        (:then
          (Default|FightStarted _bgm_manager_ref_2) ; Start Fight BGM
        )
        (:else)))))

(event Custom|appartion_monster
  (bind _returnvalue (Game|GetPlayerCharacter 0))
  (Utilities|FlowControl|Sequence
    (:then_0
      ;[0 0.3796 1] Enable AI
      (for _array_element (Variables|Default|GetlistAIs)
        (Class|AIBase|EnableAI _array_element true))
      ;[0.107 1 0 1 25] Reactivate Chara
      (bind _asmain_character (Utilities|Casting|CastToMainCharacter _returnvalue))
      (bind _asplayer_controller (Utilities|Casting|CastToPlayerController (Pawn|GetController _returnvalue)))
      (Input|EnableInput _asmain_character _asplayer_controller)
      (Class|MainCharacter|ReactivateMembers _asmain_character (Utilities|Array|MakeArray))
      ;[1 0 0.9603] Launch Combat
      (Class|Arena|EndSequencer)
      (Utilities|FlowControl|Sequence
        (:then_0
          (bind _bgm_manager_ref (Variables|Default|GetBGM_Manager_Ref)
            (:then
              (Default|FightStarted _bgm_manager_ref) ; Start Fight BGM
            )
            (:else)))))
    (:then_1
      (bind _asbp_game_hud (Utilities|Casting|CastToBp_GameHUD (HUD|GetHUD (Game|GetPlayerController 0))))
      (Class|MainHUD|ShowUI _asbp_game_hud)
      (Class|FocusSystem|SetFocusto (Class|MainHUD|GetFocusSystem _asbp_game_hud) "GAME" 0 true false))))

(event Custom|onClearArena_Event
  (params (exitGate :type Alien%20Door%20Object%20Reference) (giveBonus :type Boolean))
  (bind _questmanager (Variables|Default|GetQuestManager))
  (bind _output (Utilities|ResolveSoftReference _questmanager))
  (Utilities|FlowControl|Sequence
    (:then_0
      (bind _questtovalid (Variables|Default|GetQuestToValid)
        (:then
          (Class|QuestManager|ValidQuest _output (Utilities|ResolveSoftReference _questtovalid)))
        (:else)))
    (:then_1
      (bind _questtoinit (Variables|Default|GetQuestToInit)
        (:then
          (Class|QuestManager|AddQuest _output (Utilities|ResolveSoftReference _questtoinit)))
        (:else)))
    (:then_2
      ;[1 1 1] Combat Ended
      (bind _bgm_manager_ref (Variables|Default|GetBGM_Manager_Ref)
        (:then
          (Default|FightEnded _bgm_manager_ref (Class|Arena|GetFinalArena)) ; End Fight BGM
        )
        (:else)))))

(event EventBeginPlay
  (EventDispatchers|AssignOnCloseArena (delegate Custom|onCloseArena_Event))
  (EventDispatchers|AssignOnClearArena (delegate Custom|onClearArena_Event)))

(fn ConstructionScript)